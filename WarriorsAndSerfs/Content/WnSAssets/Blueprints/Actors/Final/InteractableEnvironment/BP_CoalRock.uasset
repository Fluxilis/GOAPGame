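; BP_CoalRock is a harvestable coal rock that sinks as its resource is depleted.
; On BeginPlay it stores the model's start location and computes a lower end point from its bounds, offset to keep it visible.
; It overrides the parent's harvest visual event to lerp the model between those points by the ratio of remaining to maximum resource.
; A test boolean on Tick triggers a single harvest.
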(event EventBeginPlay
  (|CallParentFunction)
  (ResourceAmountVisual|InitModelSinkingLocations))

(event EventHandleHarvestResourceVisual
  ;[1 1 1] Override HandleHarvestResourceVisual
  (ResourceAmountVisual|RockHandleHarvestResourceVisual))

(event EventTick
  (params (DeltaSeconds :type Float%20%28single-precision%29))
  (if (Variables|Default|GetTESTINGBOOL)
    (CallFunction|HarvestResource)
    (Variables|Default|SetTESTINGBOOL false)))

(fn ConstructionScript
  (|CallParentFunction))

(fn RockHandleHarvestResourceVisual
  (Transformation|SetWorldLocation (Variables|Default|GetModel) (Math|Vector|Lerp(Vector) (Variables|ResourceAmountVisual|GetmodelFinalLocation) (Variables|ResourceAmountVisual|GetmodelStartLocation) (/ (Math|Conversions|ToFloat(Integer) (Variables|Default|GetresourceAmount)) (Math|Conversions|ToFloat(Integer) (Variables|Default|GetmaxResourceAmount)))) false false))

(fn InitModelSinkingLocations
  (bind _model (Variables|Default|GetModel))
  (bind _returnvalue (Transformation|GetWorldLocation _model))
  (bind (_x _y _z) (Math|Vector|BreakVector _returnvalue))
  (Variables|ResourceAmountVisual|SetmodelStartLocation (Transformation|GetWorldLocation (Variables|Default|GetModel)))
  (Variables|ResourceAmountVisual|SetmodelFinalLocation (Math|Vector|MakeVector _x _y (+ (* 2 (- _z (.z (.BoxExtent (Collision|GetComponentBounds (Variables|Default|GetModel)))))) 3e+01))))