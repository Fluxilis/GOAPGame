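; BP_Builder is a civilian subject whose job is to seek out construction sites of its owning player that can currently be built on.
; FindAndAssignJob keeps a valid target or scans the ActorManager's sites with a distance check meant to find the closest, though ClosestDistance is never updated in the loop.
; HasValidJob clears the target when it is invalid or unbuildable.
; The job description reflects eating, moving to a site or idling.
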(event EventUpdateCurrentJobDescription
  ;[1 1 1] Override Update Job Description
  (if (Variables|Default|GetgoingToEat)
    (Variables|Default|SetCurrentJobDescription "Currently going to eat.")
    (elif (Variables|Job|GethasTarget)
      (Variables|Default|SetCurrentJobDescription "Currently moving to a constructionsite.")
      (else
        (Variables|Default|SetCurrentJobDescription "Currently idle.")))))

(fn ConstructionScript
  (|CallParentFunction))

(fn FindandAssignJob
  (if (Variables|Job|GethasTarget)
    (if (Utilities|IsValidandNotNull (Variables|Job|GetcurrentConstructionsite))
      (return true) ; Already has target
      (else
        (Variables|Job|SethasTarget false) ; If has a target, but no target is defined\nset hastarget to false and search a new one.
      )))
  ;[1 1 1] Find the closest Construction site
  (for _array_element (Variables|/Game/WnSAssets/Blueprints/Logics/Managers/BP_ActorManager.BP_ActorManager_C|GetConstructionsites (Variables|Default|GetactorManager))
    (if (< (Utilities|VectorDistanceAbs (Transformation|GetWorldLocation (Variables|Default|GetCapsuleComponent)) (Default|GetDoorLocation _array_element)) (LocalVariables|GetclosestDistance)) ; is this closer than the previous closest?
      (bind _returnvalue (Class|ConstructionComponent|CanBuild (Variables|/Game/WnSAssets/Blueprints/Actors/Final/Construction/BP_ConstructionSite.BP_ConstructionSite_C|GetConstruction _array_element)))
      (if _returnvalue ; Can we build here?
        (if (Utilities|Name|Equal(Name) (Variables|/Game/WnSAssets/Blueprints/Actors/Intermediates/Lots/BP_Lot.BP_Lot_C|GetowningPlayerName _array_element) (Variables|Default|GetowningPlayerName)) ; does this construction belong to my player?
          (LocalVariables|SetclosestConstructionSite _array_element)))))
  (if (Utilities|IsValidandNotNull (LocalVariables|GetclosestConstructionSite))
    (Variables|Job|SethasTarget true)
    (Variables|Job|SetcurrentConstructionsite (LocalVariables|GetclosestConstructionSite))
    (CallFunction|UpdateJobDescriptiononServer)
    (return true)
    (else
      (CallFunction|UpdateJobDescriptiononServer)
      (return false) ; Could not find a target
    )))

(fn HasValidJob
  (if (Variables|Job|GethasTarget)
    (if (Utilities|IsValidandNotNull (Variables|Job|GetcurrentConstructionsite))
      (bind _returnvalue (Class|ConstructionComponent|CanBuild (Variables|/Game/WnSAssets/Blueprints/Actors/Final/Construction/BP_ConstructionSite.BP_ConstructionSite_C|GetConstruction (Variables|Job|GetcurrentConstructionsite))))
      (if _returnvalue ; Can we build at this constructionsite \nright now? (enough materials?"
        (return true)
        (else
          _))))
  (Variables|Job|SethasTarget false)
  (Variables|Job|SetcurrentConstructionsite 0)
  (return false))