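; Miner civilian subject Blueprint, a child class that specializes inherited home and job behavior for mine workers.
; FindPlantJob always returns false, and SetHarvestType stores the given type in HarvestTargetType.
; FindNewHome calls the parent version, but its follow-up logic is disconnected and never runs.
; That unused logic would map a coal, gold or iron mine home building to the matching harvest type.
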(event EventBeginPlay
  (|CallParentFunction))

(event Collision|EventActorBeginOverlap
  (params (OtherActor :type Actor%20Object%20Reference))
  (|CallParentFunction OtherActor))

(event EventTick
  (params (DeltaSeconds :type Float%20%28single-precision%29))
  (|CallParentFunction DeltaSeconds))

(fn ConstructionScript
  (|CallParentFunction))

(fn FindPlantJob
  (return false))

(fn FindNewHome
  (bind _foundahome_ (|CallParentFunction)))

(fn SetHarvestType
  (params (harvestableType :type Name))
  (Variables|Default|SetharvestTargetType harvestableType))