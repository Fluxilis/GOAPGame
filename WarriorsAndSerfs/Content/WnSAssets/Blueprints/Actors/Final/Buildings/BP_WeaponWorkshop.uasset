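; Weapon Workshop building Blueprint that adds tutorial tracking for crafted hand axes on top of its parent's behavior.
; Tick runs a time-throttled check that stops once the "Basic08" tutorial is completed.
; Each check sends the increase in the Crafting component's lifetime recipe count since the previous check to the tutorial manager as hand axes.
; The manager reference is lazily fetched from the player controller and cached.
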(event EventTick
  (params (DeltaSeconds :type Float%20%28single-precision%29))
  (|CallParentFunction DeltaSeconds)
  (Tutorial|HandleBasic08))

(fn ConstructionScript
  (|CallParentFunction))

(fn HandleBasic08
  (if (not (Variables|Tutorial|GetBasic08Completed))
    ;[1 1 1] The check part of the function is kind of performant, I don't want to do it every tick.
    (if (> (Utilities|Time|GetGameTimeinSeconds) (+ (Variables|Tutorial|GetBasic08LastCheckedTime) (Variables|Tutorial|GetBasic08CheckTimeDelay))) ; Has enough time passed?
      (Variables|Tutorial|SetBasic08LastCheckedTime (Utilities|Time|GetGameTimeinSeconds))
      (if (Utilities|IsValidandNotNull (Variables|Tutorial|GettutManager))
        (bind _completed (Default|GetTutorialCompletionStatus (Variables|Tutorial|GettutManager) "Basic08" :!label _label))
        (if _completed
          (Variables|Tutorial|SetBasic08Completed true)
          (else
            ;[1 1 1] Adds as many handaxes to the tutmanager as were produced since the last time this code was executed.
            ; ->Ensures that tutmanager counts all axes that were produced here
            (Default|Basic08AddHandAxes (Variables|Tutorial|GettutManager) (Math|Float|Truncate (- (Variables|/Script/WarriorsAndSerfs.CraftingComponent|GetlifeTimeRecipes (Variables|Default|GetCrafting)) (Math|Conversions|ToFloat(Integer) (Variables|Tutorial|GetlastCheckAxesCraftedAmt)))))
            (Variables|Tutorial|SetlastCheckAxesCraftedAmt (Math|Float|Truncate (Variables|/Script/WarriorsAndSerfs.CraftingComponent|GetlifeTimeRecipes (Variables|Default|GetCrafting))))))
        (else
          (bind _aswn_s_player_controller (Utilities|Casting|CastToWnS_PlayerController (Game|GetPlayerController 0))
            (:then
              (Variables|Tutorial|SettutManager (Variables|/Game/WnSAssets/Blueprints/Player/WnS_PlayerController.WnS_PlayerController_C|GettutorialManager _aswn_s_player_controller))
              (goto _label))
            (:CastFailed
              (Utilities|PrintStringRed15 "WeaponWorkshop HandleBasic08 cast to pc failed!"))))))))