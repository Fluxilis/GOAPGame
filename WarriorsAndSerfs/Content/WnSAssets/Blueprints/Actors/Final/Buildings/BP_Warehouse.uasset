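; Warehouse building Blueprint that can start with a preset stock of resources and advances the basic tutorial when its UI opens.
; On BeginPlay, it creates fixed amounts of goods and gold if the starting-inventory flag is set.
; Opening the UI runs a sequenced check that completes tutorial Basic03 once Basic02 is done, caching both statuses locally from the player controller's TutorialManager.
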(event EventBeginPlay
  (|CallParentFunction)
  (if (Variables|BuildingSpecific|GethasStartingInventory)
    (CallFunction|AddStartingInventory)))

(event EventOpenUI
  (params (isOwnerUI :type Boolean))
  (|CallParentFunction isOwnerUI)
  (Tutorial|HandleTutBasic03))

(fn ConstructionScript
  (|CallParentFunction))

(fn AddStartingInventory
  (Class|Lot|MakeItem "Log" 10)
  (Class|Lot|MakeItem "Stone" 20)
  (Class|Lot|MakeItem "Fish" 20)
  (Class|Lot|MakeItem "Lumber" 20)
  (Class|Lot|MakeItem "GoldCoins" 80)
  (Class|Lot|MakeItem "Bread" 20))

(fn HandleTutBasic03
  (Utilities|FlowControl|Sequence
    (:then_0
      (if (Variables|Tutorial|GetBasic03Completed) ; Was tutorial basic03 completed yet?\n(check local)
        (return)
        (else
          (bind _aswn_s_player_controller (Utilities|Casting|CastToWnS_PlayerController (Game|GetPlayerController 0))
            (:then
              (bind _completed (Default|GetTutorialCompletionStatus (Variables|/Game/WnSAssets/Blueprints/Player/WnS_PlayerController.WnS_PlayerController_C|GettutorialManager _aswn_s_player_controller) "Basic03"))
              (if _completed ; Was tutorial basic03 ACTUALLY completed yet?\n(Check tutorial manager)
                (Variables|Tutorial|SetBasic03Completed true)
                (return)))
            (:CastFailed
              (Utilities|PrintStringRed15 "warehouse open UI cast to playercontroller failed"))))))
    (:then_1
      (if (not (Variables|Tutorial|GetBasic02Completed)) ; Was the previous tut completed yet?\n(check local)
        (bind _aswn_s_player_controller_2 (Utilities|Casting|CastToWnS_PlayerController (Game|GetPlayerController 0))
          (:then
            (bind _completed_2 (Default|GetTutorialCompletionStatus (Variables|/Game/WnSAssets/Blueprints/Player/WnS_PlayerController.WnS_PlayerController_C|GettutorialManager _aswn_s_player_controller_2) "Basic02"))
            (if _completed_2 ; Was tutorial basic02 ACTUALLY completed yet?\n(Check tutorial manager)
              (Variables|Tutorial|SetBasic02Completed true)
              (else
                (return))))
          (:CastFailed
            (Utilities|PrintStringRed15 "warehouse open UI cast to playercontroller failed (2)")))))
    (:then_2
      (bind _aswn_s_player_controller_3 (Utilities|Casting|CastToWnS_PlayerController (Game|GetPlayerController 0)))
      (Default|CompleteTutorial (Variables|/Game/WnSAssets/Blueprints/Player/WnS_PlayerController.WnS_PlayerController_C|GettutorialManager _aswn_s_player_controller_3) "Basic03"))))