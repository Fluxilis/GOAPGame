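; Residential house building that houses citizens and raises the citizen limit while registered with the actor manager.
; Overrides of add and remove from the actor manager add or subtract its capacity from that limit.
; Each tick, while below capacity and once a spawn delay has passed, it spawns a serf at its door, owned by the same player, with itself as residence.
; AddResident and RemoveResident maintain the resident list and count.
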(event EventBeginPlay
  (|CallParentFunction) ; This node is disabled and will not be called.\nDrag off pins to build functionality.
)

(event Collision|EventActorBeginOverlap
  (params (OtherActor :type Actor%20Object%20Reference)))

(event EventTick
  (params (DeltaSeconds :type Float%20%28single-precision%29))
  (|CallParentFunction DeltaSeconds)
  (ResidentialHouse|SpawnNewCitizens))

(event EventRemovefromActorManager
  ;[1 1 1] Override Add/Remove from actor manager, to change Citizen limit.
  (|CallParentFunction)
  (ResidentialHouse|ResidentialHouseRemovefromActorManager))

(event EventAddtoActorManager
  ;[1 1 1] Override Add/Remove from actor manager, to change Citizen limit.
  (|CallParentFunction)
  (ResidentialHouse|ResidentialHouseAddtoActorManager))

(fn ConstructionScript
  (|CallParentFunction))

(fn ResidentialHouseAddtoActorManager
  (Default|ChangeCitizenLimit (Variables|Default|GetactorManager) (Variables|ResidentialHouse|GetcitizenCapacity)))

(fn ResidentialHouseRemovefromActorManager
  (Default|ChangeCitizenLimit (Variables|Default|GetactorManager) (* (Variables|ResidentialHouse|GetcitizenCapacity) -1)))

(fn SpawnNewCitizens
  (if (< (Variables|ResidentialHouse|GetcurrentCitizenCount) (Variables|ResidentialHouse|GetcitizenCapacity)) ; capacity for more citizens?
    (if (> (Utilities|Time|GetGameTimeinSeconds) (+ (Variables|ResidentialHouse|GetlastCitizenSpawnedTime) (Variables|ResidentialHouse|GetnewCitizenSpawnDelay))) ; time to spawn new?
      (Variables|ResidentialHouse|SetlastCitizenSpawnedTime (Utilities|Time|GetGameTimeinSeconds))
      ;[1 1 1] Spawn new citizen
      (bind _returnvalue (Game|SpawnActorfromClass "/Game/WnSAssets/Blueprints/Actors/Final/Subjects/Civilian/BP_Serf.BP_Serf_C" (Math|Conversions|ToTransform(Vector) (CallFunction|GetDoorLocation)) "Undefined" 0 (Variables|Default|GetowningPlayerName) "None" false 0))
      (Default|SetResidence _returnvalue self))))

(fn AddResident
  (params (newResident :type BP%20Subject%20Object%20Reference))
  (Utilities|Array|Add (Variables|ResidentialHouse|Getresidents) newResident)
  (Math|Integer|IncrementInt (Variables|ResidentialHouse|GetcurrentCitizenCount)))

(fn RemoveResident
  (params (newResident :type BP%20Subject%20Object%20Reference))
  (Utilities|Array|RemoveItem (Variables|ResidentialHouse|Getresidents) newResident)
  (Math|Integer|DecrementInt (Variables|ResidentialHouse|GetcurrentCitizenCount)))