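; Woodcutters building actor that adds tracking for the "Basic05" tutorial on top of its parent class's behavior.
; Until that tutorial is known to be complete, Tick polls the player controller's TutorialManager for its status.
; A positive lifetime production count on the Harvesting component sets the woodcutter flag on the manager.
; When both that flag and the Sawmill flag are set, it completes the tutorial.
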(event EventTick
  (params (DeltaSeconds :type Float%20%28single-precision%29))
  (|CallParentFunction DeltaSeconds)
  (if (not (Variables|Tutorial|Getbasic05Completed))
    (CallFunction|HandleBasic05)))

(fn ConstructionScript
  (|CallParentFunction))

(fn HandleBasic05
  (if (not (Variables|Tutorial|Getbasic05Completed))
    (bind _aswn_s_player_controller (Utilities|Casting|CastToWnS_PlayerController (Game|GetPlayerController 0))
      (:then
        (bind _output_get (LocalVariables|SettutManager (Variables|/Game/WnSAssets/Blueprints/Player/WnS_PlayerController.WnS_PlayerController_C|GettutorialManager _aswn_s_player_controller)))
        (bind _completed (Default|GetTutorialCompletionStatus _output_get "Basic05"))
        (if _completed ; Has the tutorial Basic05 \nbeen completed yet?
          (Variables|Tutorial|Setbasic05Completed true)
          (else
            (Utilities|FlowControl|Sequence
              (:then_0
                ;[1 0 0] Sequence Then 0
                (if (> (Variables|/Script/WarriorsAndSerfs.HarvestingComponent|GetlifeTimePolishes (Variables|Default|GetHarvesting)) 0.0) ; has this woodcutter ever \nmade an item?
                  (Variables|/Game/WnSAssets/Tutorial/TutorialManager.TutorialManager_C|SetBasic05WoodCutter (LocalVariables|GettutManager) true)))
              (:then_1
                (if (and (Variables|/Game/WnSAssets/Tutorial/TutorialManager.TutorialManager_C|GetBasic05Sawmill (LocalVariables|GettutManager)) (Variables|/Game/WnSAssets/Tutorial/TutorialManager.TutorialManager_C|GetBasic05WoodCutter (LocalVariables|GettutManager))) ; Have all components of \nthe tutorial been completed?
                  (Default|CompleteTutorial (LocalVariables|GettutManager) "Basic05")))))))
      (:CastFailed
        (Utilities|PrintStringRed15 "Woodcutters HandleBasic05 cast to pc failed!")))))