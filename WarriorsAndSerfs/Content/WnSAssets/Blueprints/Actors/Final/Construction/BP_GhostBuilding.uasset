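; BP_GhostBuilding is a placement preview for a building, showing whether it fits at its current spot.
; InitGhostBuilding briefly spawns the real building class to copy its mesh, model transform and door position, then destroys it and sets the overhead icon.
; GhostMesh overlaps drive CanPlaceBuildingHere and swap materials: red when blocked, default ghost when clear.
; TintCanPlaceHere re-checks overlaps, tinting green or red.
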(event OnComponentEndOverlap(GhostMesh)
  (params (OverlappedComponent :type Primitive%20Component%20Object%20Reference) (OtherActor :type Actor%20Object%20Reference) (OtherComp :type Primitive%20Component%20Object%20Reference) (OtherBodyIndex :type Integer))
  (if (<= (Utilities|Array|Length (Collision|GetOverlappingActors (Variables|Default|GetGhostMesh) 0 :!class /Script/Engine.PrimitiveComponent)) 0) ; If not overlapping anything else
    (if true
      (Rendering|Material|CreateDynamicMaterialInstance (Variables|Default|GetGhostMesh) 0 "/Game/WnSAssets/Visual/Mats/M_GhostBuilding.M_GhostBuilding" "None" :!class /Script/Engine.PrimitiveComponent)
      (Variables|Default|SetCanPlaceBuildingHere true))))

(event OnComponentBeginOverlap(GhostMesh)
  (params (OverlappedComponent :type Primitive%20Component%20Object%20Reference) (OtherActor :type Actor%20Object%20Reference) (OtherComp :type Primitive%20Component%20Object%20Reference) (OtherBodyIndex :type Integer) (bFromSweep :type Boolean) (SweepResult :type Hit%20Result%20Structure%20%28by%20ref%29))
  (Rendering|Material|CreateDynamicMaterialInstance (Variables|Default|GetGhostMesh) 0 "/Game/WnSAssets/Visual/Mats/M_GhostBuildingTintRed.M_GhostBuildingTintRed" "None" :!class /Script/Engine.PrimitiveComponent)
  (Variables|Default|SetCanPlaceBuildingHere false))

(fn ConstructionScript)

(fn InitGhostBuilding
  (params (whatBuilding :type Name))
  (bind _ghostmesh (Variables|Default|GetGhostMesh))
  (bind _ghostmesh_2 (Variables|Default|GetGhostMesh))
  (bind _output_get (Variables|Default|SetRealBuildingType whatBuilding))
  (CallFunction|SetOverheadIconandUi)
  (bind _output_get_2 (Variables|Default|SetRealBuildingBlueprint (CallFunction|GetBuildingClassDT _output_get)))
  (bind _returnvalue (Game|SpawnActorfromClass _output_get_2 (Transformation|GetWorldTransform (Variables|Default|GetGhostMesh)) "AlwaysSpawn" 0 "DONOTHANDLE" 0)) ; I need to spawn the actual building to get the model out of it.\nThis object will be deleted by the end of this function.
  ;[1 1 1] Sets Mesh of the Ghostbuilding to that of the final building.
  ; SetScale, rotation and position are necessary in case the model is rotated, scaled or moved in the building BP viewport.
  (Components|StaticMesh|SetStaticMesh _ghostmesh_2 (Variables|/Script/Engine.StaticMeshComponent|GetStaticMesh (Variables|/Game/WnSAssets/Blueprints/Actors/Intermediates/Lots/BP_Lot.BP_Lot_C|GetModel _returnvalue)))
  (Transformation|SetRelativeScale3D _ghostmesh_2 (Variables|/Script/Engine.SceneComponent|GetRelativeScale3D (Variables|/Game/WnSAssets/Blueprints/Actors/Intermediates/Lots/BP_Lot.BP_Lot_C|GetModel _returnvalue)))
  (Transformation|SetRelativeRotation _ghostmesh_2 (Variables|/Script/Engine.SceneComponent|GetRelativeRotation (Variables|/Game/WnSAssets/Blueprints/Actors/Intermediates/Lots/BP_Lot.BP_Lot_C|GetModel _returnvalue)) false false)
  (Transformation|SetRelativeLocation _ghostmesh_2 (Variables|/Script/Engine.SceneComponent|GetRelativeLocation (Variables|/Game/WnSAssets/Blueprints/Actors/Intermediates/Lots/BP_Lot.BP_Lot_C|GetModel _returnvalue)) false false)
  (Transformation|SetWorldTransform (Variables|Default|Getdoor) (Transformation|GetWorldTransform (Variables|/Game/WnSAssets/Blueprints/Actors/Intermediates/Lots/BP_Lot.BP_Lot_C|GetDoor _returnvalue)) false false)
  (Class|Lot|DestroyLot _returnvalue)
  ;[1 1 1] Tint red if cannot place building
  (if (<= (Utilities|Array|Length (Collision|GetOverlappingActors (Variables|Default|GetGhostMesh) 0 :!class /Script/Engine.PrimitiveComponent)) 0) ; If not overlapping anything else
    (Rendering|Material|CreateDynamicMaterialInstance _ghostmesh 0 "/Game/WnSAssets/Visual/Mats/M_GhostBuilding.M_GhostBuilding" "None" :!class /Script/Engine.PrimitiveComponent)
    (Variables|Default|SetCanPlaceBuildingHere true)
    (else
      (Rendering|Material|CreateDynamicMaterialInstance _ghostmesh 0 "/Game/WnSAssets/Visual/Mats/M_GhostBuildingTintRed.M_GhostBuildingTintRed" "None" :!class /Script/Engine.PrimitiveComponent)
      (Variables|Default|SetCanPlaceBuildingHere false))))

(fn TintCanPlaceHere
  (bind _ghostmesh (Variables|Default|GetGhostMesh))
  (if (<= (Utilities|Array|Length (Collision|GetOverlappingActors (Variables|Default|GetGhostMesh) 0 :!class /Script/Engine.PrimitiveComponent)) 0) ; Is not Overlapping something?
    (Rendering|Material|CreateDynamicMaterialInstance _ghostmesh 0 "/Game/WnSAssets/Visual/Mats/M_GhostBuildingTintGreen.M_GhostBuildingTintGreen" "None" :!class /Script/Engine.PrimitiveComponent)
    (Variables|Default|SetCanPlaceBuildingHere true)
    (else
      (Rendering|Material|CreateDynamicMaterialInstance _ghostmesh 0 "/Game/WnSAssets/Visual/Mats/M_GhostBuildingTintRed.M_GhostBuildingTintRed" "None" :!class /Script/Engine.PrimitiveComponent)
      (Variables|Default|SetCanPlaceBuildingHere false))))

(fn CheckCanPlaceHere
  (return (<= (Utilities|Array|Length (Collision|GetOverlappingActors (Variables|Default|GetGhostMesh) 0 :!class /Script/Engine.PrimitiveComponent)) 0)))

(fn SetOverheadIconandUi
  ;[1 1 1] Set Overhead Icon (Temporary)
  (bind _astexture_2d (Utilities|Casting|CastToTexture2D (CallFunction|GetBuildingIconDT (Variables|Default|GetRealBuildingType)))
    (:then
      (Rendering|Components|Sprite|SetSprite (Variables|Default|GetbuildingIcon) _astexture_2d)
      (Development|SetHiddeninGame (Variables|Default|GetbuildingIcon) false false))
    (:CastFailed
      (Utilities|PrintStringRed15 "Ghostbuilding setoverheadIcon cast to texture2d failed!"))))