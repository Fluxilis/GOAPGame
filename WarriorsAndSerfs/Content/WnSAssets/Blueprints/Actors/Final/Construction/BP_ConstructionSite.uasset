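; BP_ConstructionSite is the placeholder lot for a building under construction.
; Placement briefly spawns the real building to copy its mesh, recipe, door and health, creates material stockpiles and updates tutorials.
; Builder hits raise the mesh from below ground and add health until the real building replaces the site.
; It also handles a movable harvest-area marker for harvesting buildings and partially refunds used materials in loot boxes when unfinished.
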(event Custom|SetHarvestingAreaOnServer
  (params (location :type Vector))
  ;[1 1 1] Replication - Set Harvesting Area
  (HarvestingBuildingConstruction|SetNewHarvestingAreaLocation location) ; Set locally first
  (bind _aswn_s_player_controller (Utilities|Casting|CastToWnS_PlayerController (Game|GetPlayerController 0)))
  (Default|SetConstructionHarvestingArea _aswn_s_player_controller self location))

(event Custom|NotifyClientsInitVisuals
  (params (mesh :type Static%20Mesh%20Object%20Reference) (scale :type Vector) (rotation :type Rotator) (location :type Vector) (playerLabel :type String))
  ;[1 1 1] Replication - Init Variables on clients
  (CallFunction|InitVisuals mesh scale rotation location playerLabel))

(event Custom|NotifyClientsNewHarvestingArea
  (params (location :type Vector))
  ;[1 1 1] Replication - Set Harvesting Area
  (HarvestingBuildingConstruction|SetNewHarvestingAreaLocation location))

(event EventOpenUI
  (params (isOwnerUI :type Boolean))
  ;[1 1 1] Override Open UI - also show harvesting marker, if constructionsite is for harvesting building.
  (|CallParentFunction isOwnerUI)
  (if isOwnerUI ; Only show for Owner of Building
    (if (Utilities|ClassIsChildOf (Variables|Construction|GetRealBuildingBP) "/Game/WnSAssets/Blueprints/Actors/Intermediates/Lots/BP_HarvestingBuilding.BP_HarvestingBuilding_C") ; Is the construction for a \nharvesting building?
      (HarvestingBuildingConstruction|ShowHarvestingAreaMarker true))))

(event EventCloseUI
  ;[1 1 1] Override Close UI - if constructionsite is for harvesting building: Hide Harvest Area marker, and cancel moving harvesting area
  (|CallParentFunction)
  (if (Utilities|ClassIsChildOf (Variables|Construction|GetRealBuildingBP) "/Game/WnSAssets/Blueprints/Actors/Intermediates/Lots/BP_HarvestingBuilding.BP_HarvestingBuilding_C") ; Is the construction for a \nharvesting building?
    (HarvestingBuildingConstruction|ShowHarvestingAreaMarker false)
    (bind _aswns_player (Utilities|Casting|CastToWnsPlayer (Pawn|GetControlledPawn (Game|GetPlayerController 0)))
      (:then
        (Default|CancelMoveHarvestingArea _aswns_player))
      (:CastFailed
        (Development|PrintString "HarvestingBuiliding CloseUI Cast to wnsPlayer failed!")))))

(event EventHandleIncreaseJobPriorities
  ;[1 1 1] Override HandleIncreaseJobPriorities - Do not increase priorities for palace construction sites!
  (if (not (== (Variables|Construction|GetRealBuildingBP) "/Game/WnSAssets/Blueprints/Actors/Final/Buildings/BP_Palace.BP_Palace_C")) ; Do not increase priorities for palace.
    (|CallParentFunction)))

(event EventDestroyed
  ;[1 1 1] Override Destroyed
  ; If Harvesting Construction: destroy area marker
  (if (Utilities|ClassIsChildOf (Variables|Construction|GetRealBuildingBP) "/Game/WnSAssets/Blueprints/Actors/Intermediates/Lots/BP_HarvestingBuilding.BP_HarvestingBuilding_C")
    (Actor|DestroyActor (Variables|HarvestingBuildingConstruction|GetharvestingAreaMarker))
    (|CallParentFunction)))

(event EventBeginPlay
  ;[1 1 1] Begin Play
  ; If constructing harvesting building: Init Harvest Area Marker and Set variable in component
  (|CallParentFunction)
  (if (Utilities|ClassIsChildOf (Variables|Construction|GetRealBuildingBP) "/Game/WnSAssets/Blueprints/Actors/Intermediates/Lots/BP_HarvestingBuilding.BP_HarvestingBuilding_C")
    (HarvestingBuildingConstruction|InitHarvestingAreaMarker)))

(fn ConstructionScript
  (|CallParentFunction))

(fn InitPlaced
  (Tutorial|HandleTutorials)
  (Networking|SwitchHasAuthority
    (:Authority
      ;[1 1 1] I need to set a few things based on the building that will be constructed here.
      ; In order to do this, I spawn that building and read defaults, then despawn it.
      ; (I cannot use the class defaults node for all of these)
      (bind _returnvalue (Game|SpawnActorfromClass (Variables|Construction|GetRealBuildingBP) (Transformation|GetWorldTransform (Variables|Default|GetDefaultSceneRoot)) "AlwaysSpawn" 0 "DONOTHANDLE" 0)) ; I need to spawn the actual building to get the model out of it.\nThis object will be deleted by the end of this function.
      ;[1 1 1] Set the return variables needed for the visuals
      (LocalVariables|SetreturnMesh (Variables|/Script/Engine.StaticMeshComponent|GetStaticMesh (Variables|/Game/WnSAssets/Blueprints/Actors/Intermediates/Lots/BP_Lot.BP_Lot_C|GetModel _returnvalue)))
      (LocalVariables|SetreturnScale (Variables|/Script/Engine.SceneComponent|GetRelativeScale3D (Variables|/Game/WnSAssets/Blueprints/Actors/Intermediates/Lots/BP_Lot.BP_Lot_C|GetModel _returnvalue)))
      (LocalVariables|SetreturnRotation (Variables|/Script/Engine.SceneComponent|GetRelativeRotation (Variables|/Game/WnSAssets/Blueprints/Actors/Intermediates/Lots/BP_Lot.BP_Lot_C|GetModel _returnvalue)))
      (LocalVariables|SetreturnLocation (Variables|/Script/Engine.SceneComponent|GetRelativeLocation (Variables|/Game/WnSAssets/Blueprints/Actors/Intermediates/Lots/BP_Lot.BP_Lot_C|GetModel _returnvalue)))
      (LocalVariables|SetreturnPlayerLabel (Variables|/Script/WarriorsAndSerfs.Lot|GetplayerLabel _returnvalue))
      (Variables|/Script/WarriorsAndSerfs.ConstructionComponent|SetmyLot (Variables|Default|GetConstruction) self)
      ;[1 1 1] Create Stockpiles with construction materials
      (bind _output_get (Variables|/Script/WarriorsAndSerfs.ConstructionComponent|SetconstructionRecipe (Variables|Default|GetConstruction) (Variables|/Game/WnSAssets/Blueprints/Actors/Intermediates/Lots/BP_Building.BP_Building_C|GetconstructionRecipe _returnvalue)))
      (for _array_element (.materials (Utilities|Struct|BreakConstructionRecipe _output_get))
        (Class|Lot|AddStockpile (.itemType (Utilities|Struct|BreakItemAmount _array_element)) "Educt" (.amount (Utilities|Struct|BreakItemAmount _array_element))))
      ;[1 1 1] Set Location of the "Door" (for pathfinding)
      (Transformation|SetWorldTransform (Variables|Default|GetDoor) (Transformation|GetWorldTransform (Variables|/Game/WnSAssets/Blueprints/Actors/Intermediates/Lots/BP_Lot.BP_Lot_C|GetDoor _returnvalue)) false false)
      ;[1 1 1] Set health
      (Variables|Default|SetmaxHealth (Variables|/Script/WarriorsAndSerfs.Lot|GetmaxHealth _returnvalue))
      (Variables|Default|SetcurrentHealth 1.0)
      (Class|Lot|DestroyLot _returnvalue)
      (return (LocalVariables|GetreturnMesh) (LocalVariables|GetreturnScale) (LocalVariables|GetreturnRotation) (LocalVariables|GetreturnLocation) (LocalVariables|GetreturnPlayerLabel)))))

(fn CompleteBuilding
  (Variables|Construction|SetconstructionComplete true)
  (Networking|SwitchHasAuthority
    (:Authority
      (bind _returnvalue (Game|SpawnActorfromClass (Variables|Construction|GetRealBuildingBP) (Transformation|GetWorldTransform (Variables|Default|GetDefaultSceneRoot)) "AlwaysSpawn" 0 (Variables|Default|GetowningPlayerName) 0))
      (Default|InitConstructionComplete _returnvalue (Utilities|Text|ToText(String) (Variables|Default|GetplayerLabel)) (Variables|Default|GetcurrentHealth) (Variables|HarvestingBuildingConstruction|GetharvestAreaLocation))
      ;[1 1 1] Finish off.
      ; open new UI if UI was open, then destroy the constructionsite.
      (Utilities|IsValid (Variables|Default|GetmyUI)
        (:Is%20Valid
          (Default|OpenUI _returnvalue (Variables|/Game/WnSAssets/Blueprints/UI/BP_UI.BP_UI_C|GetisOwnerUI (Variables|Default|GetmyUI))))
        (:Is%20Not%20Valid
          _))
      (Class|Lot|DestroyLot self))))

(fn SetBuildingMeshStartPosition
  (bind _model (Variables|Default|GetModel))
  (bind _returnvalue (Transformation|GetWorldLocation _model))
  (bind (_x _y _z) (Math|Vector|BreakVector _returnvalue))
  (bind _output_get (Variables|Construction|SetBuildingStartPos (Math|Vector|MakeVector _x _y (* 2 (- _z (.z (.BoxExtent (Collision|GetComponentBounds (Variables|Default|GetfinishedBuildingMesh))))))))))

(fn InitVisuals
  (params (mesh :type Static%20Mesh%20Object%20Reference) (scale :type Vector) (rotation :type Rotator) (location :type Vector) (playerLabel :type String))
  (bind _model (Variables|Default|GetModel))
  (bind _finishedbuildingmesh (Variables|Default|GetfinishedBuildingMesh))
  (bind _buildingicon (Variables|Default|GetbuildingIcon))
  (bind _returnvalue (Transformation|GetWorldLocation _buildingicon))
  (bind (_x _y _z) (Math|Vector|BreakVector _returnvalue))
  ;[1 1 1] Sets Mesh of the Ghostbuilding to that of the final building.
  ; SetScale, rotation and position are necessary in case the model is rotated, scaled or moved in the building BP viewport.
  ; This needs to be done for both the building mesh, and the ghost mesh.
  ;
  ; The location of the finished Building is however NOT set, as it should rise up from below.
  (Components|StaticMesh|SetStaticMesh _finishedbuildingmesh mesh)
  (Transformation|SetRelativeScale3D _finishedbuildingmesh scale)
  (Transformation|SetRelativeRotation _finishedbuildingmesh rotation false false)
  (Components|StaticMesh|SetStaticMesh _model mesh)
  (Transformation|SetRelativeScale3D _model scale)
  (Transformation|SetRelativeRotation _model rotation false false)
  (Transformation|SetRelativeLocation _model location false false)
  (CallFunction|SetBuildingMeshStartPosition) ; Set Start position of the mesh rising Up (just below ground)
  (CallFunction|SetPlayerLabel (Utilities|Text|ToText(String) playerLabel))
  (bind _astexture_2d (Utilities|Casting|CastToTexture2D (CallFunction|GetBuildingIconDT (Variables|Construction|GetRealBuildingType)))
    (:then
      (Rendering|Components|Sprite|SetSprite (Variables|Default|GetbuildingIcon) _astexture_2d)
      (if (Utilities|Name|Equal(Name) (Variables|Construction|GetRealBuildingType) "Palace")
        (Transformation|SetWorldLocation (Variables|Default|GetbuildingIcon) (Math|Vector|MakeVector _x _y (+ _z 2.2e+02)) false false))
      (Audio|PlaySoundatLocation "/Game/WnSAssets/Audio/Files/FX/placeBuilding.placeBuilding" (Transformation|GetWorldLocation (Variables|Default|GetDefaultSceneRoot)) "0, 0, 0" 1.0 1.0 0.0 0 0 0))
    (:CastFailed
      (Utilities|PrintStringRed15 "constructionsite initvisuals cast to texture2d failed!"))))

(fn UpdateConstructingVisuals
  (Transformation|SetWorldLocation (Variables|Default|GetfinishedBuildingMesh) (Math|Vector|Lerp(Vector) (Variables|Construction|GetBuildingStartPos) (Transformation|GetWorldLocation (Variables|Default|GetModel)) (Variables|/Script/WarriorsAndSerfs.ConstructionComponent|GetprogressPercent (Variables|Default|GetConstruction))) false false))

(fn InitHarvestingAreaMarker
  (bind _realbuildingbp (Variables|Construction|GetRealBuildingBP))
  (bind _output_get (Variables|HarvestingBuildingConstruction|SetharvestAreaLocation (Transformation|GetWorldLocation (Variables|Default|GetDoor))))
  (bind _returnvalue (Game|SpawnActorfromClass "/Game/WnSAssets/Blueprints/Actors/Final/BP_HarvestingAreaMarker.BP_HarvestingAreaMarker_C" (Math|Conversions|ToTransform(Vector) _output_get) "Undefined" 0 0))
  (bind _output_get_2 (Variables|HarvestingBuildingConstruction|SetharvestingAreaMarker _returnvalue))
  (bind _asbp_harvesting_building (Utilities|Casting|CastToBP_HarvestingBuildingClass _realbuildingbp)
    (:then
      (Variables|HarvestingBuildingConstruction|SetharvestAreaMaxDistFromDoor (.harvestAreaMaxDistFromDoor (Utilities|GetClassDefaults _asbp_harvesting_building)))
      (bind _output_get_3 (Variables|HarvestingBuildingConstruction|SetharvestAreaRadius (.harvestAreaRadius (Utilities|GetClassDefaults _asbp_harvesting_building))))
      (Default|SetRadius _output_get_2 _output_get_3)
      (HarvestingBuildingConstruction|ShowHarvestingAreaMarker false))
    (:CastFailed
      (Utilities|PrintStringRed15 "Construction site initharvestingarea cast to harvestbuilding class failed!"
        (:Exec
          (Utilities|PrintStringRed15 (Utilities|String|Append "Class is: " (Utilities|GetClassDisplayName _realbuildingbp))))))))

(fn ShowHarvestingAreaMarker
  (params (show :type Boolean))
  (if (Utilities|IsValidandNotNull (Variables|HarvestingBuildingConstruction|GetharvestingAreaMarker))
    (Rendering|SetActorHiddenInGame (Variables|HarvestingBuildingConstruction|GetharvestingAreaMarker) (not show))
    (Default|SetPosition (Variables|HarvestingBuildingConstruction|GetharvestingAreaMarker) (Variables|HarvestingBuildingConstruction|GetharvestAreaLocation))))

(fn CancelMoveHarvestingAreaMarker
  (Default|SetPosition (Variables|HarvestingBuildingConstruction|GetharvestingAreaMarker) (Variables|HarvestingBuildingConstruction|GetharvestAreaLocation))
  (if (Utilities|IsValidandNotNull (Variables|Default|GetmyUI))
    (Utilities|PrintStringRed15 "BP Construction building CancelMoveHarvestAreaLocation   UI is open when it shouldn't be!")
    (else
      (CallFunction|OpenUI true))))

(fn SetNewHarvestingAreaLocation
  (params (location :type Vector))
  (bind _output_get (Variables|HarvestingBuildingConstruction|SetharvestAreaLocation location))
  (Default|SetPosition (Variables|HarvestingBuildingConstruction|GetharvestingAreaMarker) _output_get)
  (if (not (Utilities|IsValidandNotNull (Variables|Default|GetmyUI)))
    (CallFunction|OpenUI true)))

(fn TryStartMoveHarvestingArea
  (bind _aswns_player (Utilities|Casting|CastToWnsPlayer (Pawn|GetControlledPawn (Game|GetPlayerController 0)))
    (:then
      (Default|TryStartMoveConstructionHarvestingArea _aswns_player self))
    (:CastFailed
      (Development|PrintString "Harvestingbuilding start mvoe harvesting area cast to wnsplayer failed!"))))

(fn SetNewHarvestingAreaLocationonServer
  (params (location :type Vector))
  (CallFunction|SetHarvestingAreaonServer location))

(fn StartMoveHarvestingArea
  (CallFunction|CloseUI)
  (HarvestingBuildingConstruction|ShowHarvestingAreaMarker true) ; Needs to be called after Close UI, \nas close UI also hides the marker!
)

(fn HandleBasic04
  (bind _realbuildingtype (Variables|Construction|GetRealBuildingType))
  (if (not (Variables|Tutorial|GetBasic04Completed))
    (bind _aswn_s_player_controller (Utilities|Casting|CastToWnS_PlayerController (Game|GetPlayerController 0))
      (:then
        (bind _output_get (LocalVariables|SettutManager (Variables|/Game/WnSAssets/Blueprints/Player/WnS_PlayerController.WnS_PlayerController_C|GettutorialManager _aswn_s_player_controller)))
        (bind _completed (Default|GetTutorialCompletionStatus _output_get "Basic04"))
        (if _completed ; Has the tutorial been completed alread?
          (Variables|Tutorial|SetBasic04Completed true)
          (else
            (Utilities|FlowControl|Sequence
              (:then_0
                ;[1 0 0] Sequence Then 0
                (if (Utilities|Name|Equal(Name) _realbuildingtype "Woodcutters") ; Is the placed constructionsite\na Woodcutter's?
                  (Variables|/Game/WnSAssets/Tutorial/TutorialManager.TutorialManager_C|SetBasic04WoodCutter (LocalVariables|GettutManager) true)
                  (elif (Utilities|Name|Equal(Name) _realbuildingtype "Sawmill") ; Is the placed constructionsite\na Sawmill?
                    (Variables|/Game/WnSAssets/Tutorial/TutorialManager.TutorialManager_C|SetBasic04Sawmill (LocalVariables|GettutManager) true))))
              (:then_1
                (if (and (Variables|/Game/WnSAssets/Tutorial/TutorialManager.TutorialManager_C|GetBasic04WoodCutter (LocalVariables|GettutManager)) (Variables|/Game/WnSAssets/Tutorial/TutorialManager.TutorialManager_C|GetBasic04Sawmill (LocalVariables|GettutManager))) ; Have all required buildings \nbeen placed?
                  (Default|CompleteTutorial (LocalVariables|GettutManager) "Basic04")))))))
      (:CastFailed
        (Utilities|PrintStringRed15 "Constructionsite HandleBasic04 cast to pc failed!")))))

(fn HandleBasic06
  (if (not (Variables|Tutorial|GetBasic06Completed))
    (bind _aswn_s_player_controller (Utilities|Casting|CastToWnS_PlayerController (Game|GetPlayerController 0))
      (:then
        (bind _output_get (LocalVariables|SettutManager (Variables|/Game/WnSAssets/Blueprints/Player/WnS_PlayerController.WnS_PlayerController_C|GettutorialManager _aswn_s_player_controller)))
        (bind _completed (Default|GetTutorialCompletionStatus _output_get "Basic06"))
        (if _completed ; Has the tutorial been completed alread?
          (Variables|Tutorial|SetBasic06Completed true)
          (else
            (Utilities|FlowControl|Sequence
              (:then_0
                ;[1 0 0] Sequence Then 0
                (if (Utilities|Name|Equal(Name) (Variables|Construction|GetRealBuildingType) "ForestingLodge") ; Is the placed constructionsite\na Foresting Lodge?
                  (Variables|/Game/WnSAssets/Tutorial/TutorialManager.TutorialManager_C|SetBasic06ForestingBuilt (LocalVariables|GettutManager) true)))
              (:then_1
                (if (Math|Boolean|ANDBoolean (Variables|/Game/WnSAssets/Tutorial/TutorialManager.TutorialManager_C|GetBasic06ForesterEdu (LocalVariables|GettutManager)) (Variables|/Game/WnSAssets/Tutorial/TutorialManager.TutorialManager_C|GetBasic06ForestingBuilt (LocalVariables|GettutManager)) (Variables|/Game/WnSAssets/Tutorial/TutorialManager.TutorialManager_C|GetBasic06HarvestAreaMoved (LocalVariables|GettutManager))) ; Have all components of \nthe tutorial been completed?
                  (Default|CompleteTutorial (LocalVariables|GettutManager) "Basic06")))))))
      (:CastFailed
        (Utilities|PrintStringRed15 "Constructionsite HandleBasic06 cast to pc failed!")))))

(fn HandleTutorials
  (Utilities|FlowControl|Sequence
    (:then_0
      (if (not (Variables|Tutorial|GetBasic04Completed))
        (Tutorial|HandleBasic04)))
    (:then_1
      (if (not (Variables|Tutorial|GetBasic06Completed))
        (Tutorial|HandleBasic06)))
    (:then_2
      (if (not (Variables|Tutorial|GetBasic07Completed))
        (Tutorial|HandleBasic07)))))

(fn HandleBasic07
  (bind _realbuildingtype (Variables|Construction|GetRealBuildingType))
  (if (not (Variables|Tutorial|GetBasic07Completed))
    (bind _aswn_s_player_controller (Utilities|Casting|CastToWnS_PlayerController (Game|GetPlayerController 0))
      (:then
        (bind _output_get (LocalVariables|SettutManager (Variables|/Game/WnSAssets/Blueprints/Player/WnS_PlayerController.WnS_PlayerController_C|GettutorialManager _aswn_s_player_controller)))
        (bind _completed (Default|GetTutorialCompletionStatus _output_get "Basic07"))
        (if _completed ; Has the tutorial been completed alread?
          (Variables|Tutorial|SetBasic07Completed true)
          (else
            (Utilities|FlowControl|Sequence
              (:then_0
                ;[1 0 0] Sequence Then 0
                (if (Utilities|Name|Equal(Name) _realbuildingtype "Farm") ; Is the placed constructionsite\na Farm?
                  (Variables|/Game/WnSAssets/Tutorial/TutorialManager.TutorialManager_C|SetBasic07Farm (LocalVariables|GettutManager) true)
                  (elif (Utilities|Name|Equal(Name) _realbuildingtype "Mill") ; Is the placed constructionsite\na Mill?
                    (Variables|/Game/WnSAssets/Tutorial/TutorialManager.TutorialManager_C|SetBasic07Mill (LocalVariables|GettutManager) true)
                    (elif (Utilities|Name|Equal(Name) _realbuildingtype "Bakery") ; Is the placed constructionsite\na Bakery?
                      (Variables|/Game/WnSAssets/Tutorial/TutorialManager.TutorialManager_C|SetBasic07Bakery (LocalVariables|GettutManager) true)))))
              (:then_1
                (if (Math|Boolean|ANDBoolean (Variables|/Game/WnSAssets/Tutorial/TutorialManager.TutorialManager_C|GetBasic07Farm (LocalVariables|GettutManager)) (Variables|/Game/WnSAssets/Tutorial/TutorialManager.TutorialManager_C|GetBasic07Mill (LocalVariables|GettutManager)) (Variables|/Game/WnSAssets/Tutorial/TutorialManager.TutorialManager_C|GetBasic07Bakery (LocalVariables|GettutManager))) ; Have all components of \nthe tutorial been completed?
                  (Default|CompleteTutorial (LocalVariables|GettutManager) "Basic07")))))))
      (:CastFailed
        (Utilities|PrintStringRed15 "Constructionsite HandleBasic07 cast to pc failed!")))))

(fn MakeLootBox
  (if (Utilities|Name|NotEqual(Name) (Variables|Default|GetowningPlayerName) "DONOTHANDLE")
    ;[1 1 1] Do not make lootbox from completing construction.
    (if (not (Variables|Construction|GetconstructionComplete))
      (bind _lootbox (|CallParentFunction))
      (Utilities|FlowControl|Sequence
        (:then_0
          (for _array_element (.materials (Utilities|Struct|BreakConstructionRecipe (Variables|/Script/WarriorsAndSerfs.ConstructionComponent|GetconstructionRecipe (Variables|Default|GetConstruction)))) ; Do for each itemtype in the recipe...
            ;[1 0 0] For Loop - Find how many items of this type have been "used up" in the construction
            (bind _returnvalue (Class|Lot|HasStockpile (.itemType (Utilities|Struct|BreakItemAmount _array_element))))
            (if _returnvalue ; Is there still a stockpile for this \nitem type?
              (bind _array_element_2 (Utilities|Array|ForEachLoopwithBreak (Variables|Default|Getstockpiles) :!label _label) ; find the stockpile for this item
                (:LoopBody
                  ;;[1 0.1902 0] For Loop (break) - find the stockpile
                  (if (Utilities|Name|Equal(Name) (Utilities|Struct|BreakStockpile _array_element_2) (.itemType (Utilities|Struct|BreakItemAmount _array_element)))
                    (goto _label Break)))
                (:Completed
                  (if (> (- (.amount (Utilities|Struct|BreakItemAmount _array_element)) (Utilities|Struct|BreakStockpile _array_element_2)) 0) ; Have any items of this type been used up yet?
                    ;;[1 1 1] Add those items to the used items
                    (Utilities|Array|Add (LocalVariables|GetusedItems) (Utilities|Struct|MakeItemAmount (.itemType (Utilities|Struct|BreakItemAmount _array_element)) (- (.amount (Utilities|Struct|BreakItemAmount _array_element)) (Utilities|Struct|BreakStockpile _array_element_2)))))))
              (else
                ;;[1 1 1] no stockpile for this item anymore = all used already
                (Utilities|Array|Add (LocalVariables|GetusedItems) _array_element))))
          (for _array_element_3 (LocalVariables|GetusedItems)
            ;[1 0 0] Foreach Loop - not all used up items are returned, only a percentage.
            (if (> (Math|Float|Round (* (.amount (Utilities|Struct|BreakItemAmount _array_element_3)) (CallFunction|BuildingResourceReturnFactor))) 0) ; Are there any resources to return?
              (Utilities|Array|Add (LocalVariables|GetstockpilesToAdd) (Utilities|Struct|MakeItemAmount (.itemType (Utilities|Struct|BreakItemAmount _array_element_3)) (Math|Float|Round (* (.amount (Utilities|Struct|BreakItemAmount _array_element_3)) (CallFunction|BuildingResourceReturnFactor)))))))
          (Default|AddStockpiles _lootbox (LocalVariables|GetstockpilesToAdd)))
        (:then_1
          (return _lootbox))))))

(fn BuilderHit
  (bind _returnvalue (Class|ConstructionComponent|Hit (Variables|Default|GetConstruction)))
  (if _returnvalue ; Did Successfully hit?
    (CallFunction|HitFeedback)
    (Utilities|FlowControl|Sequence
      (:then_0
        (if (>= (Variables|/Script/WarriorsAndSerfs.ConstructionComponent|GetcurrentHitsDone (Variables|Default|GetConstruction)) (Utilities|Struct|BreakConstructionRecipe (Variables|/Script/WarriorsAndSerfs.ConstructionComponent|GetconstructionRecipe (Variables|Default|GetConstruction)))) ; is the construction complete?
          (CallFunction|CompleteBuilding)))
      (:then_1
        (return true)))
    (else
      (return false))))

(fn HitFeedback
  (Audio|PlaySoundatLocation "/Game/WnSAssets/Audio/Files/Ambience/builderHit.builderHit" (Transformation|GetWorldLocation (Variables|Default|GetDefaultSceneRoot)) "0, 0, 0" 1.0 1.0 0.0 "/Game/WnSAssets/Audio/3D.3D" 0 0)
  (CallFunction|UpdateConstructingVisuals)
  (CallFunction|HitAddHealth)
  (CallFunction|UpdateUI "BuildProgress"))

(fn HitAddHealth
  (Class|Lot|TakeDamage (* (Variables|Default|GetmaxHealth) (/ 1.0 (Math|Conversions|ToFloat(Integer) (.builderHits (Utilities|Struct|BreakConstructionRecipe (Variables|/Script/WarriorsAndSerfs.ConstructionComponent|GetconstructionRecipe (Variables|Default|GetConstruction)))))) -1.0)))