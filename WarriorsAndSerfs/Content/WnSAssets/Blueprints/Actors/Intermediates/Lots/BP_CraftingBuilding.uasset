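; Intermediate lot Blueprint for buildings that craft recipes through a Crafting component.
; Construction sets the current recipe to the first entry in the building type's data table recipe list, and BeginPlay registers the lot with the component.
; Staff assignment and removal extend parent behavior to toggle the component's staffed flag.
; A helper starts a given recipe when crafting is idle and able, then plays a 3D crafting sound at the model.
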(event EventSetasMyStaff
  (params (Who? :type BP%20Housebased%20Object%20Reference))
  (|CallParentFunction Who?)
  (Variables|/Script/WarriorsAndSerfs.CraftingComponent|SetisStaffed (Variables|Default|GetCrafting) true))

(event EventRemoveMyStaff
  (|CallParentFunction)
  (Variables|/Script/WarriorsAndSerfs.CraftingComponent|SetisStaffed (Variables|Default|GetCrafting) false))

(event EventBeginPlay
  (|CallParentFunction)
  (Variables|/Script/WarriorsAndSerfs.CraftingComponent|SetmyLot (Variables|Default|GetCrafting) self))

(fn ConstructionScript
  (|CallParentFunction)
  (Variables|/Script/WarriorsAndSerfs.CraftingComponent|SetcurrentRecipe (Variables|Default|GetCrafting) (Utilities|Array|Get(acopy) (.craftingrecipelist (CallFunction|GetBuildingDT (Variables|Default|GetbuildingType))))))

(fn IfNotCraftingStartRecipe
  (params (craftingRecipe :type Crafting%20Recipe%20Structure))
  (bind _crafting (Variables|Default|GetCrafting))
  (if (not (Variables|/Script/WarriorsAndSerfs.CraftingComponent|Getworking _crafting))
    (bind _returnvalue (Class|CraftingComponent|CanStartRecipe _crafting craftingRecipe))
    (if _returnvalue
      (Class|CraftingComponent|StartRecipe _crafting craftingRecipe)
      (CallFunction|PlayCraftingSound)
      (return))))

(fn PlayCraftingSound
  (Audio|PlaySoundatLocation (Variables|BuildingSpecific|GetcraftingSound) (Transformation|GetWorldLocation (Variables|Default|GetModel)) "0, 0, 0" 1.0 1.0 0.0 "/Game/WnSAssets/Audio/3D.3D"))