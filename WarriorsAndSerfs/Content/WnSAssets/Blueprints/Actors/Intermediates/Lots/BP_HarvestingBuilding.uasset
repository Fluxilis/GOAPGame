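; Harvesting building lot with a movable circular harvest area, defaulting to the door location and shown by a spawned marker while the owner's UI is open.
; The player pawn handles moving the area; new locations apply locally, then go through the player controller for replication.
; The Harvesting component receives its products from the building data table.
; Free points in the area are found by spawning temporary collision testers at random navigable spots, avoiding lots and trees.
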(event Custom|SetHarvestingAreaOnServer
  (params (location :type Vector))
  ;[1 1 1] Replication - Set Harvesting Area
  (CallFunction|SetNewHarvestingAreaLocation location) ; Set locally first
  (bind _aswn_s_player_controller (Utilities|Casting|CastToWnS_PlayerController (Game|GetPlayerController 0)))
  (Default|SetHarvestingArea _aswn_s_player_controller self location))

(event Custom|NotifyClientsNewHarvestingArea
  (params (location :type Vector))
  ;[1 1 1] Replication - Set Harvesting Area
  (CallFunction|SetNewHarvestingAreaLocation location))

(event EventBeginPlay
  ;[1 1 1] Begin Play
  ; Init Harvest Area Marker and Set variable in component
  (|CallParentFunction)
  (Variables|/Script/WarriorsAndSerfs.HarvestingComponent|SetmyLot (Variables|Default|GetHarvesting) self)
  (CallFunction|InitHarvestingAreaMarker))

(event EventInitConstructionComplete
  (params (playerLabel :type Text) (currentHealth :type Float%20%28single-precision%29) (harvestAreaLocation :type Vector :default "0, 0, 0"))
  ;[1 1 1] Override InitConstructionComplete - Set HarvestAreaLocation (player may choose location during construction)
  (|CallParentFunction playerLabel currentHealth harvestAreaLocation)
  (Variables|Default|SetharvestAreaLocation harvestAreaLocation))

(event EventInitiateBuildingType
  (|CallParentFunction)
  (Variables|/Script/WarriorsAndSerfs.HarvestingComponent|SetharvestingProducts (Variables|Default|GetHarvesting) (.products (Utilities|Struct|BreakHarvestingRecipe (Utilities|Array|Get(acopy) (.harvestrecipelist (CallFunction|GetBuildingDT (Variables|Default|GetbuildingType))))))))

(event EventOpenUI
  (params (isOwnerUI :type Boolean))
  ;[1 1 1] Open UI
  ; Also show harvest area marker
  (|CallParentFunction isOwnerUI)
  (if isOwnerUI ; Only show for Owner of Building
    (CallFunction|ShowHarvestingAreaMarker true)))

(event EventCloseUI
  ;[1 1 1] Close UI
  ; Also Hide Harvest Area marker, and cancel moving harvesting area
  (CallFunction|ShowHarvestingAreaMarker false)
  (bind _aswns_player (Utilities|Casting|CastToWnsPlayer (Pawn|GetControlledPawn (Game|GetPlayerController 0)))
    (:then
      (Default|CancelMoveHarvestingArea _aswns_player)
      (|CallParentFunction))
    (:CastFailed
      (Development|PrintString "HarvestingBuiliding CloseUI Cast to wnsPlayer failed!"))))

(event EventDestroyed
  ;[1 1 1] Override Destroyed - Destroy area marker
  (Actor|DestroyActor (Variables|Default|GetharvestingAreaMarker))
  (|CallParentFunction))

(fn ConstructionScript
  (|CallParentFunction))

(fn InitHarvestingAreaMarker
  (if (Math|Vector|Equal(Vector) (Variables|Default|GetharvestAreaLocation) "0, 0, 0" 0.0001)
    (bind _output_get (Variables|Default|SetharvestAreaLocation (Transformation|GetWorldLocation (Variables|Default|GetDoor)))))
  (bind _returnvalue (Game|SpawnActorfromClass "/Game/WnSAssets/Blueprints/Actors/Final/BP_HarvestingAreaMarker.BP_HarvestingAreaMarker_C" (Math|Conversions|ToTransform(Vector) _output_get) "Undefined" 0 0))
  (bind _output_get_2 (Variables|Default|SetharvestingAreaMarker _returnvalue))
  (Default|SetRadius _output_get_2 (Variables|BuildingSpecific|GetharvestAreaRadius))
  (CallFunction|ShowHarvestingAreaMarker false))

(fn SetNewHarvestingAreaLocationonServer
  (params (location :type Vector))
  (CallFunction|SetHarvestingAreaonServer location))

(fn TryStartMoveHarvestingArea
  (bind _aswns_player (Utilities|Casting|CastToWnsPlayer (Pawn|GetControlledPawn (Game|GetPlayerController 0)))
    (:then
      (Default|TryStartMoveHarvestingArea _aswns_player self))
    (:CastFailed
      (Development|PrintString "Harvestingbuilding start mvoe harvesting area cast to wnsplayer failed!"))))

(fn IsinHarvestingArea
  (params (location :type Vector))
  (return (< (Utilities|VectorDistanceAbs location (Variables|Default|GetharvestAreaLocation)) (Variables|BuildingSpecific|GetharvestAreaRadius))))

(fn GetPointinHarvestingArea
  (bind _harvestarearadius (Variables|BuildingSpecific|GetharvestAreaRadius))
  (bind _harvestarealocation (Variables|Default|GetharvestAreaLocation))
  (bind _randomlocation (Class|NavigationSystem|GetRandomPointinNavigableRadius _harvestarealocation _harvestarearadius))
  (bind (_x _y) (Math|Vector|BreakVector _randomlocation))
  (bind _returnvalue (Math|Vector|MakeVector _x _y 0.0))
  (for _index (range 0 9) ; Try 10 times per frame
    (LocalVariables|SetreturnLocation _returnvalue)
    (bind _returnvalue_2 (Game|SpawnActorfromClass "/Game/WnSAssets/Blueprints/Actors/Helpers/BP_PlantTreeCollisionsTester.BP_PlantTreeCollisionsTester_C" (Math|Conversions|ToTransform(Vector) _returnvalue) "Undefined" 0 0))
    (if (and (<= (Utilities|Array|Length (Collision|GetOverlappingActors (Variables|/Game/WnSAssets/Blueprints/Actors/Helpers/BP_PlantTreeCollisionsTester.BP_PlantTreeCollisionsTester_C|GetStaticMesh _returnvalue_2) "/Script/WarriorsAndSerfs.Lot" :!class /Script/Engine.PrimitiveComponent)) 0) (<= (Utilities|Array|Length (Collision|GetOverlappingActors (Variables|/Game/WnSAssets/Blueprints/Actors/Helpers/BP_PlantTreeCollisionsTester.BP_PlantTreeCollisionsTester_C|GetStaticMesh _returnvalue_2) "/Game/WnSAssets/Blueprints/Actors/Final/Harvestable/BP_Tree.BP_Tree_C" :!class /Script/Engine.PrimitiveComponent)) 0))
      (Actor|DestroyActor _returnvalue_2)
      (return (LocalVariables|GetreturnLocation) true)
      (else
        (Actor|DestroyActor _returnvalue_2))))
  (return "0, 0, 0" false))

(fn ShowHarvestingAreaMarker
  (params (show :type Boolean))
  (if (Utilities|IsValidandNotNull (Variables|Default|GetharvestingAreaMarker))
    (Rendering|SetActorHiddenInGame (Variables|Default|GetharvestingAreaMarker) (not show))
    (Default|SetPosition (Variables|Default|GetharvestingAreaMarker) (Variables|Default|GetharvestAreaLocation))))

(fn CancelMoveHarvestingArea
  (Default|SetPosition (Variables|Default|GetharvestingAreaMarker) (Variables|Default|GetharvestAreaLocation))
  (if (Utilities|IsValidandNotNull (Variables|Default|GetmyUI))
    (Utilities|PrintStringRed15 "BP Harvesting building CancelMoveHarvestAreaLocation   UI is open when it shouldn't be!")
    (else
      (CallFunction|OpenUI true))))

(fn SetNewHarvestingAreaLocation
  (params (location :type Vector))
  (bind _output_get (Variables|Default|SetharvestAreaLocation location))
  (Default|SetPosition (Variables|Default|GetharvestingAreaMarker) _output_get)
  (if (not (Utilities|IsValidandNotNull (Variables|Default|GetmyUI)))
    (CallFunction|OpenUI true)))

(fn StartMoveHarvestingArea
  (CallFunction|CloseUI)
  (CallFunction|ShowHarvestingAreaMarker true) ; Needs to be called after Close UI, \nas close UI also hides the marker!
)