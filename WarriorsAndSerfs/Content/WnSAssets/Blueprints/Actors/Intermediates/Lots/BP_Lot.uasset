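; Base Blueprint for a player-owned lot (building) in a multiplayer strategy game.
; On authority it registers with its player's JobManager and the ActorManager, creating either if missing, then periodically makes jobs and raises their priorities.
; Clicking spawns an owner or non-owner UI actor; label changes and destruction requests route through the PlayerController.
; Destruction unregisters it and drops stockpile contents in a timed loot box, except for "DONOTHANDLE" placeholders and DeadDrop lots.
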(event Custom|UpdateUIOnClients
  (params (uiToUpdate :type Name))
  (UI|UpdateUI uiToUpdate))

(event Custom|SetPlayerLabelOnServer
  (params (newLabel :type Text))
  ;[1 1 1] Replication - Changing PlayerLabel through UI
  (CallFunction|SetPlayerLabel self newLabel) ; Set locally so there is instant feedback\nuntil the change from server comes back.
  (bind _aswn_s_player_controller (Utilities|Casting|CastToWnS_PlayerController (Game|GetPlayerController 0)))
  (Default|SetLotPlayerLabel _aswn_s_player_controller self newLabel))

(event Custom|NotifyClientsChangedPlayerLabel
  (params (newLabel :type Text))
  ;[1 1 1] Replication - Changing PlayerLabel through UI
  (CallFunction|SetPlayerLabel self newLabel))

(event Custom|DestroyOnServer
  ;[1 1 1] Replication - Destroying Lot (called from UI button)
  (bind _aswn_s_player_controller (Utilities|Casting|CastToWnS_PlayerController (Game|GetPlayerController 0)))
  (Default|DestroyLot _aswn_s_player_controller self)
  (CallFunction|NotifyClientsDestroyLot))

(event Custom|RemakeUIOnClients
  (UI|RemakeUI))

(event Custom|NotifyClientsDestroyLot
  ;[1 1 1] Replication - Destroying Lot (called from UI button)
  (CallFunction|DestroyLotonClient))

(event EventTick
  (params (DeltaSeconds :type Float%20%28single-precision%29))
  (Jobs|MakeJobAfterSeconds DeltaSeconds)
  (Jobs|HandleIncreaseJobPriorities))

(event EventBeginPlay
  (if (Utilities|Name|NotEqual(Name) (Variables|Default|GetowningPlayerName) "DONOTHANDLE")
    (Jobs|GetJobManagerandAddtoLots)
    (CallFunction|AddtoActorManager)))

(event EventUpdateActiveUI
  (params (uiToUpdate :type Name :default "None"))
  (UI|CallUpdateUIonClients uiToUpdate))

(event EventDestroyed
  ;[1 1 1] Destroyed Event
  (UI|CloseUI))

(event EventDestroyLot
  (CallFunction|HandleDestroyLot))

(fn ConstructionScript)

(fn GetDoorLocation
  (return (Transformation|GetWorldLocation (Variables|Default|GetDoor))))

(fn LookatCamera
  (params (Who%20looks? :type Scene%20Component%20Object%20Reference))
  (Transformation|SetWorldRotation Who%20looks? (Math|Rotator|FindLookatRotation (Transformation|GetWorldLocation Who%20looks?) (Transformation|GetWorldLocation (Variables|/Script/Engine.PlayerCameraManager|GetTransformComponent (Game|GetPlayerCameraManager 0)))) false false))

(fn GetJobManagerandAddtoLots
  (Networking|SwitchHasAuthority
    (:Authority
      (if (not (Utilities|IsValidandNotNull (Variables|Default|GetjobManager))) ; Do I already (NOT) have a JobManager?
        ;[1 1 1] Has my Player name been set?
        (bind _aswn_s_strategic_game_mode (Utilities|Casting|CastToWnS_StrategicGameMode (Game|GetGameMode))
          (:then
            (bind _isvalid (Default|IsValidPlayerName _aswn_s_strategic_game_mode (Variables|Default|GetowningPlayerName)))
            (if _isvalid
              (bind _outactors (Actor|GetAllActorswithTag "JobManager"))
              (if (> (Utilities|Array|Length _outactors) 0) ; Are there any jobmanagers?
                (for _array_element _outactors
                  ;[1 1 1] Check if any of the found Jobmanagers are the one for this player
                  (bind _asjob_manager (Utilities|Casting|CastToJobManager _array_element)
                    (:then
                      (if (Utilities|Name|Equal(Name) (Variables|/Script/WarriorsAndSerfs.JobManager|GetowningPlayerName _asjob_manager) (Variables|Default|GetowningPlayerName)) ; Is this the Jobmanager for my player?
                        ;;[1 1 1] Found the Job Manager. Add Lot, then RETURN (so loop doesn't continue)
                        (bind _output_get (Variables|Default|SetjobManager _asjob_manager))
                        (Class|JobManager|AddLot _output_get self)
                        (return)))
                    (:CastFailed
                      (Development|PrintString (Utilities|String|Append (Variables|Default|GetplayerLabel) "Lot GetJobManagerAddToLots Could Not cast to JobManager!!"))))))
              (bind _returnvalue (Game|SpawnActorfromClass "/Game/WnSAssets/Blueprints/Logics/Managers/BP_JobManager.BP_JobManager_C" (Math|Transform|MakeTransform "0, 0, 0") "AlwaysSpawn" 0 0)) ; If no JobManager was found for this player, create a new one!
              (Variables|/Script/WarriorsAndSerfs.JobManager|SetowningPlayerName _returnvalue (Variables|Default|GetowningPlayerName))
              (bind _output_get_2 (Variables|Default|SetjobManager _returnvalue))
              (Class|JobManager|AddLot _output_get_2 self)
              (elif (not (Utilities|Name|Equal(Name) (Variables|Default|GetowningPlayerName) "DONOTHANDLE"))
                (Development|PrintString (Utilities|String|Append "Owning Playername has not been set for " (Variables|Default|GetplayerLabel)) true true "(R=0.000000,G=0.660000,B=1.000000,A=1.000000)" 15.0))))
          (:CastFailed
            (Development|PrintString "Lot GetJobManager cast to gamemode failed!")))))))

(fn OpenUI
  (params (isOwnerUI :type Boolean))
  ;[1 1 1] Spawn and Cast to Widget, then spawn UI
  (if (not (Utilities|IsValid (Variables|UI|GetmyUI)))
    (bind _returnvalue (Game|SpawnActorfromClass "/Game/WnSAssets/Blueprints/UI/BP_LotUI.BP_LotUI_C" (Transformation|GetWorldTransform (Variables|Default|GetUISpawnPoint)) "AlwaysSpawn" 0 0))
    (Variables|UI|SetmyUI _returnvalue)
    (Variables|/Game/WnSAssets/Blueprints/UI/BP_UI.BP_UI_C|SetmyActor _returnvalue self)
    (Default|OpenUI _returnvalue isOwnerUI)))

(fn SetPlayerLabel
  (params (newLabel :type Text))
  (Variables|Default|SetplayerLabel (Utilities|String|ToString(Text) newLabel))
  (UI|UpdateUI "Labels"))

(fn CallUpdateUIonClients
  (params (uiToUpdate :type Name))
  (CallFunction|UpdateUIonClients uiToUpdate))

(fn GetLotWidget
  (bind _asw_lot (Utilities|Casting|CastToW_Lot (UserInterface|GetUserWidgetObject (Variables|/Game/WnSAssets/Blueprints/UI/BP_UI.BP_UI_C|GetUIWidget (Variables|UI|GetmyUI))))
    (:then
      (return _asw_lot))
    (:CastFailed
      (Development|PrintString (Utilities|String|Append "BP_Lot::GetLotWidget Failed! In:" (Variables|Default|GetplayerLabel))))))

(fn Clicked
  (params (clickingPlayer :type Name))
  (if (Utilities|Name|Equal(Name) clickingPlayer (Variables|Default|GetowningPlayerName))
    (UI|OpenUI true)
    (else
      (UI|OpenUI false))))

(fn HandleDestroyLot
  (bind _self self)
  (bind _jobmanager (Variables|Default|GetjobManager))
  (if (Utilities|Name|NotEqual(Name) (Variables|Default|GetowningPlayerName) "DONOTHANDLE")
    (if (Utilities|IsValidandNotNull _jobmanager)
      ;[1 1 1] Remove from JobManager
      (Class|JobManager|RemoveLot _jobmanager _self)
      (Class|JobManager|RemoveJobs _jobmanager _self))
    (CallFunction|RemovefromActorManager)
    (UI|CloseUI)
    (CallFunction|MakeLootBox)
    (Actor|DestroyActor)
    (else
      (Actor|DestroyActor))))

(fn CloseUI
  (bind _myui (Variables|UI|GetmyUI))
  (Utilities|IsValid _myui
    (:Is%20Valid
      (Actor|DestroyActor _myui))))

(fn SetLotType
  (params (newLabel :type ELotType%20Enum :default "MissingNo"))
  (Variables|Default|SetlotType newLabel)
  (UI|CallUpdateUIonClients "None"))

(fn RemovefromActorManager
  (Default|RemoveLot (Variables|Default|GetactorManager) self))

(fn AddtoActorManager
  (Utilities|FlowControl|Sequence
    (:then_0
      (Networking|SwitchHasAuthority
        (:Authority
          (bind _outactors (Actor|GetAllActorswithTag "ActorManager"))
          (if (> (Utilities|Array|Length _outactors) 0)
            (for _array_element _outactors
              (bind _asbp_actor_manager (Utilities|Casting|CastToBP_ActorManager _array_element)
                (:then
                  (Variables|Default|SetactorManager _asbp_actor_manager))
                (:CastFailed
                  (Development|PrintString (Utilities|String|Append (Variables|Default|GetplayerLabel) " Could Not cast to LotManager!!")))))
            (else
              (bind _returnvalue (Game|SpawnActorfromClass "/Game/WnSAssets/Blueprints/Logics/Managers/BP_ActorManager.BP_ActorManager_C" (Math|Transform|MakeTransform "0, 0, 0") "AlwaysSpawn" 0 0)) ; If no LotManager was found, create a new one!
              (Variables|Default|SetactorManager _returnvalue))))))
    (:then_1
      (Default|AddLot (Variables|Default|GetactorManager) self))))

(fn MakeJobAfterSeconds
  (params (DeltaTime :type Float%20%28single-precision%29))
  (Networking|SwitchHasAuthority
    (:Authority
      (bind _output_get (Variables|Jobs|SetcurrentDelay (+ DeltaTime (Variables|Jobs|GetcurrentDelay))))
      (if (> _output_get (Variables|Jobs|GetmakeJobDelay))
        (Variables|Jobs|SetcurrentDelay 0.0)
        (Class|Lot|MakeJob (Variables|Default|GetjobManager))))))

(fn UpdateUI
  (params (uiToUpdate :type Name))
  (bind _myui (Variables|UI|GetmyUI))
  (Utilities|IsValid _myui
    (:Is%20Valid
      (Default|UpdateUI _myui uiToUpdate))))

(fn RemakeUI
  (bind _myui (Variables|UI|GetmyUI))
  (Utilities|IsValid _myui
    (:Is%20Valid
      (Default|RemakeUI _myui))))

(fn CallRemakeUIonClients
  (CallFunction|RemakeUIonClients))

(fn DestroyLotonClient
  (Audio|SpawnSoundatLocation "/Game/WnSAssets/Audio/Files/FX/destroyBuilding.destroyBuilding" (Transformation|GetWorldLocation (Variables|Default|GetDefaultSceneRoot)) "0, 0, 0" 1.0 1.0 0.0 0 0))

(fn MakeLootBox
  (if (not (or (Utilities|Enum|Equal(Enum) (Variables|Default|GetlotType) "DeadDrop") (Utilities|Name|Equal(Name) (Variables|Default|GetowningPlayerName) "DONOTHANDLE"))) ; Under some conditions, \ndo not make a loot box.
    (Utilities|FlowControl|Sequence
      (:then_0
        (bind _returnvalue (Game|SpawnActorfromClass "/Game/WnSAssets/Blueprints/Actors/Final/LootBox.LootBox_C" (Transformation|GetWorldTransform (Variables|Default|GetDefaultSceneRoot)) "AlwaysSpawn" 0 (Variables|Default|GetowningPlayerName) 0))
        (LocalVariables|SetnewLootBox _returnvalue)
        (for _array_element (Variables|Default|Getstockpiles)
          ;[1 0 0] Foreach Loop - Create an array of itemAmounts with the CurrentStored Contents of all stockpiles
          (Utilities|Array|Add (LocalVariables|GetstockpilesContent) (Utilities|Struct|MakeItemAmount (.itemType (Utilities|Struct|BreakStockpile _array_element)) (.currentStored (Utilities|Struct|BreakStockpile _array_element)))))
        (Default|AddStockpiles (LocalVariables|GetnewLootBox) (LocalVariables|GetstockpilesContent))
        (Default|InitLifetime (LocalVariables|GetnewLootBox) 9e+01))
      (:then_1
        (return (LocalVariables|GetnewLootBox))))))

(fn HandleIncreaseJobPriorities
  (if (> (Utilities|Time|GetGameTimeinSeconds) (+ (Variables|Jobs|GetlastIncreaseJobPrioritiesTime) 1.0))
    (Class|Lot|IncreaseJobPriorities (CallFunction|JobPriorityIncreasePerSecond))
    (Variables|Jobs|SetlastIncreaseJobPrioritiesTime (Utilities|Time|GetGameTimeinSeconds))))