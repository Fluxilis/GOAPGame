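; Building lot actor that holds a building's type, assigned worker, health and construction recipe.
; BuildingType drives data-table lookups for stats, jobs, stockpiles and overhead icon, run from both construction script and BeginPlay.
; Tick polls a timestamp to send one delayed missing-worker notification, also informing the TutorialManager.
; Destruction clears the worker's home, and loot boxes receive a factored share of construction materials unless the owner name is DONOTHANDLE.
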(event EventTick
  (params (DeltaSeconds :type Float%20%28single-precision%29))
  ;[1 1 1] Event Tick
  (|CallParentFunction DeltaSeconds)
  (Staff|CheckforStaffMissingNotification))

(event EventHandleDestroyLot
  ;[1 1 1] Destroy Lot Handle Destroy Building
  (CallFunction|HandleDestroyBuilding)
  (|CallParentFunction))

(event EventBeginPlay
  ;[1 1 1] Begin Play
  (|CallParentFunction)
  (CallFunction|InitiateBuildingType))

(fn ConstructionScript
  (|CallParentFunction)
  (CallFunction|InitiateBuildingType))

(fn GetMesh
  (return (Variables|/Script/Engine.StaticMeshComponent|GetStaticMesh (Variables|Default|GetModel))))

(fn RemoveMyStaff
  (Variables|Staff|SetMyStaff 0)
  ;[1 1 1] Remake UI
  (if (Utilities|IsValidandNotNull (Variables|Default|GetmyUI))
    (Default|RemakeUI (Variables|Default|GetmyUI)))
  (Staff|StartMissingStaffTimer))

(fn SetasMyStaff
  (params (Who? :type BP%20Housebased%20Object%20Reference))
  (Variables|Staff|SetMyStaff Who?)
  (CallFunction|CallRemakeUIonClients))

(fn HandleDestroyBuilding
  (if (Utilities|IsValidandNotNull (Variables|Staff|GetMyStaff))
    (Default|RemoveHome (Variables|Staff|GetMyStaff))))

(fn InitConstructionComplete
  (params (playerLabel :type Text) (currentHealth :type Float%20%28single-precision%29) (harvestAreaLocation :type Vector))
  (CallFunction|SetPlayerLabelonServer playerLabel) ; needed to replicate
  (Variables|Default|SetcurrentHealth currentHealth)
  (CallFunction|GetJobManagerandAddtoLots))

(fn StartMissingStaffTimer
  ;[1 1 1] Check for missing Staff and start timer
  (if (Utilities|Name|NotEqual(Name) (Variables|BuildingSpecific|GetwhoWorksHere) "None") ; Does this building require a worker?
    (if (not (Utilities|IsValidandNotNull (Variables|Staff|GetMyStaff))) ; Is this building missing its worker?
      (Variables|Staff|SetmissingStaffStartTime (Utilities|Time|GetGameTimeinSeconds))
      (Variables|Staff|SetsentMissingStaffNotification false))))

(fn CheckforStaffMissingNotification
  ;[1 1 1] Notify Player that building is missing worker.
  (if (not (Variables|Staff|GetsentMissingStaffNotification)) ; Has the notification been sent already?
    (if (Utilities|Name|NotEqual(Name) (Variables|BuildingSpecific|GetwhoWorksHere) "None") ; Does this building require a worker?
      (if (not (Utilities|IsValidandNotNull (Variables|Staff|GetMyStaff))) ; Is this building missing its worker?
        (if (< (+ (Variables|Staff|GetmissingStaffStartTime) (Variables|Staff|GetmissingStaffNotificationDelay)) (Utilities|Time|GetGameTimeinSeconds)) ; has the building been missing \nits worker for the specified duration?
          (bind _aswn_s_player_controller (Utilities|Casting|CastToWnS_PlayerController (Game|GetPlayerController 0))
            (:then
              (bind _w_hud (Default|GetWHud _aswn_s_player_controller))
              (Default|MakeNotification _w_hud (Utilities|Text|FormatText "This {BuildingType} is missing its worker, a {workerType}." (CallFunction|GetBuildingDisplayNameDT (Variables|BuildingSpecific|GetbuildingType)) (CallFunction|GetSubjectDisplayNameDT (Variables|BuildingSpecific|GetwhoWorksHere))) "/Game/WnSAssets/Visual/Icons/Notifications/newsIcon.newsIcon" "0, 0, 0" self)
              (Variables|Staff|SetsentMissingStaffNotification true)
              ;[1 1 1] Tell TutorialManager that an unoccupied notification was made.
              (bind _aswn_s_player_controller_2 (Utilities|Casting|CastToWnS_PlayerController (Game|GetPlayerController 0))
                (:then
                  (Default|UnoccupiedNotifWasSent (Variables|/Game/WnSAssets/Blueprints/Player/WnS_PlayerController.WnS_PlayerController_C|GettutorialManager _aswn_s_player_controller_2)))
                (:CastFailed
                  (Utilities|PrintStringRed15 "Building Check for missing staff notif cast to pc failed"))))
            (:CastFailed
              (Utilities|PrintStringRed15 "subject handle die cast to pc failed!"))))))))

(fn MakeLootBox
  (if (Utilities|Name|NotEqual(Name) (Variables|Default|GetowningPlayerName) "DONOTHANDLE")
    (bind _lootbox (|CallParentFunction))
    (Utilities|FlowControl|Sequence
      (:then_0
        (for _array_element (.materials (Variables|BuildingSpecific|GetconstructionRecipe))
          ;[1 0 0] Foreach Loop
          (if (> (Math|Float|Round (* (.amount (Utilities|Struct|BreakItemAmount _array_element)) (CallFunction|BuildingResourceReturnFactor))) 0) ; Would at least one item of this type be returned?
            (Utilities|Array|Add (LocalVariables|GetstockpilesToAdd) (Utilities|Struct|MakeItemAmount (.itemType (Utilities|Struct|BreakItemAmount _array_element)) (Math|Float|Round (* (.amount (Utilities|Struct|BreakItemAmount _array_element)) (CallFunction|BuildingResourceReturnFactor)))))))
        (Default|AddStockpiles _lootbox (LocalVariables|GetstockpilesToAdd)))
      (:then_1
        (return _lootbox)))))

(fn SetOverheadIcon
  ;[1 1 1] Set Overhead Icon (Temporary)
  (bind _astexture_2d (Utilities|Casting|CastToTexture2D (CallFunction|GetBuildingIconfromNameDT (Variables|BuildingSpecific|GetbuildingType)))
    (:then
      (Rendering|Components|Sprite|SetSprite (Variables|Default|GetbuildingIcon%28Temp%29) _astexture_2d)
      (Development|SetHiddeninGame (Variables|Default|GetbuildingIcon%28Temp%29) false false))
    (:CastFailed
      (Utilities|PrintStringRed15 "building begin player cast to texture2d failed!"))))

(fn InitiateBuildingType
  (bind _buildingtype (Variables|BuildingSpecific|GetbuildingType))
  (bind _dtsbuilding (CallFunction|GetBuildingDT _buildingtype))
  (bind (_displayname _maxhealth _whoworkshere _pulljoblimit _pushjoblimit _constructionrecipe _stockpiles) (Utilities|Struct|BreakDTS_Building _dtsbuilding))
  (Variables|Default|SetplayerLabel (Utilities|String|ToString(Text) _displayname))
  (bind _output_get (Variables|Default|SetmaxHealth _maxhealth))
  (Variables|Default|SetcurrentHealth _output_get)
  (Variables|BuildingSpecific|SetwhoWorksHere _whoworkshere)
  (Variables|Default|SetpullJobLimit (Math|Conversions|ToFloat(Integer) _pulljoblimit))
  (Variables|Default|SetpushJobLimit (Math|Conversions|ToFloat(Integer) _pushjoblimit))
  (Variables|BuildingSpecific|SetconstructionRecipe _constructionrecipe)
  (Variables|Default|Setstockpiles _stockpiles)
  (CallFunction|SetOverheadIcon)
  (Staff|StartMissingStaffTimer))