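; BP_Subject is the base Blueprint for citizens, initializing health, education cost and overhead icon from occupation data, with job descriptions left to child overrides.
; On authority it registers with a found or spawned BP_ActorManager.
; Clicking opens an owner or non-owner W_Subject widget through the HUD; label, job and kill requests route through WnS_PlayerController, with notify events updating clients.
; Death posts a HUD notification, then authority notifies clients, unregisters and destroys the actor.
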(event Custom|RemakeUIOnClients
  ;[1 1 1] Replication - Updates UI for all clients (NOT NEEDED!?)
  (UI|RemakeUI))

(event Custom|SetPlayerLabelOnServer
  (params (newLabel :type Text))
  ;[1 1 1] Replication - Changing PlayerLabel through UI
  (CallFunction|SetPlayerLabel self newLabel) ; Set locally so there is instant feedback\nuntil the change from server comes back.
  (bind _aswn_s_player_controller (Utilities|Casting|CastToWnS_PlayerController (Game|GetPlayerController 0)))
  (Default|SetSubjectPlayerLabel _aswn_s_player_controller self newLabel))

(event Custom|UpdateJobDescriptionOnServer
  ;[1 1 1] Replication - Updating Job description
  (bind _aswn_s_player_controller (Utilities|Casting|CastToWnS_PlayerController (Game|GetPlayerController 0)))
  (Default|UpdateJobDescription _aswn_s_player_controller self))

(event Custom|NotifyClientsUpdatedJobDescription
  (params (jobDescription :type Text))
  ;[1 1 1] Replication - Updating Job description
  (Variables|Job|SetCurrentJobDescription jobDescription)
  (UI|UpdateUI "Job"))

(event Custom|NotifyClientsChangedPlayerLabel
  (params (newLabel :type Text))
  ;[1 1 1] Replication - Changing PlayerLabel through UI
  (CallFunction|SetPlayerLabel self newLabel))

(event Custom|UpdateUIOnClients
  (params (uiToUpdate :type Name))
  ;[1 1 1] Replication - Updates UI for all clients (NOT NEEDED!?)
  (UI|UpdateUI uiToUpdate))

(event Custom|DestroyOnServer
  ;[1 1 1] Replication - Destroying Subject
  (UI|CloseUI)
  (bind _aswn_s_player_controller (Utilities|Casting|CastToWnS_PlayerController (Game|GetPlayerController 0)))
  (Default|KillSubject _aswn_s_player_controller self))

(event Custom|NotifyClientsHandleSubjectDie
  ;[1 1 1] Replication - Destroying Subject
  (CallFunction|SubjectHandleDieonClient))

(event EventBeginPlay
  (|CallParentFunction)
  (CallFunction|InitiateSubjectType)
  (Networking|SwitchHasAuthority
    (:Authority
      ;[1 0 0] SWITCH
      (CallFunction|AddtoActorManager))))

(event EventSubjectDie
  ;[1 1 1] Subject Die
  (CallFunction|SubjectHandleDie)
  (|CallParentFunction))

(event EventUpdateActiveUI
  (params (uiToUpdate :type Name :default "None"))
  ;[1 1 1] This event is called from C++
  ; updates UI on clients
  (CallFunction|UpdateUIonClients uiToUpdate))

(fn ConstructionScript
  (|CallParentFunction)
  (Variables|Default|SetowningPlayerName "wnsplayer0")
  (CallFunction|InitiateSubjectType))

(fn Clicked
  (params (clickingPlayer :type Name))
  (if (Utilities|Name|Equal(Name) clickingPlayer (Variables|Default|GetowningPlayerName))
    (UI|OpenUI true)
    (else
      (UI|OpenUI false))))

(fn OpenUI
  (params (isOwnerUI :type Boolean))
  (bind _self self)
  (Utilities|IsValid (Variables|Default|GetmyUI) ; Already open?
    (:Is%20Not%20Valid
      (bind _returnvalue (UserInterface|CreateWidget "/Game/WnSAssets/Widgets/Gameplay/ActorUI/Subjects/W_Subject.W_Subject_C" 0 0 _self isOwnerUI _self))
      (Variables|Default|SetmyUI _returnvalue)
      (bind _aswn_s_player_controller (Utilities|Casting|CastToWnS_PlayerController (Game|GetPlayerController 0))
        (:then
          (bind _w_hud (Default|GetWHud _aswn_s_player_controller))
          (Default|AddActorUI _w_hud _returnvalue))
        (:CastFailed
          (Utilities|PrintStringRed15 "subject openUi cast to pc failed"))))))

(fn CallUpdateUIonClients
  (CallFunction|UpdateUIonClients "None"))

(fn CloseUI
  (Utilities|IsValid (Variables|Default|GetmyUI)
    (:Is%20Valid
      (Widget|RemovefromParent (Variables|Default|GetmyUI))
      (Variables|Default|SetmyUI 0))))

(fn AddtoActorManager
  (Utilities|FlowControl|Sequence
    (:then_0
      (bind _outactors (Actor|GetAllActorswithTag "ActorManager"))
      (if (> (Utilities|Array|Length _outactors) 0)
        (for _array_element _outactors
          (bind _asbp_actor_manager (Utilities|Casting|CastToBP_ActorManager _array_element)
            (:then
              (Variables|Default|SetactorManager _asbp_actor_manager))
            (:CastFailed
              (Development|PrintString (Utilities|String|Append (Variables|Default|GetplayerLabel) " Could Not cast to ActorManager!!")))))
        (else
          (bind _returnvalue (Game|SpawnActorfromClass "/Game/WnSAssets/Blueprints/Logics/Managers/BP_ActorManager.BP_ActorManager_C" (Math|Transform|MakeTransform "0, 0, 0") "AlwaysSpawn" 0 0)) ; If no LotManager was found, create a new one!
          (Variables|Default|SetactorManager _returnvalue))))
    (:then_1
      (Default|AddSubject (Variables|Default|GetactorManager) self))))

(fn SubjectHandleDie
  ;[1 1 1] Notify player subject Died
  ;;[1 1 1] Find Deathcause
  (if (<= (Variables|Default|GetcurrentFood) 0.0)
    (LocalVariables|SetdeathcauseText " of Hunger"))
  (bind _aswn_s_player_controller (Utilities|Casting|CastToWnS_PlayerController (Game|GetPlayerController 0))
    (:then
      (bind _w_hud (Default|GetWHud _aswn_s_player_controller))
      (Default|MakeNotification _w_hud (Utilities|Text|FormatText "{PlayerLabel}, one of your citizens with Job {SubjectType} died{Deathcause}." (Utilities|Text|ToText(String) (Variables|Default|GetplayerLabel)) (CallFunction|GetSubjectDisplayNameDT (Variables|Default|GetsubjectOccupation)) (LocalVariables|GetdeathcauseText)) "/Game/WnSAssets/Visual/Icons/Notifications/deadIcon.deadIcon" (Transformation|GetWorldLocation (Variables|Default|GetCapsuleComponent)))
      (Networking|SwitchHasAuthority
        (:Authority
          (UI|CloseUI)
          (CallFunction|NotifyClientsHandleSubjectDie)
          (CallFunction|RemovefromActorManager)
          (Actor|DestroyActor))))
    (:CastFailed
      (Utilities|PrintStringRed15 "subject handle die cast to pc failed!"))))

(fn UpdateCurrentJobDescription
  (Variables|Job|SetCurrentJobDescription "MISSING SUBJECT JOB OVERRIDE!")
  (UI|UpdateUI "Job"))

(fn UpdateUI
  (params (uiToUpdate :type Name))
  (Utilities|IsValid (Variables|Default|GetmyUI)
    (:Is%20Valid
      (Default|UpdateUI (Variables|Default|GetmyUI) uiToUpdate))))

(fn SetPlayerLabel
  (params (newLabel :type Text))
  (Variables|Default|SetplayerLabel (Utilities|String|ToString(Text) newLabel))
  (UI|UpdateUI "Labels"))

(fn CallRemakeUIonClients
  (CallFunction|RemakeUIonClients))

(fn RemakeUI
  (bind _mysubjectui (Variables|Default|GetmySubjectUI))
  (Utilities|IsValid _mysubjectui
    (:Is%20Valid
      (Default|RemakeUI _mysubjectui))))

(fn SubjectHandleDieonClient
  (Audio|SpawnSoundatLocation "/Game/WnSAssets/Audio/Files/FX/death1.death1" (Transformation|GetWorldLocation (Variables|Default|GetCapsuleComponent)) "0, 0, 0" 1.0 1.0 0.0 0 0)
  (UI|CloseUI))

(fn RemovefromActorManager
  (Default|RemoveSubject (Variables|Default|GetactorManager) self))

(fn InitiateSubjectType
  (bind _subjectoccupation (Variables|Default|GetsubjectOccupation))
  (bind _dtssubject (CallFunction|GetSubjectDT _subjectoccupation))
  (bind (_subjectname _maxhealth _educatecost) (Utilities|Struct|BreakDTS_Subject _dtssubject))
  (bind _output_get (Variables|Default|SetmaxHealth _maxhealth))
  (Variables|Default|SetcurrentHealth _output_get)
  (CallFunction|UpdateOverheadIcon)
  (Variables|Default|SetsubjectEducateCost _educatecost))

(fn UpdateOverheadIcon
  ;[1 1 1] Set Overhead Icon (Temporary)
  (bind _astexture_2d (Utilities|Casting|CastToTexture2D (CallFunction|GetSubjectIconDT (Variables|Default|GetsubjectOccupation)))
    (:then
      (Rendering|Components|Sprite|SetSprite (Variables|Components|GetSubjectIcon%20%28Temp%29) _astexture_2d)
      (Development|SetHiddeninGame (Variables|Components|GetSubjectIcon%20%28Temp%29) false false))
    (:CastFailed
      (Utilities|PrintStringRed15 "subject begin play cast to texture2d failed!"))))