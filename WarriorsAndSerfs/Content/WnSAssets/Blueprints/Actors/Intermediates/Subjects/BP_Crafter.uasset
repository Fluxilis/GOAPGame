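; BP_Crafter is a subject worker that crafts recipes at its home crafting building and rests between jobs.
; A None, Crafting, Resting job status gates work readiness and sets wait times from recipe craft duration or rest duration.
; Recipe checks and completion go to the building's Crafting member through casts.
; Status changes and home removal trigger a server job description update, with home removal also rebuilding the subject UI.
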(event EventUpdateCurrentJobDescription
  ;[1 1 1] Override - Update Job Description
  (if (Variables|Default|GetgoingHome)
    (Variables|Default|SetCurrentJobDescription "Currently going home.")
    (elif (Variables|Default|GetgoingToEat)
      (Variables|Default|SetCurrentJobDescription "Currently going to eat.")
      (else
        (Variables|Default|SetCurrentJobDescription (Utilities|Text|ToText(String) (Utilities|String|Append "Currently " (Class|Globals|GetCraftingJobType (Variables|Job|GetcurrentJobStatus)) ".")))))))

(event EventRemoveHome
  ;[1 1 1] Override Remove Home
  (CallFunction|HarvesterRemoveHome))

(fn ConstructionScript
  (|CallParentFunction))

(fn HomeCanCraft
  (bind _asbp_crafting_building (Utilities|Casting|CastToBP_CraftingBuilding (Variables|Default|GetHomeBuilding))
    (:then
      (bind _returnvalue (Class|CraftingComponent|CanStartRecipe (Variables|/Game/WnSAssets/Blueprints/Actors/Intermediates/Lots/BP_CraftingBuilding.BP_CraftingBuilding_C|GetCrafting _asbp_crafting_building) (Variables|/Script/WarriorsAndSerfs.CraftingComponent|GetcurrentRecipe (Variables|/Game/WnSAssets/Blueprints/Actors/Intermediates/Lots/BP_CraftingBuilding.BP_CraftingBuilding_C|GetCrafting _asbp_crafting_building))))
      (return _returnvalue))
    (:CastFailed
      (Development|PrintString "Crafter CanCraft Cast Failed!")
      (return false))))

(fn IsReadytoWork
  (bind _isready_ (|CallParentFunction))
  (return (and _isready_ (Utilities|Enum|Equal(Enum) (Variables|Job|GetcurrentJobStatus) "None"))))

(fn CompleteCrafting
  (bind _asbp_crafting_building (Utilities|Casting|CastToBP_CraftingBuilding (Variables|Default|GetHomeBuilding))
    (:then
      (Class|CraftingComponent|RecipeDone (Variables|/Game/WnSAssets/Blueprints/Actors/Intermediates/Lots/BP_CraftingBuilding.BP_CraftingBuilding_C|GetCrafting _asbp_crafting_building))
      (CallFunction|SetJobStatus "Resting")
      (return true))
    (:CastFailed
      (Development|PrintString "Crafter CompleteCrafting Cast failed!")
      (return false))))

(fn CompleteResting
  (CallFunction|SetJobStatus "None")
  (return true))

(fn GetCurrentJobWaitTime
  (switch Utilities|FlowControl|Switch|SwitchonECraftingJobType (Variables|Job|GetcurrentJobStatus)
    (:None
      (return 0.0))
    (:Crafting
      (bind _asbp_crafting_building (Utilities|Casting|CastToBP_CraftingBuilding (Variables|Default|GetHomeBuilding)))
      (LocalVariables|SetthisJobWaitTime (.craftduration (Variables|/Script/WarriorsAndSerfs.CraftingComponent|GetcurrentRecipe (Variables|/Game/WnSAssets/Blueprints/Actors/Intermediates/Lots/BP_CraftingBuilding.BP_CraftingBuilding_C|GetCrafting _asbp_crafting_building)))))
    (:Resting
      (LocalVariables|SetthisJobWaitTime (Variables|Job|GetrestDuration))))
  (return (LocalVariables|GetthisJobWaitTime)))

(fn GetCurrentJobDescription
  (if (Variables|Default|GetgoingToEat)
    (Variables|Default|SetCurrentJobDescription "Currently going to eat.")
    (else
      (Variables|Default|SetCurrentJobDescription (Utilities|Text|ToText(String) (Utilities|String|Append "Currently " (Class|Globals|GetCraftingJobType (Variables|Job|GetcurrentJobStatus)) "."))))))

(fn SetJobStatus
  (params (currentJobStatus :type ECraftingJobType%20Enum :default "None"))
  (Variables|Job|SetcurrentJobStatus currentJobStatus)
  (CallFunction|UpdateJobDescriptiononServer))

(fn HarvesterRemoveHome
  (Variables|Job|SetcurrentJobStatus "None")
  (CallFunction|UpdateJobDescriptiononServer)
  (if (Utilities|IsValidandNotNull (Variables|Default|GetmySubjectUI))
    (Default|RemakeUI (Variables|Default|GetmySubjectUI))))