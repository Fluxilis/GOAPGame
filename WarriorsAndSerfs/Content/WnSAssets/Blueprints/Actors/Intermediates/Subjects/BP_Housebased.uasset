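; BP_Housebased is an intermediate subject Blueprint for characters who staff a home building matching their occupation and owning player.
; FindNewHome keeps an existing home or scans ActorManager's buildings for the closest unstaffed match, registers as its staff and rebuilds client UI.
; Readiness to work means being near the home's door and not going to eat.
; Death releases the building's staff slot, while RemoveHome clears the reference and refreshes the UI.
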(event EventBeginPlay
  (|CallParentFunction))

(event Collision|EventActorBeginOverlap
  (params (OtherActor :type Actor%20Object%20Reference))
  (|CallParentFunction OtherActor))

(event EventSubjectHandleDie
  (CallFunction|HandleHousebasedDie)
  (|CallParentFunction))

(event EventTick
  (params (DeltaSeconds :type Float%20%28single-precision%29))
  (|CallParentFunction DeltaSeconds))

(fn ConstructionScript
  (|CallParentFunction))

(fn IsatHome
  (if (Utilities|IsValidandNotNull (Variables|Default|GetHomeBuilding))
    (return (and (not (Variables|Default|GetgoingToEat)) (< (Utilities|VectorDistanceAbs (Transformation|GetWorldLocation (Variables|Default|GetCapsuleComponent self)) (Default|GetDoorLocation (Variables|Default|GetHomeBuilding))) 3e+02)))
    (else
      (return false))))

(fn FindNewHome
  (if (Utilities|IsValidandNotNull (Variables|Default|GetHomeBuilding)) ; If already has a home, don't look for a new one.
    (return true)
    (else
      (for _array_element (Variables|/Game/WnSAssets/Blueprints/Logics/Managers/BP_ActorManager.BP_ActorManager_C|GetBuildings (Variables|Default|GetactorManager))
        ;[1 1 1] Foreach Loop - Check if subject can work in this building, and i is closer than the last.
        (if (Utilities|Name|Equal(Name) (Variables|/Game/WnSAssets/Blueprints/Actors/Intermediates/Lots/BP_Lot.BP_Lot_C|GetowningPlayerName _array_element) (Variables|Default|GetowningPlayerName)) ; does this building belong to my player?
          (if (Utilities|Name|Equal(Name) (Variables|/Game/WnSAssets/Blueprints/Actors/Intermediates/Lots/BP_Building.BP_Building_C|GetwhoWorksHere _array_element) (Variables|Default|GetsubjectOccupation)) ; Is this a building I can work at?
            (if (not (Utilities|IsValidandNotNull (Variables|/Game/WnSAssets/Blueprints/Actors/Intermediates/Lots/BP_Building.BP_Building_C|GetMyStaff _array_element))) ; Is this building unstaffed?
              (if (< (Transformation|GetDistanceTo _array_element self) (LocalVariables|GetclosestBuildingDist)) ; Is this closer than the last closest?
                (LocalVariables|SetclosestBuilding _array_element)
                (LocalVariables|SetclosestBuildingDist (Transformation|GetDistanceTo _array_element self)))))))
      (if (Utilities|IsValidandNotNull (LocalVariables|GetclosestBuilding))
        (Default|SetasMyStaff (LocalVariables|GetclosestBuilding) self) ; Set as Staff
        (bind _output_get (Variables|Default|SetHomeBuilding (LocalVariables|GetclosestBuilding))) ; also set reference to that \nbuilding on this subject!
        (CallFunction|RemakeUIonClients)
        (return (Utilities|IsValidandNotNull _output_get))
        (else
          (return false))))))

(fn HandleHousebasedDie
  (if (Utilities|IsValidandNotNull (Variables|Default|GetHomeBuilding))
    (Default|RemoveMyStaff (Variables|Default|GetHomeBuilding))))

(fn RemoveHome
  (Variables|Default|SetHomeBuilding 0)
  (if (Utilities|IsValidandNotNull (Variables|Default|GetmySubjectUI))
    (Default|RemakeUI (Variables|Default|GetmySubjectUI))))

(fn IsReadytoWork
  (bind _ishome_ (CallFunction|IsatHome))
  (return _ishome_))

(fn GetCurrentJobWaitTime
  (return 0.0))