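; BP_Harvester is a Subject that plants, harvests and polishes resources for its home harvesting building.
; Find-job functions check occupation data tables, then spawn a harvestable or pick a random grown, unclaimed one in the building's area within planted-count limits.
; Complete-job functions advance the job status and feed raw material to the building; tending is stubbed.
; It notifies the player when harvestables are repeatedly missing and releases its target on death.
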(event EventBeginPlay
  (|CallParentFunction))

(event Collision|EventActorBeginOverlap
  (params (OtherActor :type Actor%20Object%20Reference))
  (|CallParentFunction OtherActor))

(event EventUpdateCurrentJobDescription
  ;[1 1 1] Override - Update Job Description
  (if (Variables|Default|GetgoingHome)
    (if (Utilities|Enum|Equal(Enum) (Variables|Harvester|GetcurrentJobStatus) "ReturningWithHarvest")
      (if (Variables|Default|GetgoingToEat) :!label _label
        (Variables|Default|SetCurrentJobDescription "Currently going to eat.")
        (else
          (Variables|Default|SetCurrentJobDescription (Utilities|Text|ToText(String) (Utilities|String|Append "Currently " (Class|Globals|GetHarvestingJobType (Variables|Harvester|GetcurrentJobStatus)) ".")))))
      (else
        (Variables|Default|SetCurrentJobDescription "Currently going home.")))
    (else
      (goto _label))))

(event EventSubjectHandleDie
  (params (invisible :type Boolean))
  ;[1 1 1] Override Handle Die - do additional stuff
  (Harvester|HandleHarvesterDie invisible)
  (|CallParentFunction invisible))

(event EventRemoveHome
  ;[1 1 1] Override Remove Home
  (|CallParentFunction)
  (Harvester|HarvesterRemoveHome))

(fn ConstructionScript
  (|CallParentFunction))

(fn FindHarvestJob
  (bind _availableharvestables (LocalVariables|GetavailableHarvestables))
  (bind _returnvalue (Utilities|Array|Length _availableharvestables))
  (if (CallFunction|GetOccupationDoesHarvestingJobTypeDT (Variables|Default|GetsubjectOccupation) "Harvesting") ; Does this Subject do this kind of harvestingJob at all?
    (bind _asbp_harvesting_building (Utilities|Casting|CastToBP_HarvestingBuilding (Variables|Default|GetHomeBuilding))
      (:then
        (bind _output_get (LocalVariables|SetharvestingHome _asbp_harvesting_building))
        (bind _returnvalue_2 (Class|HarvestingComponent|SpaceforHarvest (Variables|/Game/WnSAssets/Blueprints/Actors/Intermediates/Lots/BP_HarvestingBuilding.BP_HarvestingBuilding_C|GetHarvesting _output_get)))
        (if _returnvalue_2 ; Have space for harvest?
          (for _array_element (Default|ReturnArrayOfClass (Variables|Default|GetactorManager) (CallFunction|GetHarvestableClassDT (Variables|Harvester|GetharvestTargetType)))
            ;[1 1 1] Find a Harvestable to harvest
            (bind _asbp_harvestable (Utilities|Casting|CastToBP_Harvestable _array_element)
              (:then
                (if (Default|IsinHarvestingArea (LocalVariables|GetharvestingHome) (Transformation|GetWorldLocation (Variables|/Game/WnSAssets/Blueprints/Actors/Intermediates/BP_Harvestable.BP_Harvestable_C|GetDefaultSceneRoot _asbp_harvestable))) ; Is this in range for me?
                  (Math|Integer|IncrementInt (LocalVariables|GetreachableHarvestables)
                    (:%20%20
                      (if (Variables|/Game/WnSAssets/Blueprints/Actors/Intermediates/BP_Harvestable.BP_Harvestable_C|GetfullyGrown _asbp_harvestable) ; Is it fully grown?
                        (if (not (Variables|/Game/WnSAssets/Blueprints/Actors/Intermediates/BP_Harvestable.BP_Harvestable_C|GettargetForHarvest _asbp_harvestable)) ; Is already targeted by someone?
                          (Utilities|Array|AddUnique (LocalVariables|GetavailableHarvestables) _asbp_harvestable)))))))
              (:CastFailed
                (Development|PrintString "Harvester Find HarvestJob Cast to Interact.. failed")
                (return false))))
          (if (> (LocalVariables|GetreachableHarvestables) 0) ; Are there any harvestables at \nall in range for this harvester?
            (if (>= (LocalVariables|GetreachableHarvestables) (Variables|Harvester|GetminHarvestablesPlantedForHarvest)) ; Have enough harvestables been planted?
              (if (> _returnvalue 0) ; are there any available for harvest?
                (bind _output_get_2 (Variables|Harvester|SetcurrentJobTarget (Utilities|Array|Get(acopy) _availableharvestables (Math|Random|RandomInteger _returnvalue)))) ; Set a random available harvestable as job target
                (Default|SetHarvesting _output_get_2)
                (Harvester|SetJobStatus "Harvesting")
                (return true)
                (else
                  (return false) ; No Grown Harvestables\nin range.
                ))
              (else
                (return false) ; Only harvest if enough \nare planted.
              ))
            (else
              (Notifications|NoHarvestablesFound)
              (return false) ; None found at all.
            ))
          (else
            (return false))))
      (:CastFailed
        (Development|PrintString "Harvester find harvestJob Cast to HarvestingBuilding failed!")))
    (else
      (return false))))

(fn FindPolishJob
  (if (CallFunction|GetOccupationDoesHarvestingJobTypeDT (Variables|Default|GetsubjectOccupation) "Polishing") ; Does this Subject do this kind of harvestingJob at all?
    (bind _asbp_harvesting_building (Utilities|Casting|CastToBP_HarvestingBuilding (Variables|Default|GetHomeBuilding))
      (:then
        (if (Variables|/Script/WarriorsAndSerfs.HarvestingComponent|GethasRawMaterial (Variables|/Game/WnSAssets/Blueprints/Actors/Intermediates/Lots/BP_HarvestingBuilding.BP_HarvestingBuilding_C|GetHarvesting _asbp_harvesting_building))
          (Harvester|SetJobStatus "Polishing")
          (return true)
          (else
            (return false))))
      (:CastFailed
        (Development|PrintString "FindPolishJob Cast failed!")))
    (else
      (return false))))

(fn FindPlantJob
  (if (CallFunction|GetOccupationDoesHarvestingJobTypeDT (Variables|Default|GetsubjectOccupation) "Planting") ; Does this Subject do this kind of harvestingJob at all?
    (bind _asbp_harvesting_building (Utilities|Casting|CastToBP_HarvestingBuilding (Variables|Default|GetHomeBuilding))
      (:then
        (LocalVariables|SetharvestingHome _asbp_harvesting_building)
        (for _array_element (Default|ReturnArrayOfClass (Variables|Default|GetactorManager) (CallFunction|GetHarvestableClassDT (Variables|Harvester|GetharvestTargetType)))
          ;[1 1 1] Count how many harvestables are in ther current area
          (bind _asbp_harvestable (Utilities|Casting|CastToBP_Harvestable _array_element)
            (:then
              (if (Default|IsinHarvestingArea (LocalVariables|GetharvestingHome) (Transformation|GetWorldLocation (Variables|/Game/WnSAssets/Blueprints/Actors/Intermediates/BP_Harvestable.BP_Harvestable_C|GetDefaultSceneRoot _asbp_harvestable))) ; Is this in range for me?
                (Math|Integer|IncrementInt (LocalVariables|GetreachableHarvestables))))
            (:CastFailed
              (Development|PrintString "Harvester Find HarvestJob Cast to Harvestable failed")
              (return false))))
        (if (>= (LocalVariables|GetreachableHarvestables) (Variables|Harvester|GetmaxHarvestablesPlantedForPlanting)) ; Have too many harvestables been planted?
          (return false) ; Too many already planted, \ndo not plant more!
          (else
            ;[1 1 1] Start Planting
            (bind (_location _foundlocation) (Default|GetPointinHarvestingArea (LocalVariables|GetharvestingHome)))
            (if _foundlocation
              (bind _returnvalue (Game|SpawnActorfromClass (CallFunction|GetHarvestableClassDT (Variables|Harvester|GetharvestTargetType)) (Math|Conversions|ToTransform(Vector) _location) "AdjustIfPossibleButAlwaysSpawn" 0 0))
              (bind _output_get (Variables|Harvester|SetcurrentJobTarget _returnvalue))
              (Default|SetPlanting _output_get)
              (Harvester|SetJobStatus "Planting")
              (return true)
              (else
                (Variables|Harvester|SetcurrentJobTarget 0)
                (Harvester|SetJobStatus "None")
                (return false))))))
      (:CastFailed
        (Development|PrintString "Harvester find harvestJob Cast to HarvestingBuilding failed!")))
    (else
      (return false))))

(fn FindTendJob
  (if (CallFunction|GetOccupationDoesHarvestingJobTypeDT (Variables|Default|GetsubjectOccupation) "Tending") ; Does this Subject do this kind of harvestingJob at all?
    (return false)
    (else
      (return false))))

(fn CompleteHarvestingJob
  (Default|HarvestResource (Variables|Harvester|GetcurrentJobTarget))
  (Harvester|SetJobStatus "ReturningWithHarvest")
  (return true))

(fn CompleteReturnwithHarvestJob
  (if (Utilities|IsValidandNotNull (Variables|Default|GetHomeBuilding))
    (bind _asbp_harvesting_building (Utilities|Casting|CastToBP_HarvestingBuilding (Variables|Default|GetHomeBuilding))
      (:then
        (Class|HarvestingComponent|AddRawMaterial (Variables|/Game/WnSAssets/Blueprints/Actors/Intermediates/Lots/BP_HarvestingBuilding.BP_HarvestingBuilding_C|GetHarvesting _asbp_harvesting_building))
        (Harvester|SetJobStatus "Resting")
        (return true))
      (:CastFailed
        (Development|PrintString "CompletePolishJob Cast failed!")
        (return false)))
    (else
      (return false))))

(fn CompletePlantingJob
  (Default|Planted (Variables|Harvester|GetcurrentJobTarget))
  (Variables|Harvester|SetcurrentJobTarget 0)
  (Harvester|SetJobStatus "Resting")
  (return true))

(fn CompleteTendingJob
  (return false))

(fn CompletePolishingJob
  (bind _asbp_harvesting_building (Utilities|Casting|CastToBP_HarvestingBuilding (Variables|Default|GetHomeBuilding))
    (:then
      (Class|HarvestingComponent|FinishPolishingJob (Variables|/Game/WnSAssets/Blueprints/Actors/Intermediates/Lots/BP_HarvestingBuilding.BP_HarvestingBuilding_C|GetHarvesting _asbp_harvesting_building))
      (Harvester|SetJobStatus "Resting")
      (return true))
    (:CastFailed
      (Development|PrintString "CompletePolishJob Cast failed!")
      (return false))))

(fn CompleteReturningJob
  (return false))

(fn HandleHarvesterDie
  (params (invisible :type Boolean))
  (bind _currentjobtarget (Variables|Harvester|GetcurrentJobTarget))
  (if (Utilities|IsValidandNotNull _currentjobtarget)
    (Default|CancelHarvesting _currentjobtarget)))

(fn IsatHome
  (bind _ishome_ (|CallParentFunction))
  (return _ishome_))

(fn IsReadytoWork
  (bind _isready_ (|CallParentFunction))
  (return (and _isready_ (Utilities|Enum|Equal(Enum) (Variables|Harvester|GetcurrentJobStatus) "None"))))

(fn OverrideJobDurations
  (params (tendJobDuration :type Float%20%28single-precision%29) (harvestJobDuration :type Float%20%28single-precision%29) (polishJobDuration :type Float%20%28single-precision%29) (plantJobDuration :type Float%20%28single-precision%29) (restJobDuration :type Float%20%28single-precision%29))
  (if (> tendJobDuration 0.0)
    (Variables|Harvester|SettendJobDuration tendJobDuration))
  (if (> harvestJobDuration 0.0)
    (Variables|Harvester|SetharvestJobDuration harvestJobDuration))
  (if (> polishJobDuration 0.0)
    (Variables|Harvester|SetpolishJobDuration polishJobDuration))
  (if (> plantJobDuration 0.0)
    (Variables|Harvester|SetplantJobDuration plantJobDuration))
  (if (> restJobDuration 0.0)
    (Variables|Harvester|SetrestJobDuration restJobDuration)))

(fn CompleteRestingJob
  (Variables|Harvester|SetcurrentJobTarget 0)
  (Harvester|SetJobStatus "None")
  (return true))

(fn GetCurrentJobWaitTime
  (switch Utilities|FlowControl|Switch|SwitchonEHarvestingJobType (Variables|Harvester|GetcurrentJobStatus)
    (:None
      _)
    (:Planting
      (LocalVariables|SetjobStatusString "Plant")
      (bind _returnvalue (Class|Subject|CalculateWorkDuration (Utilities|String|StringToName (Utilities|String|Append (Utilities|String|ToString(Name) (Variables|Harvester|GetharvestTargetType)) (LocalVariables|GetjobStatusString))) (.polishDuration (Utilities|Struct|BreakHarvestingRecipe (Utilities|Array|Get(acopy) (Utilities|Struct|BreakDTS_Building (CallFunction|GetBuildingDT (Variables|/Game/WnSAssets/Blueprints/Actors/Intermediates/Lots/BP_Building.BP_Building_C|GetbuildingType (Variables|Default|GetHomeBuilding))))))) :!label _label))
      (return _returnvalue))
    (:Returning
      _)
    (:Tending
      (LocalVariables|SetjobStatusString "Tend")
      (goto _label))
    (:Harvesting
      (LocalVariables|SetjobStatusString "Harvest")
      (goto _label))
    (:ReturningWithHarvest
      _)
    (:Polishing
      (LocalVariables|SetjobStatusString "Polish")
      (goto _label))
    (:Resting
      (return 2.0)))
  (return 0.0))

(fn SetJobStatus
  (params (currentJobStatus :type EHarvestingJobType%20Enum :default "None"))
  (Variables|Harvester|SetcurrentJobStatus currentJobStatus)
  (CallFunction|UpdateJobDescriptiononServer))

(fn NoHarvestablesFound
  (bind _returnvalue (Utilities|Time|GetGameTimeinSeconds))
  (Math|Integer|IncrementInt (Variables|Notifications|Getdidn'tFindHarvestableCounter)
    (:%20%20
      (if (>= (Variables|Notifications|Getdidn'tFindHarvestableCounter) (Variables|Notifications|Getdidn'tFindHarvestableLimit)) ; Has the harvester not found harvestables often enough?\n(This function is called every few ticks!)
        (if (>= _returnvalue (+ (Variables|Notifications|GetlastNoHarvestablesNotifTime) (Variables|Notifications|GetnoHarvestablesNotifDelay))) ; is it time for another notification?
          (Variables|Notifications|SetlastNoHarvestablesNotifTime _returnvalue)
          (Variables|Notifications|Setdidn'tFindHarvestableCounter 0)
          (bind _aswn_s_player_controller (Utilities|Casting|CastToWnS_PlayerController (Game|GetPlayerController 0))
            (:then
              (bind _w_hud (Default|GetWHud _aswn_s_player_controller))
              (Default|MakeNotification _w_hud (Utilities|Text|FormatText "This {SubjectType} cannot find any {Harvestable}s in their assigned area. Perhaps you should move their Harvesting Area." (CallFunction|GetSubjectDisplayNameDT (Variables|Default|GetsubjectOccupation)) (CallFunction|GetHarvestableDisplayNameDT (Variables|Harvester|GetharvestTargetType))) "/Game/WnSAssets/Visual/Icons/Notifications/newsIcon.newsIcon" "0, 0, 0" (Variables|Default|GetHomeBuilding))
              (Default|NoHarvestablesNotifWasSent (Variables|/Game/WnSAssets/Blueprints/Player/WnS_PlayerController.WnS_PlayerController_C|GettutorialManager _aswn_s_player_controller)))
            (:CastFailed
              (Utilities|PrintStringRed15 "subject handle die cast to pc failed!"))))))))

(fn HarvesterRemoveHome
  (Variables|Harvester|SetcurrentJobStatus "None")
  (CallFunction|UpdateJobDescriptiononServer))

(fn FindNewHome
  (bind _foundahome_ (|CallParentFunction))
  (if _foundahome_
    (Variables|Harvester|SetharvestTargetType (.interactEnvType (Utilities|Struct|BreakHarvestingRecipe (Utilities|Array|Get(acopy) (.HarvestRecipeList (Utilities|Struct|BreakDTS_Building (CallFunction|GetBuildingDT (Variables|/Game/WnSAssets/Blueprints/Actors/Intermediates/Lots/BP_Building.BP_Building_C|GetbuildingType (Variables|Default|GetHomeBuilding)))))))))
    (return true)
    (else
      (return false))))

(fn SetNewHome
  (params (newHomeBuilding :type BP%20Building%20Object%20Reference))
  (bind _foundahome_ (|CallParentFunction newHomeBuilding))
  (if _foundahome_
    (Variables|Harvester|SetharvestTargetType (.interactEnvType (Utilities|Struct|BreakHarvestingRecipe (Utilities|Array|Get(acopy) (Utilities|Struct|BreakDTS_Building (CallFunction|GetBuildingDT (Variables|/Game/WnSAssets/Blueprints/Actors/Intermediates/Lots/BP_Building.BP_Building_C|GetbuildingType (Variables|Default|GetHomeBuilding))))))))
    (return true)
    (else
      (return false))))