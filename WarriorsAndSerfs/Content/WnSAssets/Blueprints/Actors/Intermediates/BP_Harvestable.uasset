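; Base harvestable resource actor that grows over time, gets harvested one unit at a time and destroys itself when depleted.
; Type data sets growth time, capacity and growability, while Tick scales the model by growth at a randomized rate.
; It registers with a tag-found ActorManager, spawning one if none exists.
; It also offers nav-checked interaction points with fallbacks, a click-spawned UI actor and an empty harvest-visual hook.
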(event EventBeginPlay
  (|CallParentFunction)
  (CallFunction|InitiateHarvestableType)
  (General|FindandAddtoActorManager)
  (Growing|UpdateGrowthVisual))

(event Collision|EventActorBeginOverlap
  (params (OtherActor :type Actor%20Object%20Reference)))

(event EventTick
  (params (DeltaSeconds :type Float%20%28single-precision%29))
  (|CallParentFunction DeltaSeconds)
  (Growing|GrowOverTime DeltaSeconds))

(fn ConstructionScript
  (|CallParentFunction)
  (CallFunction|InitiateHarvestableType))

(fn FindandAddtoActorManager
  (bind _outactors (Actor|GetAllActorswithTag "ActorManager"))
  (if (> (Utilities|Array|Length _outactors) 0)
    (for _array_element _outactors
      (bind _asbp_actor_manager (Utilities|Casting|CastToBP_ActorManager _array_element)
        (:then
          (bind _output_get (Variables|Default|SetactorManager _asbp_actor_manager))
          (Default|AddHarvestable _output_get self))
        (:CastFailed
          (Development|PrintString (Utilities|String|Append "" " Could Not cast to ActorManager!!")))))
    (else
      (bind _returnvalue (Game|SpawnActorfromClass "/Game/WnSAssets/Blueprints/Logics/Managers/BP_ActorManager.BP_ActorManager_C" (Math|Transform|MakeTransform "0, 0, 0") "AlwaysSpawn" 0 0)) ; If no LotManager was found, create a new one!
      (Development|PrintString "Spawned new ActorManager!")
      (bind _output_get_2 (Variables|Default|SetactorManager _returnvalue))
      (Default|AddHarvestable _output_get_2 self))))

(fn GetInteractionLocation
  (bind _interactionloc (Variables|Default|GetinteractionLoc))
  (bind _interactionloc2 (Variables|Default|GetinteractionLoc2))
  (bind _interactionloc3 (Variables|Default|GetinteractionLoc3))
  (bind _returnvalue (Transformation|GetWorldLocation _interactionloc3))
  (bind _returnvalue_2 (Transformation|GetWorldLocation _interactionloc))
  (bind _returnvalue_3 (Transformation|GetWorldLocation _interactionloc2))
  (if (.ReturnValue (AI|Navigation|ProjectPointtoNavigation _returnvalue_2 0 0 "0, 0, 0"))
    (return _returnvalue_2)
    (elif (.ReturnValue (AI|Navigation|ProjectPointtoNavigation _returnvalue_3 0 0 "0, 0, 0"))
      (return _returnvalue_3)
      (elif (.ReturnValue (AI|Navigation|ProjectPointtoNavigation _returnvalue 0 0 "0, 0, 0"))
        (return _returnvalue)
        (else
          (return "-999999.000000,-999999.000000,-999999.000000"))))))

(fn HarvestResource
  (bind _result (Math|Integer|DecrementInt (Variables|HarvestableSpecific|GetresourceAmount))
    (:%20%20
      (if (<= _result 0) ; Has this harvestable been \ncompletely harvested?
        (General|DestroyHarvestable)
        (else
          (Interacting|CancelHarvesting)
          (Interacting|HandleHarvestResourceVisual)
          (UI|UpdateUi))))))

(fn GrowOverTime
  (params (deltaTime :type Float%20%28single-precision%29))
  (if (Variables|Default|GetallowGrowth) ; if for some reason not allowed, do not grow.
    (if (< (Variables|Default|GetcurrentGrowthAmt) 1.0) ; Only grow if not fully grown yet.
      (if (<= (Variables|HarvestableSpecific|GetgrowthRate) 0.0) ; If not cached growth rate yet, do so first.
        (Variables|HarvestableSpecific|SetgrowthRate (/ 1.0 (Math|Random|RandomFloatinRange (Variables|HarvestableSpecific|GettimeUntilGrownMIN) (Variables|HarvestableSpecific|GettimeUntilGrownMAX)))))
      (Variables|Default|SetcurrentGrowthAmt (+ (Variables|Default|GetcurrentGrowthAmt) (* (Variables|HarvestableSpecific|GetgrowthRate) deltaTime)))
      (Growing|UpdateGrowthVisual)
      (UI|UpdateUi)
      (else
        (Networking|SwitchHasAuthority
          (:Authority
            (Variables|Default|SetfullyGrown true)
            (Variables|Default|SetallowGrowth false)))))))

(fn UpdateGrowthVisual
  (bind _currentgrowthamt (Variables|Default|GetcurrentGrowthAmt))
  (Transformation|SetRelativeScale3D (Variables|Default|GetModel) (Math|Vector|MakeVector _currentgrowthamt _currentgrowthamt _currentgrowthamt)))

(fn SetPlanting
  (Variables|Default|SetallowGrowth false))

(fn Planted
  (Variables|Default|SetallowGrowth true))

(fn SetHarvesting
  (Variables|Default|SettargetForHarvest true))

(fn CancelHarvesting
  (Variables|Default|SettargetForHarvest false))

(fn DestroyHarvestable
  (Default|RemoveHarvestable (Variables|Default|GetactorManager) self)
  (UI|CloseUI)
  (Actor|DestroyActor))

(fn HandleHarvestResourceVisual)

(fn CloseUI
  (bind _myui (Variables|UI|GetmyUI))
  (Utilities|IsValid _myui
    (:Is%20Valid
      (Actor|DestroyActor _myui))))

(fn OpenUI
  ;[1 1 1] Spawn and Cast to Widget, then spawn UI
  (if (not (Utilities|IsValid (Variables|UI|GetmyUI)))
    (bind _returnvalue (Game|SpawnActorfromClass "/Game/WnSAssets/Blueprints/UI/BP_HarvestableUI.BP_HarvestableUI_C" (Transformation|GetWorldTransform (Variables|Default|GetUISpawnPoint)) "AlwaysSpawn" 0 0))
    (Variables|UI|SetmyUI _returnvalue)
    (Variables|/Game/WnSAssets/Blueprints/UI/BP_UI.BP_UI_C|SetmyActor _returnvalue self)
    (Default|OpenUI _returnvalue true)))

(fn UpdateUi
  (bind _myui (Variables|UI|GetmyUI))
  (Utilities|IsValid _myui
    (:Is%20Valid
      (Default|UpdateUI _myui "None"))))

(fn RemakeUi
  (bind _myui (Variables|UI|GetmyUI))
  (Utilities|IsValid _myui
    (:Is%20Valid
      (Default|RemakeUI _myui))))

(fn GetWidget
  (bind _asw_harvestable (Utilities|Casting|CastToW_Harvestable (UserInterface|GetUserWidgetObject (Variables|/Game/WnSAssets/Blueprints/UI/BP_UI.BP_UI_C|GetUIWidget (Variables|UI|GetmyUI))))
    (:then
      (return _asw_harvestable))
    (:CastFailed
      (Development|PrintString (Utilities|String|Append "BP_Harvestable::GetWidget Failed! In:" (Utilities|String|ToString(Text) (CallFunction|GetHarvestableDisplayNameDT (Variables|HarvestableSpecific|GetharvestableType))))))))

(fn Clicked
  (UI|OpenUI))

(fn InitiateHarvestableType
  (bind _harvestabletype (Variables|HarvestableSpecific|GetharvestableType))
  (bind _dtsharvestable (CallFunction|GetHarvestableDT _harvestabletype))
  (bind (_harvestablename _displayname _orderinlists _helptext _icon _mesh _blueprintclass _timeuntilgrownmin _timeuntilgrownmax _cangrow _maxresourceamount) (Utilities|Struct|BreakDTS_Harvestable _dtsharvestable))
  (Variables|HarvestableSpecific|SettimeUntilGrownMIN _timeuntilgrownmin)
  (Variables|HarvestableSpecific|SettimeUntilGrownMAX _timeuntilgrownmax)
  (bind _output_get (Variables|HarvestableSpecific|SetmaxResourceAmount _maxresourceamount))
  (Variables|HarvestableSpecific|SetresourceAmount _output_get)
  (Variables|Default|SetallowGrowth _cangrow))