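; Player state that tracks which building types and education subjects the player is allowed to build or teach.
; Setters add or remove entries in the allowed lists, either singly or in bulk from the DT_Buildings row names or the subject enum.
; Building changes also tell the first player controller's HUD to remake its building list, while subject changes do not refresh the UI.
; Query functions report whether a given building or subject is allowed.
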(event EventBeginPlay)

(event EventTick
  (params (DeltaSeconds :type Float%20%28single-precision%29)))

(fn ConstructionScript)

(fn SetAllowBuilding
  (params (buildingType :type Name) (allowed :type Boolean))
  (Utilities|FlowControl|Sequence
    (:then_0
      (if allowed
        (Utilities|Array|AddUnique (Variables|Default|GetallowedBuildings) buildingType)
        (else
          (Utilities|Array|RemoveItem (Variables|Default|GetallowedBuildings) buildingType))))
    (:then_1
      (bind _aswn_s_player_controller (Utilities|Casting|CastToWnS_PlayerController (Game|GetPlayerController 0))
        (:then
          (bind _w_hud (Default|GetWHud _aswn_s_player_controller))
          (if (Utilities|IsValidandNotNull _w_hud)
            (Default|RemakeBuildingList _w_hud)))
        (:CastFailed
          (Utilities|PrintStringRed15 "playerstate set allow building cast to pc failed!"))))))

(fn SetAllowSubject
  (params (subjectType :type ESubjectType%20Enum :default "MissingNo") (allowed :type Boolean))
  (if allowed
    (Utilities|Array|AddUnique (Variables|Default|GetallowedSubjects) subjectType)
    (else
      (Utilities|Array|RemoveItem (Variables|Default|GetallowedSubjects) subjectType))))

(fn CanBuildBuilding
  (params (buildingType :type Name))
  (return (Utilities|Array|ContainsItem (Variables|Default|GetallowedBuildings) buildingType)))

(fn CanEducateSubject
  (params (subjectType :type ESubjectType%20Enum :default "MissingNo"))
  (return (Utilities|Array|ContainsItem (Variables|Default|GetallowedSubjects) subjectType)))

(fn SetAllowAllBuildings
  (params (allowed :type Boolean))
  (bind _outrownames (DataTable|GetDataTableRowNames "/Game/WnSAssets/Data/Buildings/DT_Buildings.DT_Buildings"))
  (for _array_element _outrownames
    ;[1 0 0] LOOP
    (if allowed
      (Utilities|Array|AddUnique (Variables|Default|GetallowedBuildings) _array_element)
      (else
        (Utilities|Array|RemoveItem (Variables|Default|GetallowedBuildings) _array_element))))
  (bind _aswn_s_player_controller (Utilities|Casting|CastToWnS_PlayerController (Game|GetPlayerController 0))
    (:then
      (bind _w_hud (Default|GetWHud _aswn_s_player_controller))
      (if (Utilities|IsValidandNotNull _w_hud)
        (Default|RemakeBuildingList _w_hud)))
    (:CastFailed
      (Utilities|PrintStringRed15 "playerstate set allow all buildings cast to pc failed!"))))

(fn SetAllowAllSubjects
  (params (allowed :type Boolean))
  (bind _enumvalue (|ForEachESubjectType)
    (:LoopBody
      (if allowed
        (Utilities|Array|AddUnique (Variables|Default|GetallowedSubjects) _enumvalue)
        (else
          (Utilities|Array|RemoveItem (Variables|Default|GetallowedSubjects) _enumvalue))))))