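; Central registry of strategy-game actors: buildings, construction sites, subjects and harvestables, which registers itself on the game mode at BeginPlay.
; Add and Remove functions route actors by type into per-class arrays, queryable by class or for the first warehouse.
; Buildings and subjects also keep per-type counts, updated by replacing struct entries, alongside an adjustable citizen limit.
; Removing a lot or subject triggers the game mode's game-over check.
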(event EventBeginPlay
  ;[1 1 1] Begin Play - get ref to gamemode
  (bind _aswn_s_strategic_game_mode (Utilities|Casting|CastToWnS_StrategicGameMode (Game|GetGameMode))
    (:then
      (bind _output_get (Variables|References|SetgameMode _aswn_s_strategic_game_mode))
      (Variables|/Game/WnSAssets/Blueprints/Logics/WnS_StrategicGameMode.WnS_StrategicGameMode_C|SetactorManager _output_get self))
    (:CastFailed
      (Utilities|PrintStringRed15 "ActorManager beginplay cat to gamemode failed"
        (:Exec
          _))))
  (bind _aswn_s_player_controller (Utilities|Casting|CastToWnS_PlayerController (Game|GetPlayerController 0))
    (:then
      (Variables|References|SetplayerController _aswn_s_player_controller))
    (:CastFailed
      (Utilities|PrintStringRed15 "ActorManager beginplay cast to playercontroller failed"
        (:Exec
          _))))
  (bind _aswns_player (Utilities|Casting|CastToWnsPlayer (Pawn|GetControlledPawn (Game|GetPlayerController 0)))
    (:then
      (Variables|References|SetwnsPlayer _aswns_player))
    (:CastFailed
      (Utilities|PrintStringRed15 "ActorManager beginplay cast to wnsPlayer failed"))))

(fn ConstructionScript)

(fn AddLot
  (params (Lot :type BP%20Lot%20Object%20Reference))
  (LocalVariables|SetinLot Lot)
  (if (Utilities|Enum|Equal(Enum) (Variables|/Script/WarriorsAndSerfs.Lot|GetlotType (LocalVariables|GetinLot)) "Building")
    (bind _asbp_building (Utilities|Casting|CastToBP_Building (LocalVariables|GetinLot))
      (:then
        (CallFunction|AddBuilding _asbp_building))
      (:CastFailed
        (Development|PrintString "LotManager::AddLot Cast to building Failed!!")))
    (elif (Utilities|Enum|Equal(Enum) (Variables|/Script/WarriorsAndSerfs.Lot|GetlotType (LocalVariables|GetinLot)) "Constructionsite")
      (bind _asbp_construction_site (Utilities|Casting|CastToBP_ConstructionSite (LocalVariables|GetinLot))
        (:then
          (Utilities|Array|AddUnique (Variables|Lists|GetConstructionsites) _asbp_construction_site))
        (:CastFailed
          (Development|PrintString "LotManager::AddLot Cast to constructionsite Failed!!"))))))

(fn RemoveLot
  (params (lot :type BP%20Lot%20Object%20Reference))
  (LocalVariables|SetinLot lot)
  (Utilities|FlowControl|Sequence
    (:then_0
      (if (Utilities|Enum|Equal(Enum) (Variables|/Script/WarriorsAndSerfs.Lot|GetlotType (LocalVariables|GetinLot)) "Building")
        (bind _asbp_building (Utilities|Casting|CastToBP_Building (LocalVariables|GetinLot))
          (:then
            (CallFunction|RemoveBuilding _asbp_building))
          (:CastFailed
            (Development|PrintString "LotManager::REmoveFromAll cast to building failed")))
        (elif (Utilities|Enum|Equal(Enum) (Variables|/Script/WarriorsAndSerfs.Lot|GetlotType (LocalVariables|GetinLot)) "Constructionsite")
          (bind _asbp_construction_site (Utilities|Casting|CastToBP_ConstructionSite (LocalVariables|GetinLot))
            (:then
              (Utilities|Array|RemoveItem (Variables|Lists|GetConstructionsites) _asbp_construction_site))
            (:CastFailed
              (Development|PrintString "LotManager::REmoveFromAll cast to constructionsite failed"))))))
    (:then_1
      (Default|CheckGameOver (Variables|References|GetgameMode)))))

(fn AddHarvestable
  (params (Harvestable :type BP%20Harvestable%20Object%20Reference))
  (bind _output_get (LocalVariables|SettheObject Harvestable))
  (switch name (Variables|/Game/WnSAssets/Blueprints/Actors/Intermediates/BP_Harvestable.BP_Harvestable_C|GetharvestableType _output_get)
    (:Default
      (Utilities|PrintStringRed15 (Utilities|String|Append "couldn't add unknown harvestable \"" (Utilities|String|ToString(Name) (Variables|/Game/WnSAssets/Blueprints/Actors/Intermediates/BP_Harvestable.BP_Harvestable_C|GetharvestableType _output_get)) "\" to actor manager!")))
    (:Tree
      (bind _asbp_tree (Utilities|Casting|CastToBP_Tree (LocalVariables|GettheObject))
        (:then
          (Utilities|Array|AddUnique (Variables|Lists|GetTrees) _asbp_tree))
        (:CastFailed
          (Development|PrintString "AddHarvestable cast to Tree failed!"))))
    (:Wheat
      (bind _asbp_wheat (Utilities|Casting|CastToBP_Wheat (LocalVariables|GettheObject))
        (:then
          (Utilities|Array|AddUnique (Variables|Lists|GetWheat) _asbp_wheat))
        (:CastFailed
          (Development|PrintString "AddHarvestable cast to Wheat failed!"))))
    (:Stone
      (bind _asbp_rock (Utilities|Casting|CastToBP_Rock (LocalVariables|GettheObject))
        (:then
          (Utilities|Array|AddUnique (Variables|Lists|GetRocks) _asbp_rock))
        (:CastFailed
          (Development|PrintString "AddHarvestable cast to Rock failed!"))))
    (:Goldmine
      (bind _asbp_gold_rock (Utilities|Casting|CastToBP_GoldRock (LocalVariables|GettheObject))
        (:then
          (Utilities|Array|AddUnique (Variables|Lists|GetGoldRocks) _asbp_gold_rock))
        (:CastFailed
          (Development|PrintString "AddHarvestable cast to GoldRock failed!"))))
    (:Ironmine
      (bind _asbp_iron_rock (Utilities|Casting|CastToBP_IronRock (LocalVariables|GettheObject))
        (:then
          (Utilities|Array|AddUnique (Variables|Lists|GetIronRocks) _asbp_iron_rock))
        (:CastFailed
          (Development|PrintString "AddHarvestable cast to IronRock failed!"))))
    (:Coalmine
      (bind _asbp_coal_rock (Utilities|Casting|CastToBP_CoalRock (LocalVariables|GettheObject))
        (:then
          (Utilities|Array|AddUnique (Variables|Lists|GetCoalRocks) _asbp_coal_rock))
        (:CastFailed
          (Development|PrintString "AddHarvestable cast to CoalRock failed!"))))))

(fn RemoveHarvestable
  (params (Harvestable :type BP%20Harvestable%20Object%20Reference))
  (bind _output_get (LocalVariables|SettheObject Harvestable))
  (switch name (Variables|/Game/WnSAssets/Blueprints/Actors/Intermediates/BP_Harvestable.BP_Harvestable_C|GetharvestableType _output_get)
    (:Default
      (Utilities|PrintStringRed15 (Utilities|String|Append "Couldn't remove unkown Harvestable \"" (Utilities|String|ToString(Name) (Variables|/Game/WnSAssets/Blueprints/Actors/Intermediates/BP_Harvestable.BP_Harvestable_C|GetharvestableType _output_get)) "\" from ActorManager")))
    (:Tree
      (bind _asbp_tree (Utilities|Casting|CastToBP_Tree (LocalVariables|GettheObject))
        (:then
          (Utilities|Array|RemoveItem (Variables|Lists|GetTrees) _asbp_tree))
        (:CastFailed
          (Development|PrintString "RemoveHarvestable cast to Tree failed!"))))
    (:Wheat
      (bind _asbp_wheat (Utilities|Casting|CastToBP_Wheat (LocalVariables|GettheObject))
        (:then
          (Utilities|Array|RemoveItem (Variables|Lists|GetWheat) _asbp_wheat))
        (:CastFailed
          (Development|PrintString "RemoveHarvestable cast to Wheat failed!"))))
    (:Stone
      (bind _asbp_rock (Utilities|Casting|CastToBP_Rock (LocalVariables|GettheObject))
        (:then
          (Utilities|Array|RemoveItem (Variables|Lists|GetRocks) _asbp_rock))
        (:CastFailed
          (Development|PrintString "RemoveHarvestable cast to Rock failed!"))))
    (:Goldmine
      (bind _asbp_gold_rock (Utilities|Casting|CastToBP_GoldRock (LocalVariables|GettheObject))
        (:then
          (Utilities|Array|RemoveItem (Variables|Lists|GetGoldRocks) _asbp_gold_rock))
        (:CastFailed
          (Development|PrintString "RemoveHarvestable cast to GoldRock failed!"))))
    (:Ironmine
      (bind _asbp_iron_rock (Utilities|Casting|CastToBP_IronRock (LocalVariables|GettheObject))
        (:then
          (Utilities|Array|RemoveItem (Variables|Lists|GetIronRocks) _asbp_iron_rock))
        (:CastFailed
          (Development|PrintString "RemoveHarvestable cast to IronRock failed!"))))
    (:Coalmine
      (bind _asbp_coal_rock (Utilities|Casting|CastToBP_CoalRock (LocalVariables|GettheObject))
        (:then
          (Utilities|Array|RemoveItem (Variables|Lists|GetCoalRocks) _asbp_coal_rock))
        (:CastFailed
          (Development|PrintString "RemoveHarvestable cast to CoalRock failed!"))))))

(fn ReturnArrayOfClass
  (params (class :type Actor%20Class%20Reference))
  (LocalVariables|SetinClass class)
  (if (== (LocalVariables|GetinClass) "/Game/WnSAssets/Blueprints/Actors/Final/Harvestable/BP_Tree.BP_Tree_C")
    (return (Variables|Lists|GetTrees))
    (elif (== (LocalVariables|GetinClass) "/Game/WnSAssets/Blueprints/Actors/Intermediates/Lots/BP_Building.BP_Building_C")
      (return (Variables|Lists|GetBuildings))
      (elif (== (LocalVariables|GetinClass) "/Game/WnSAssets/Blueprints/Actors/Final/Harvestable/BP_Wheat.BP_Wheat_C")
        (return (Variables|Lists|GetWheat))
        (elif (== (LocalVariables|GetinClass) "/Game/WnSAssets/Blueprints/Actors/Final/Construction/BP_ConstructionSite.BP_ConstructionSite_C")
          (return (Variables|Lists|GetConstructionsites))
          (elif (== (LocalVariables|GetinClass) "/Game/WnSAssets/Blueprints/Actors/Intermediates/Subjects/BP_Subject.BP_Subject_C")
            (return (Variables|Lists|GetSubjects))
            (elif (== (LocalVariables|GetinClass) "/Game/WnSAssets/Blueprints/Actors/Final/Harvestable/BP_Rock.BP_Rock_C")
              (return (Variables|Lists|GetRocks))
              (elif (== (LocalVariables|GetinClass) "/Game/WnSAssets/Blueprints/Actors/Final/Harvestable/BP_GoldRock.BP_GoldRock_C")
                (return (Variables|Lists|GetGoldRocks))
                (elif (== (LocalVariables|GetinClass) "/Game/WnSAssets/Blueprints/Actors/Final/Harvestable/BP_IronRock.BP_IronRock_C")
                  (return (Variables|Lists|GetIronRocks))
                  (elif (== (LocalVariables|GetinClass) "/Game/WnSAssets/Blueprints/Actors/Final/Harvestable/BP_CoalRock.BP_CoalRock_C")
                    (return (Variables|Lists|GetCoalRocks))))))))))))

(fn AddSubject
  (params (subject :type BP%20Subject%20Object%20Reference))
  (bind _subjectoccupation (Variables|/Script/WarriorsAndSerfs.Subject|GetsubjectOccupation subject))
  (Utilities|Array|AddUnique (Variables|Lists|GetSubjects) subject)
  (bind (_array_element _array_index) (Utilities|Array|ForEachLoopwithBreak (Variables|Amounts|GetsubjectAmounts) :!label _label)
    (:LoopBody
      ;[1 0 0] Foreach Loop
      (if (Utilities|Name|Equal(Name) (.subjectType (Utilities|Struct|BreaksubjectAmount _array_element)) _subjectoccupation)
        ;;[1 1 1] Cannot change the subjectAmount in the list, so need to make new, delete the old and add the new...
        (LocalVariables|SetnewSubjectAmt (Utilities|Struct|MakesubjectAmount _subjectoccupation (+ (.amount (Utilities|Struct|BreaksubjectAmount _array_element)) 1)))
        (Utilities|Array|RemoveIndex (Variables|Amounts|GetsubjectAmounts) _array_index)
        (Utilities|Array|Add (Variables|Amounts|GetsubjectAmounts) (LocalVariables|GetnewSubjectAmt))
        (LocalVariables|SetaddedSubject true)
        (goto _label Break)))
    (:Completed
      (if (not (LocalVariables|GetaddedSubject)) ; was the subject added to the subjectAmount?
        (Utilities|Array|Add (Variables|Amounts|GetsubjectAmounts) (Utilities|Struct|MakesubjectAmount _subjectoccupation 1))))))

(fn RemoveSubject
  (params (subject :type BP%20Subject%20Object%20Reference))
  (bind _subjectoccupation (Variables|/Script/WarriorsAndSerfs.Subject|GetsubjectOccupation subject))
  (Utilities|Array|RemoveItem (Variables|Lists|GetSubjects) subject)
  (Utilities|FlowControl|Sequence
    (:then_0
      (bind (_array_element _array_index) (Utilities|Array|ForEachLoopwithBreak (Variables|Amounts|GetsubjectAmounts) :!label _label)
        (:LoopBody
          ;[1 0 0] Foreach Loop
          (if (Utilities|Name|Equal(Name) (.subjectType (Utilities|Struct|BreaksubjectAmount _array_element)) _subjectoccupation)
            ;;[1 1 1] Cannot change the subjectAmount in the list, so need to make new, delete the old and add the new...
            (LocalVariables|SetnewSubjectAmt (Utilities|Struct|MakesubjectAmount _subjectoccupation (- (.amount (Utilities|Struct|BreaksubjectAmount _array_element)) 1)))
            (Utilities|Array|RemoveIndex (Variables|Amounts|GetsubjectAmounts) _array_index)
            (Utilities|Array|Add (Variables|Amounts|GetsubjectAmounts) (LocalVariables|GetnewSubjectAmt))
            (goto _label Break)))))
    (:then_1
      (Default|CheckGameOver (Variables|References|GetgameMode)))))

(fn GetFirstWarehouse
  (for _array_element (Variables|Lists|GetBuildings)
    (if (Utilities|Name|Equal(Name) (Variables|/Game/WnSAssets/Blueprints/Actors/Intermediates/Lots/BP_Building.BP_Building_C|GetbuildingType _array_element) "Warehouse")
      (bind _asbp_warehouse (Utilities|Casting|CastToBP_Warehouse _array_element)
        (:then
          (return _asbp_warehouse))
        (:CastFailed
          (Utilities|PrintStringRed15 "actormanager getwarehouse cast to warehouse failed!")))))
  (Utilities|PrintStringRed15 "no warehouse found.."
    (:Exec
      (return 0))))

(fn AddBuilding
  (params (building :type BP%20Building%20Object%20Reference))
  (bind _buildingtype (Variables|/Game/WnSAssets/Blueprints/Actors/Intermediates/Lots/BP_Building.BP_Building_C|GetbuildingType building))
  (Utilities|Array|AddUnique (Variables|Lists|GetBuildings) building)
  (bind (_array_element _array_index) (Utilities|Array|ForEachLoopwithBreak (Variables|Amounts|GetbuildingAmounts) :!label _label)
    (:LoopBody
      ;[1 0 0] Foreach Loop
      (if (Utilities|Name|Equal(Name) (.buildingType (Utilities|Struct|BreakBuildingAmount _array_element)) _buildingtype)
        ;;[1 1 1] Cannot change the buildingAmount in the list, so need to make new, delete the old and add the new...
        (LocalVariables|SetnewBuildingAmt (Utilities|Struct|MakeBuildingAmount _buildingtype (+ (.amount (Utilities|Struct|BreakBuildingAmount _array_element)) 1)))
        (Utilities|Array|RemoveIndex (Variables|Amounts|GetbuildingAmounts) _array_index)
        (Utilities|Array|Add (Variables|Amounts|GetbuildingAmounts) (LocalVariables|GetnewBuildingAmt))
        (LocalVariables|SetaddedBuilding true)
        (goto _label Break)))
    (:Completed
      (if (not (LocalVariables|GetaddedBuilding)) ; was the building added to the buildingAmount?
        (Utilities|Array|Add (Variables|Amounts|GetbuildingAmounts) (Utilities|Struct|MakeBuildingAmount _buildingtype 1))))))

(fn RemoveBuilding
  (params (building :type BP%20Building%20Object%20Reference))
  (bind _buildingtype (Variables|/Game/WnSAssets/Blueprints/Actors/Intermediates/Lots/BP_Building.BP_Building_C|GetbuildingType building))
  (Utilities|Array|RemoveItem (Variables|Lists|GetBuildings) building)
  (bind (_array_element _array_index) (Utilities|Array|ForEachLoopwithBreak (Variables|Amounts|GetbuildingAmounts) :!label _label)
    (:LoopBody
      ;[1 0 0] Foreach Loop
      (if (Utilities|Name|Equal(Name) (.buildingType (Utilities|Struct|BreakBuildingAmount _array_element)) _buildingtype)
        ;;[1 1 1] Cannot change the buildingAmount in the list, so need to make new, delete the old and add the new...
        (LocalVariables|SetnewBuildingAmt (Utilities|Struct|MakeBuildingAmount _buildingtype (- (.amount (Utilities|Struct|BreakBuildingAmount _array_element)) 1)))
        (Utilities|Array|RemoveIndex (Variables|Amounts|GetbuildingAmounts) _array_index)
        (Utilities|Array|Add (Variables|Amounts|GetbuildingAmounts) (LocalVariables|GetnewBuildingAmt))
        (goto _label Break)))))

(fn ChangeCitizenLimit
  (params (limitIncrease :type Integer))
  (Variables|Amounts|SetCitizenLimit (+ limitIncrease (Variables|Amounts|GetCitizenLimit))))