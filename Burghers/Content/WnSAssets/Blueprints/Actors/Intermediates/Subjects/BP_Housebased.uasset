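; Intermediate Blueprint for subjects tied to a home building where they work as its staff.
; SetNewHome links subject and building both ways, while death clears the building's staff slot and RemoveHome clears the subject's reference.
; Work readiness requires standing near the home's door and not going to eat.
; FindNewHome's nearest-unstaffed-building search by owner and occupation is disconnected, so it never runs.
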(event EventBeginPlay
  (|CallParentFunction))

(event Collision|EventActorBeginOverlap
  (params (OtherActor :type Actor%20Object%20Reference))
  (|CallParentFunction OtherActor))

(event EventSubjectHandleDie
  (params (invisible :type Boolean))
  (Housebased|HandleHousebasedDie invisible)
  (|CallParentFunction invisible))

(event EventTick
  (params (DeltaSeconds :type Float%20%28single-precision%29))
  (|CallParentFunction DeltaSeconds))

(fn ConstructionScript
  (|CallParentFunction))

(fn IsatHome
  (if (Utilities|IsValidandNotNull (Variables|Default|GetHomeBuilding))
    (return (and (not (Variables|Default|GetgoingToEat)) (< (Utilities|VectorDistanceAbs (Transformation|GetWorldLocation (Variables|Default|GetCapsuleComponent self)) (Default|GetDoorLocation (Variables|Default|GetHomeBuilding))) 3e+02)))
    (else
      (return false))))

(fn FindNewHome)

(fn HandleHousebasedDie
  (params (invisible :type Boolean))
  (if (Utilities|IsValidandNotNull (Variables|Default|GetHomeBuilding))
    (Default|RemoveMyStaff (Variables|Default|GetHomeBuilding))
    (CallFunction|UpdateUI "HomeButton")))

(fn RemoveHome
  (Variables|Default|SetHomeBuilding 0)
  (if (Utilities|IsValidandNotNull (Variables|Default|GetmyUI))
    (CallFunction|UpdateUI "HomeButton")
    (Utilities|PrintStringRed15 "updateHomeButton")))

(fn IsReadytoWork
  (bind _ishome_ (Housebased|IsatHome))
  (return _ishome_))

(fn GetCurrentJobWaitTime
  (return 0.0))

(fn SetNewHome
  (params (newHomeBuilding :type BP%20Building%20Object%20Reference))
  (Default|SetasMyStaff newHomeBuilding self) ; Set as Staff
  (bind _output_get (Variables|Default|SetHomeBuilding newHomeBuilding)) ; also set reference to that \nbuilding on this subject!
  (CallFunction|UpdateUI "HomeButton")
  (return (Utilities|IsValidandNotNull _output_get)))