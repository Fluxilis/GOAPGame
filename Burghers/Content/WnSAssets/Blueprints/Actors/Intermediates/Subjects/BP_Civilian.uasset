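; BP_Civilian is an intermediate Subject Blueprint that gives civilians meal behavior and a job description.
; EatAtInn asks an inn to feed the civilian, refills food on success, clears GoingToEat either way and refreshes the description on the server.
; The job description override shows the going-to-eat text or a missing-override warning.
; SkipMeal flips a toggle and returns its previous value, so successive calls alternate.
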(event Collision|EventActorBeginOverlap
  (params (OtherActor :type Actor%20Object%20Reference)))

(event EventUpdateCurrentJobDescription
  ;[1 1 1] Override Update Job Description
  (if (Variables|Default|GetgoingToEat)
    (Variables|Default|SetCurrentJobDescription "Currently going to eat.")
    (CallFunction|UpdateUI "Job")
    (else
      (Variables|Default|SetCurrentJobDescription "MISSING SUBJECT JOB OVERRIDE!")
      (CallFunction|UpdateUI "Job"))))

(event EventTick
  (params (DeltaSeconds :type Float%20%28single-precision%29))
  (|CallParentFunction DeltaSeconds))

(fn ConstructionScript
  (|CallParentFunction))

(fn EatatInn
  (params (whatInn :type BP%20Inn%20Object%20Reference))
  (bind _ate (Default|SubjectEatHere whatInn self))
  (Variables|Default|SetgoingToEat false) ; If ate, set false bc no longer need to eat\nIf not, set false because skip meal
  (if _ate ; Did Subject Eat?
    (Variables|Default|SetcurrentFood (Variables|Default|GetmaxFood))
    (CallFunction|UpdateJobDescriptiononServer)
    (return true)
    (else
      (CallFunction|UpdateJobDescriptiononServer)
      (return false))))

(fn SkipMeal
  (bind _output_get (Variables|Default|SetshouldSkipMeal (not (Variables|Default|GetshouldSkipMeal)))) ; Toggle this bool
  (return (not _output_get)))