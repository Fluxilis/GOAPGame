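; BP_Subject is the citizen actor, with a random name, data-table-driven occupation stats and icon, a clickable UI and death notifications.
; It registers with BP_ActorManager and periodically claims a free residence from its list.
; Serfs apply for building jobs by suitability margin and for builder jobs unconditionally.
; Changing occupation spawns a replacement of the new class, copies name, stats and residence, then invisibly kills the original.
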(event Custom|RemakeUIOnClients
  ;[1 1 1] Replication - Updates UI for all clients (NOT NEEDED!?)
  (UI|RemakeUI))

(event Custom|SetPlayerLabelOnServer
  (params (newLabel :type Text))
  ;[1 1 1] Replication - Changing PlayerLabel through UI
  (CallFunction|SetPlayerLabel self newLabel) ; Set locally so there is instant feedback\nuntil the change from server comes back.
  (bind _aswn_s_player_controller (Utilities|Casting|CastToWnS_PlayerController (Game|GetPlayerController 0)))
  (Default|SetSubjectPlayerLabel _aswn_s_player_controller self newLabel))

(event Custom|UpdateJobDescriptionOnServer
  ;[1 1 1] Replication - Updating Job description
  (bind _aswn_s_player_controller (Utilities|Casting|CastToWnS_PlayerController (Game|GetPlayerController 0)))
  (Default|UpdateJobDescription _aswn_s_player_controller self))

(event Custom|NotifyClientsUpdatedJobDescription
  (params (jobDescription :type Text))
  ;[1 1 1] Replication - Updating Job description
  (Variables|Job|SetCurrentJobDescription jobDescription)
  (UI|UpdateUI "Job"))

(event Custom|NotifyClientsChangedPlayerLabel
  (params (newLabel :type Text))
  ;[1 1 1] Replication - Changing PlayerLabel through UI
  (CallFunction|SetPlayerLabel self newLabel))

(event Custom|UpdateUIOnClients
  (params (uiToUpdate :type Name))
  ;[1 1 1] Replication - Updates UI for all clients (NOT NEEDED!?)
  (UI|UpdateUI uiToUpdate))

(event Custom|DestroyOnServer
  ;[1 1 1] Replication - Destroying Subject
  (UI|CloseUI)
  (bind _aswn_s_player_controller (Utilities|Casting|CastToWnS_PlayerController (Game|GetPlayerController 0)))
  (Default|KillSubject _aswn_s_player_controller self))

(event Custom|NewJobAvailable
  (params (building :type BP%20Building%20Object%20Reference))
  ;[1 1 1] called from BP_building when a job becomes available (construction complete, employee dies or changes job...)
  (ChangeOccupation|ConsiderApplyingforJob building))

(event Custom|NotifyClientsHandleSubjectDie
  (params (invisible :type Boolean))
  ;[1 1 1] Replication - Destroying Subject
  (CallFunction|SubjectHandleDieonClient invisible))

(event Custom|BuilderJobAvailable
  (params (constructionSite :type BP%20Construction%20Site%20Object%20Reference))
  ;[1 1 1] called from constructionsites when there has been no construction progress in a while.
  (ChangeOccupation|ConsiderApplyingforBuilderJob constructionSite))

(event EventTick
  (params (DeltaSeconds :type Float%20%28single-precision%29))
  (|CallParentFunction DeltaSeconds)
  (Residence|HandleFindResidence))

(event EventBeginPlay
  (|CallParentFunction)
  (CallFunction|InitiateSubjectType)
  (CallFunction|SetRandomName)
  (Networking|SwitchHasAuthority
    (:Authority
      ;[1 0 0] SWITCH
      (CallFunction|AddtoActorManager))))

(event EventSubjectDie
  (params (invisible :type Boolean))
  ;[1 1 1] Subject Die
  (CallFunction|SubjectHandleDie invisible)
  (|CallParentFunction invisible))

(event EventUpdateActiveUI
  (params (uiToUpdate :type Name :default "None"))
  ;[1 1 1] This event is called from C++
  ; updates UI on clients
  (CallFunction|UpdateUIonClients uiToUpdate))

(fn ConstructionScript
  (|CallParentFunction)
  ;[1 1 1] If this subject was spawned as a result of switching occupation
  (if (Variables|ChangeOccupation|GetconstructChangedOccupation)
    (Variables|Default|SetowningPlayerName "wnsplayer0")
    (Variables|Default|SetsubjectOccupation (Variables|Default|GetconstructSubjectOccupation))
    (CallFunction|InitiateSubjectType)
    (else
      (if (Utilities|Name|NotEqual(Name) (Variables|Default|GetowningPlayerName) "DONOTHANDLE") ; set singleplayer playername \n(except special cases)
        (Variables|Default|SetowningPlayerName "wnsplayer0"))
      (if (Utilities|Name|Equal(Name) (Variables|Default|GetsubjectOccupation) "None")
        (Variables|Default|SetsubjectOccupation (Variables|Default|GetconstructSubjectOccupation)))
      (CallFunction|InitiateSubjectType))))

(fn Clicked
  (params (clickingPlayer :type Name))
  (if (Utilities|Name|Equal(Name) clickingPlayer (Variables|Default|GetowningPlayerName))
    (UI|OpenUI true)
    (else
      (UI|OpenUI false))))

(fn OpenUI
  (params (isOwnerUI :type Boolean))
  (bind _self self)
  (Utilities|IsValid (Variables|UI|GetmyUI) ; Already open?
    (:Is%20Not%20Valid
      (bind _returnvalue (UserInterface|CreateWidget "/Game/WnSAssets/Widgets/Gameplay/ActorUI/Subjects/W_Subject.W_Subject_C" 0 0 _self _self isOwnerUI))
      (Variables|UI|SetmyUI _returnvalue)
      (bind _aswn_s_player_controller (Utilities|Casting|CastToWnS_PlayerController (Game|GetPlayerController 0))
        (:then
          (bind _w_hud (Default|GetWHud _aswn_s_player_controller))
          (Default|AddActorUI _w_hud _returnvalue))
        (:CastFailed
          (Utilities|PrintStringRed15 "subject openUi cast to pc failed"))))))

(fn CallUpdateUIonClients
  (CallFunction|UpdateUIonClients "None"))

(fn CloseUI
  (Utilities|IsValid (Variables|UI|GetmyUI)
    (:Is%20Valid
      (Widget|RemovefromParent (Variables|UI|GetmyUI))
      (Variables|UI|SetmyUI 0))))

(fn AddtoActorManager
  (Utilities|FlowControl|Sequence
    (:then_0
      (bind _outactors (Actor|GetAllActorswithTag "ActorManager"))
      (if (> (Utilities|Array|Length _outactors) 0)
        (for _array_element _outactors
          (bind _asbp_actor_manager (Utilities|Casting|CastToBP_ActorManager _array_element)
            (:then
              (Variables|Default|SetactorManager _asbp_actor_manager))
            (:CastFailed
              (Development|PrintString (Utilities|String|Append (Variables|Default|GetplayerLabel) " Could Not cast to ActorManager!!")))))
        (else
          (bind _returnvalue (Game|SpawnActorfromClass "/Game/WnSAssets/Blueprints/Logics/Managers/BP_ActorManager.BP_ActorManager_C" (Math|Transform|MakeTransform "0, 0, 0") "AlwaysSpawn" 0 0)) ; If no LotManager was found, create a new one!
          (Variables|Default|SetactorManager _returnvalue))))
    (:then_1
      (Default|AddSubject (Variables|Default|GetactorManager) self))))

(fn SubjectHandleDie
  (params (invisible :type Boolean))
  (if invisible
    (Networking|SwitchHasAuthority :!label _label
      (:Authority
        (UI|CloseUI)
        (CallFunction|NotifyClientsHandleSubjectDie invisible)
        (CallFunction|RemovefromActorManager)
        (Residence|RemovefromResidence)
        (Actor|DestroyActor)))
    (else
      (Utilities|FlowControl|Sequence
        (:then_0
          ;[1 1 1] Notify player subject Died
          ;;[1 1 1] Find Deathcause
          (if (<= (Variables|Default|GetcurrentFood) 0.0)
            (LocalVariables|SetdeathcauseText " of Hunger"))
          (bind _aswn_s_player_controller (Utilities|Casting|CastToWnS_PlayerController (Game|GetPlayerController 0))
            (:then
              (bind _w_hud (Default|GetWHud _aswn_s_player_controller))
              (Default|MakeNotification _w_hud (Utilities|Text|FormatText "{PlayerLabel}, one of your citizens with Job {SubjectType} died{Deathcause}." (Utilities|Text|ToText(String) (Variables|Default|GetplayerLabel)) (CallFunction|GetSubjectDisplayNameDT (Variables|Default|GetsubjectOccupation)) (LocalVariables|GetdeathcauseText)) "/Game/WnSAssets/Visual/Icons/Notifications/deadIcon.deadIcon" (Transformation|GetWorldLocation (Variables|Default|GetCapsuleComponent)))
              (CallFunction|MakeHungerDeathNotif))
            (:CastFailed
              (Utilities|PrintStringRed15 "subject handle die cast to pc failed!"))))
        (:then_1
          (goto _label))))))

(fn UpdateCurrentJobDescription
  (Variables|Job|SetCurrentJobDescription "MISSING SUBJECT JOB OVERRIDE!")
  (UI|UpdateUI "Job"))

(fn UpdateUI
  (params (uiToUpdate :type Name))
  (Utilities|IsValid (Variables|UI|GetmyUI)
    (:Is%20Valid
      (Default|UpdateUI (Variables|UI|GetmyUI) uiToUpdate))))

(fn SetPlayerLabel
  (params (newLabel :type Text))
  (Variables|Default|SetplayerLabel (Utilities|String|ToString(Text) newLabel))
  (UI|UpdateUI "Labels"))

(fn CallRemakeUIonClients
  (CallFunction|RemakeUIonClients))

(fn RemakeUI
  (Utilities|IsValid (Variables|UI|GetmyUI)
    (:Is%20Valid
      (UI|UpdateUI "None"))))

(fn SubjectHandleDieonClient
  (params (invisible :type Boolean))
  (if invisible
    _
    (else
      ;[1 1 1] only spawn sound if death is not "invisible" (eg not when citizen switched occupation)
      (Audio|SpawnSoundatLocation "/Game/WnSAssets/Audio/Files/FX/death1.death1" (Transformation|GetWorldLocation (Variables|Default|GetCapsuleComponent)) "0, 0, 0" 1.0 1.0 0.0 0 0)))
  (UI|CloseUI))

(fn RemovefromActorManager
  (Default|RemoveSubject (Variables|Default|GetactorManager) self))

(fn InitiateSubjectType
  (bind _subjectoccupation (Variables|Default|GetsubjectOccupation))
  (bind _dtssubject (CallFunction|GetSubjectDT _subjectoccupation))
  (bind (_subjectname _maxhealth _educatecost) (Utilities|Struct|BreakDTS_Subject _dtssubject))
  (bind _output_get (Variables|Default|SetmaxHealth _maxhealth))
  (Variables|Default|SetcurrentHealth _output_get)
  (CallFunction|UpdateOverheadIcon)
  (Variables|Default|SetsubjectEducateCost _educatecost))

(fn UpdateOverheadIcon
  ;[1 1 1] Set Overhead Icon (Temporary)
  (bind _astexture_2d (Utilities|Casting|CastToTexture2D (CallFunction|GetSubjectIconDT (Variables|Default|GetsubjectOccupation)))
    (:then
      (Rendering|Components|Sprite|SetSprite (Variables|Components|GetSubjectIcon%20%28Temp%29) _astexture_2d)
      (Development|SetHiddeninGame (Variables|Components|GetSubjectIcon%20%28Temp%29) false false))
    (:CastFailed
      (Utilities|PrintStringRed15 "subject begin play cast to texture2d failed!"))))

(fn ChangeOccupation
  (params (newOccupation :type Name))
  (bind _returnvalue (Game|SpawnActorfromClass (CallFunction|GetOccupationClassDT newOccupation) (Transformation|GetActorTransform) "Undefined" 0 (Variables|Default|GetowningPlayerName) newOccupation true 0))
  (ChangeOccupation|InitChangedOccupation _returnvalue (Variables|Default|GetstatsMap) (Variables|Default|GetplayerLabel) (Variables|Default|GetcurrentFood) (Variables|Default|GetcurrentHealth))
  ;[1 1 1] need not remove original from residence, as that's handled at a later stage (this means that the residence building may have one over capacity for a couple of miliseconds (ends before THIS function is returned)
  (if (Utilities|IsValidandNotNull (Variables|Residence|Getresidence))
    (Residence|SetResidence _returnvalue (Variables|Residence|Getresidence)))
  ;[1 1 1] Delete Original, but in a way that player doesn't notice.
  (Class|Subject|SubjectDie true)
  (return _returnvalue))

(fn InitChangedOccupation
  (params (subjectStats :type Map%20of%20Names%20to%20Structs) (subjectName :type String) (currentFood :type Float%20%28single-precision%29) (currentHealth :type Float%20%28single-precision%29))
  ;[1 1 1] override in classes?
  (Variables|Default|SetinitialiseOverrideAllStats false)
  (ChangeOccupation|SetStatsMap subjectStats)
  (CallFunction|SetPlayerLabel (Utilities|Text|ToText(String) subjectName))
  (Variables|Default|SetcurrentFood currentFood)
  (Variables|Default|SetcurrentHealth currentHealth)
  (return false))

(fn SetRandomName
  (bind _returnvalue (Game|GetGameInstance))
  (bind _aswn_sgame_instance (Utilities|Casting|CastToWnSGameInstance _returnvalue))
  (Utilities|FlowControl|Sequence ; Firstname, then lastname, then set it.
    (:then_0
      (if (> (Variables|/Game/WnSAssets/Blueprints/Logics/WnSGameInstance.WnSGameInstance_C|GetDT_FirstnamesLength _aswn_sgame_instance) 0)
        (LocalVariables|SetdtLenMax (Variables|/Game/WnSAssets/Blueprints/Logics/WnSGameInstance.WnSGameInstance_C|GetDT_FirstnamesLength _aswn_sgame_instance))
        (else
          ;[1 1 1] if not already cached, find and cache length
          (bind _outrownames (DataTable|GetDataTableRowNames "/Game/WnSAssets/Data/Names/DT_Firstnames.DT_Firstnames"))
          (bind _output_get (Variables|/Game/WnSAssets/Blueprints/Logics/WnSGameInstance.WnSGameInstance_C|SetDT_FirstnamesLength _aswn_sgame_instance (Utilities|Array|Length _outrownames)))
          (LocalVariables|SetdtLenMax _output_get)))
      (bind _returnvalue_2 (Utilities|GetDataTableRow "/Game/WnSAssets/Data/Names/DT_Firstnames.DT_Firstnames" (Utilities|String|StringToName (Utilities|String|ToString(Integer) (Math|Random|RandomIntegerinRange 1 (LocalVariables|GetdtLenMax)))))
        (:then
          (LocalVariables|Setfirstname (Utilities|Struct|BreakDTS_Firstnames _returnvalue_2)))
        (:RowNotFound
          (Utilities|PrintStringRed15 "BP_Civilian SetRandomName didn't find row with firstname"))))
    (:then_1
      (if (> (Variables|/Game/WnSAssets/Blueprints/Logics/WnSGameInstance.WnSGameInstance_C|GetDT_LastnamesLength _aswn_sgame_instance) 0)
        (LocalVariables|SetdtLenMax (Variables|/Game/WnSAssets/Blueprints/Logics/WnSGameInstance.WnSGameInstance_C|GetDT_LastnamesLength _aswn_sgame_instance))
        (else
          ;[1 1 1] if not already cached, find and cache length
          (bind _outrownames_2 (DataTable|GetDataTableRowNames "/Game/WnSAssets/Data/Names/DT_Lastnames.DT_Lastnames"))
          (bind _output_get_2 (Variables|/Game/WnSAssets/Blueprints/Logics/WnSGameInstance.WnSGameInstance_C|SetDT_LastnamesLength _aswn_sgame_instance (Utilities|Array|Length _outrownames_2)))
          (LocalVariables|SetdtLenMax _output_get_2)))
      (bind _returnvalue_3 (Utilities|GetDataTableRow "/Game/WnSAssets/Data/Names/DT_Lastnames.DT_Lastnames" (Utilities|String|StringToName (Utilities|String|ToString(Integer) (Math|Random|RandomIntegerinRange 1 (LocalVariables|GetdtLenMax)))))
        (:then
          (LocalVariables|Setlastname (Utilities|Struct|BreakDTS_Lastnames _returnvalue_3)))
        (:RowNotFound
          (Utilities|PrintStringRed15 "BP_Civilian SetRandomName didn't find row with lastname"))))
    (:then_2
      (CallFunction|SetPlayerLabel (Utilities|Text|FormatText "{Firstname} {Lastname}" (LocalVariables|Getfirstname) (LocalVariables|Getlastname))))))

(fn MakeHungerDeathNotif
  (if (<= (Variables|Default|GetcurrentFood) 0.0)
    ;[1 1 1] Tell TutorialManager that a hungerdeath notification was made.
    (bind _aswn_s_player_controller (Utilities|Casting|CastToWnS_PlayerController (Game|GetPlayerController 0))
      (:then
        (Default|HungerDeathNotifWasSent (Variables|/Game/WnSAssets/Blueprints/Player/WnS_PlayerController.WnS_PlayerController_C|GettutorialManager _aswn_s_player_controller)))
      (:CastFailed
        (Utilities|PrintStringRed15 "Civilian handle civilian death cast to playercontroller failed!")))))

(fn SetStatsMap
  (params (newStatsMap :type Map%20of%20Names%20to%20Structs))
  (Variables|Default|SetstatsMap newStatsMap))

(fn ConsiderApplyingforJob
  (params (building :type BP%20Building%20Object%20Reference))
  (if (Utilities|Name|Equal(Name) (Variables|Default|GetsubjectOccupation) "Serf")
    (bind _returnvalue (Class|Subject|CalculateOccupationSuitability (Utilities|Struct|BreakDTS_Building (CallFunction|GetBuildingDT (Variables|/Game/WnSAssets/Blueprints/Actors/Intermediates/Lots/BP_Building.BP_Building_C|GetbuildingType building)))))
    (bind _returnvalue_2 (Class|Subject|CalculateOccupationSuitability (Variables|Default|GetsubjectOccupation)))
    (if (> _returnvalue (+ _returnvalue_2 (CallFunction|OccupationChangeMargin)))
      (Default|ApplicationforJob building (Utilities|Struct|MakeSubjectSuitabilityScore self _returnvalue)))))

(fn JobOffer
  (params (potentialWorkplace :type BP%20Building%20Object%20Reference) (score :type Float%20%28single-precision%29))
  (bind _returnvalue (Class|Subject|CalculateOccupationSuitability (Variables|Default|GetsubjectOccupation)))
  (if (> score _returnvalue) ; if new offer still better than current (sanity check)
    (bind _newsubject (ChangeOccupation|ChangeOccupation (Utilities|Struct|BreakDTS_Building (CallFunction|GetBuildingDT (Variables|/Game/WnSAssets/Blueprints/Actors/Intermediates/Lots/BP_Building.BP_Building_C|GetbuildingType potentialWorkplace)))))
    (Default|JobOfferAnswer potentialWorkplace _newsubject true)
    (else
      (Utilities|PrintStringRed15 (Utilities|String|Append "job offer has worse suitability than current job by " (Utilities|String|ToString(Float) (- _returnvalue score)))
        (:Exec
          (Default|JobOfferAnswer potentialWorkplace 0 false))))))

(fn SetResidence
  (params (newResidence :type BP%20Residential%20House%20Object%20Reference))
  (bind _output_get (Variables|Residence|Setresidence newResidence))
  (Default|AddResident _output_get self))

(fn LoseResidence
  (Variables|Residence|Setresidence 0))

(fn HandleFindResidence
  (bind _returnvalue (Utilities|Time|GetGameTimeinSeconds))
  (if (not (Utilities|IsValidandNotNull (Variables|Residence|Getresidence)))
    (if (> _returnvalue (+ (Variables|Residence|GetlastSearchedForResidenceTime) (Variables|Residence|GetsearchForResidenceDelay))) ; time to search again?
      (Variables|Residence|SetlastSearchedForResidenceTime _returnvalue)
      (bind _array_element (Utilities|Array|ForEachLoopwithBreak (Variables|/Game/WnSAssets/Blueprints/Logics/Managers/BP_ActorManager.BP_ActorManager_C|GetResidences (Variables|Default|GetactorManager)) :!label _label)
        (:LoopBody
          ;[1 0 0] FOR LOOP
          (bind _hasspace (Default|HasSpaceforNewResident _array_element))
          (if _hasspace
            (Residence|SetResidence _array_element)
            (goto _label Break)))))))

(fn RemovefromResidence
  (bind _residence (Variables|Residence|Getresidence))
  (if (Utilities|IsValidandNotNull _residence)
    (Default|RemoveResident _residence self)))

(fn ConsiderApplyingforBuilderJob
  (params (constructionSite :type BP%20Construction%20Site%20Object%20Reference))
  (if (Utilities|Name|Equal(Name) (Variables|Default|GetsubjectOccupation) "Serf")
    (bind _returnvalue (Class|Subject|CalculateOccupationSuitability "Builder"))
    (Utilities|PrintInfo (Utilities|String|Append (Variables|Default|GetplayerLabel) (Utilities|String|ToString(Float) _returnvalue))
      (:Exec
        (bind _returnvalue_2 (Class|Subject|CalculateOccupationSuitability (Variables|Default|GetsubjectOccupation)))
        ;[1 1 1] Builders are essential, so become one wether you like it or not. (dirty fix)
        (if (> _returnvalue (+ _returnvalue_2 (CallFunction|OccupationChangeMargin)))
          _
          (else
            _))
        (Default|ApplicationforBuilderJob constructionSite (Utilities|Struct|MakeSubjectSuitabilityScore self _returnvalue))))))

(fn BuilderJobOffer
  (params (constructionSite :type BP%20Construction%20Site%20Object%20Reference) (score :type Float%20%28single-precision%29))
  (bind _newsubject (ChangeOccupation|ChangeOccupation "Builder"))
  (Default|JobOfferAnswer constructionSite true _newsubject))