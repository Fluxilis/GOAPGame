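; BP_Crafter is a worker subject that crafts recipes at its home crafting building.
; It overrides parent readiness and home-removal logic, using a job status that moves from Crafting to Resting to None.
; Completing a craft calls the building's Crafting component, whose current recipe's product and duration feed the work-time calculation, while resting takes a fixed wait.
; Job description text reflects that status or trips to eat or go home.
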(event EventUpdateCurrentJobDescription
  ;[1 1 1] Override - Update Job Description
  (if (Variables|Default|GetgoingHome)
    (Variables|Default|SetCurrentJobDescription "Currently going home.")
    (elif (Variables|Default|GetgoingToEat)
      (Variables|Default|SetCurrentJobDescription "Currently going to eat.")
      (else
        (Variables|Default|SetCurrentJobDescription (Utilities|Text|ToText(String) (Utilities|String|Append "Currently " (Class|Globals|GetCraftingJobType (Variables|CrafterJob|GetcurrentJobStatus)) ".")))))))

(event EventRemoveHome
  ;[1 1 1] Override Remove Home
  (|CallParentFunction)
  (Crafter|CrafterRemoveHome))

(fn ConstructionScript
  (|CallParentFunction))

(fn HomeCanCraft
  (bind _asbp_crafting_building (Utilities|Casting|CastToBP_CraftingBuilding (Variables|Default|GetHomeBuilding))
    (:then
      (bind _returnvalue (Class|CraftingComponent|CanStartRecipe (Variables|/Game/WnSAssets/Blueprints/Actors/Intermediates/Lots/BP_CraftingBuilding.BP_CraftingBuilding_C|GetCrafting _asbp_crafting_building) (Variables|/Script/Burghers.CraftingComponent|GetcurrentRecipe (Variables|/Game/WnSAssets/Blueprints/Actors/Intermediates/Lots/BP_CraftingBuilding.BP_CraftingBuilding_C|GetCrafting _asbp_crafting_building))))
      (return _returnvalue))
    (:CastFailed
      (Development|PrintString "Crafter CanCraft Cast Failed!")
      (return false))))

(fn IsReadytoWork
  (bind _isready_ (|CallParentFunction))
  (return (and _isready_ (Utilities|Enum|Equal(Enum) (Variables|CrafterJob|GetcurrentJobStatus) "None"))))

(fn CompleteCrafting
  (bind _asbp_crafting_building (Utilities|Casting|CastToBP_CraftingBuilding (Variables|Default|GetHomeBuilding))
    (:then
      (Class|CraftingComponent|RecipeDone (Variables|/Game/WnSAssets/Blueprints/Actors/Intermediates/Lots/BP_CraftingBuilding.BP_CraftingBuilding_C|GetCrafting _asbp_crafting_building))
      (Crafter|SetJobStatus "Resting")
      (return true))
    (:CastFailed
      (Development|PrintString "Crafter CompleteCrafting Cast failed!")
      (return false))))

(fn CompleteResting
  (Crafter|SetJobStatus "None")
  (return true))

(fn GetCurrentJobWaitTime
  (switch Utilities|FlowControl|Switch|SwitchonECraftingJobType (Variables|CrafterJob|GetcurrentJobStatus)
    (:None
      (return 0.0))
    (:Crafting
      (bind _asbp_crafting_building (Utilities|Casting|CastToBP_CraftingBuilding (Variables|Default|GetHomeBuilding))
        (:then
          (bind _returnvalue (Class|Subject|CalculateWorkDuration (Utilities|String|StringToName (Utilities|String|Append "Craft" (Utilities|String|ToString(Name) (.itemType (Utilities|Struct|BreakItemAmount (Utilities|Array|Get(acopy) (.products (Variables|/Script/Burghers.CraftingComponent|GetcurrentRecipe (Variables|/Game/WnSAssets/Blueprints/Actors/Intermediates/Lots/BP_CraftingBuilding.BP_CraftingBuilding_C|GetCrafting _asbp_crafting_building))))))))) (.craftduration (Variables|/Script/Burghers.CraftingComponent|GetcurrentRecipe (Variables|/Game/WnSAssets/Blueprints/Actors/Intermediates/Lots/BP_CraftingBuilding.BP_CraftingBuilding_C|GetCrafting _asbp_crafting_building)))))
          (return _returnvalue))
        (:CastFailed
          (Utilities|PrintStringRed15 "BP_Crafter GetCurrentJobWaitTime Cast to craftingBuilding failed!"
            (:Exec
              (return 1.0))))))
    (:Resting
      (return 2.0))))

(fn GetCurrentJobDescription
  (if (Variables|Default|GetgoingToEat)
    (Variables|Default|SetCurrentJobDescription "Currently going to eat.")
    (CallFunction|UpdateUI "Job")
    (else
      (Variables|Default|SetCurrentJobDescription (Utilities|Text|ToText(String) (Utilities|String|Append "Currently " (Class|Globals|GetCraftingJobType (Variables|CrafterJob|GetcurrentJobStatus)) ".")))
      (CallFunction|UpdateUI "Job"))))

(fn SetJobStatus
  (params (currentJobStatus :type ECraftingJobType%20Enum :default "None"))
  (Variables|CrafterJob|SetcurrentJobStatus currentJobStatus)
  (CallFunction|UpdateJobDescriptiononServer))

(fn CrafterRemoveHome
  (Crafter|SetJobStatus "None")
  (CallFunction|UpdateJobDescriptiononServer))