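; Building lot actor that configures health, worker type, job limits, recipe and stockpiles from its BuildingType data table row.
; Vacancies are broadcast to all Subjects, which submit suitability scores; after a short delay the best gets an offer, and applications reopen if none suits or it refuses.
; Tick timers reopen applications and notify the player about missing workers.
; Destruction removes the worker's home, and loot boxes refund part of the construction materials.
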(event Custom|CloseJobApplicationsDelayed
  (Utilities|FlowControl|Delay 3.0)
  (ChangeOccupation|CloseJobApplications))

(event EventTick
  (params (DeltaSeconds :type Float%20%28single-precision%29))
  ;[1 1 1] Event Tick
  (|CallParentFunction DeltaSeconds)
  (Staff|CheckforStaffMissing)
  (Staff|CheckforStaffMissingNotification))

(event EventHandleDestroyLot
  ;[1 1 1] Destroy Lot Handle Destroy Building
  (CallFunction|HandleDestroyBuilding)
  (|CallParentFunction))

(event EventBeginPlay
  ;[1 1 1] Begin Play
  (|CallParentFunction)
  (CallFunction|InitiateBuildingType))

(fn ConstructionScript
  (|CallParentFunction)
  (if (Utilities|Name|NotEqual(Name) (Variables|Default|GetowningPlayerName) "DONOTHANDLE") ; set singleplayer playername \n(except special cases)
    (Variables|Default|SetowningPlayerName "wnsplayer0"))
  (CallFunction|InitiateBuildingType))

(fn GetMesh
  (return (Variables|/Script/Engine.StaticMeshComponent|GetStaticMesh (Variables|Default|GetModel))))

(fn RemoveMyStaff
  (Variables|Staff|SetMyStaff 0)
  ;[1 1 1] Remake UI
  (if (Utilities|IsValidandNotNull (Variables|Default|GetmyActorUI))
    (CallFunction|UpdateUI "StaffButton"))
  (Staff|StartMissingStaffTimer)
  (ChangeOccupation|OpenJobApplications))

(fn SetasMyStaff
  (params (Who? :type BP%20Housebased%20Object%20Reference))
  (Variables|Staff|SetMyStaff Who?)
  (CallFunction|UpdateUI "StaffButton"))

(fn HandleDestroyBuilding
  (if (Utilities|IsValidandNotNull (Variables|Staff|GetMyStaff))
    (Default|RemoveHome (Variables|Staff|GetMyStaff))))

(fn InitConstructionComplete
  (params (playerLabel :type Text) (currentHealth :type Float%20%28single-precision%29) (harvestAreaLocation :type Vector))
  (CallFunction|SetPlayerLabelonServer playerLabel) ; needed to replicate
  (Variables|Default|SetcurrentHealth currentHealth)
  (CallFunction|GetJobManagerandAddtoLots)
  (ChangeOccupation|OpenJobApplications))

(fn StartMissingStaffTimer
  ;[1 1 1] Check for missing Staff and start timer
  (if (Utilities|Name|NotEqual(Name) (Variables|BuildingSpecific|GetwhoWorksHere) "None") ; Does this building require a worker?
    (if (not (Utilities|IsValidandNotNull (Variables|Staff|GetMyStaff))) ; Is this building missing its worker?
      (Variables|Staff|SetmissingStaffStartTime (Utilities|Time|GetGameTimeinSeconds))
      (Variables|Staff|SetsentMissingStaffNotification false))))

(fn CheckforStaffMissingNotification
  (bind _self self)
  ;[1 1 1] Notify Player that building is missing worker.
  (if (Variables|Staff|GetsentMissingStaffNotification) ; Has the notification been sent already?
    ;[1 1 1] send a new notification later
    (Variables|Staff|SetmissingStaffStartTime (Utilities|Time|GetGameTimeinSeconds))
    (Variables|Staff|SetsentMissingStaffNotification false)
    (elif (Utilities|Name|NotEqual(Name) (Variables|BuildingSpecific|GetwhoWorksHere) "None") ; Does this building require a worker?
      (if (not (Utilities|IsValidandNotNull (Variables|Staff|GetMyStaff))) ; Is this building missing its worker?
        (if (< (+ (Variables|Staff|GetmissingStaffStartTime) (Variables|Staff|GetmissingStaffNotificationDelay)) (Utilities|Time|GetGameTimeinSeconds)) ; has the building been missing \nits worker for the specified duration?
          (bind _aswn_s_player_controller (Utilities|Casting|CastToWnS_PlayerController (Game|GetPlayerController 0))
            (:then
              (bind _w_hud (Default|GetWHud _aswn_s_player_controller))
              (Default|MakeNotification _w_hud (Utilities|Text|FormatText "This {BuildingType} is missing its worker, a {workerType}." (CallFunction|GetBuildingDisplayNameDT (Variables|BuildingSpecific|GetbuildingType)) (CallFunction|GetSubjectDisplayNameDT (Variables|BuildingSpecific|GetwhoWorksHere))) "/Game/WnSAssets/Visual/Icons/Notifications/newsIcon.newsIcon" (Default|GetDoorLocation _self) _self)
              (Variables|Staff|SetsentMissingStaffNotification true)
              ;[1 1 1] Tell TutorialManager that an unoccupied notification was made.
              (bind _aswn_s_player_controller_2 (Utilities|Casting|CastToWnS_PlayerController (Game|GetPlayerController 0))
                (:then
                  (Default|UnoccupiedNotifWasSent (Variables|/Game/WnSAssets/Blueprints/Player/WnS_PlayerController.WnS_PlayerController_C|GettutorialManager _aswn_s_player_controller_2)))
                (:CastFailed
                  (Utilities|PrintStringRed15 "Building Check for missing staff notif cast to pc failed"))))
            (:CastFailed
              (Utilities|PrintStringRed15 "subject handle die cast to pc failed!"))))))))

(fn MakeLootBox
  (if (Utilities|Name|NotEqual(Name) (Variables|Default|GetowningPlayerName) "DONOTHANDLE")
    (bind _lootbox (|CallParentFunction))
    (Utilities|FlowControl|Sequence
      (:then_0
        (for _array_element (.materials (Variables|BuildingSpecific|GetconstructionRecipe))
          ;[1 0 0] Foreach Loop
          (if (> (Math|Float|Round (* (.amount (Utilities|Struct|BreakItemAmount _array_element)) (CallFunction|BuildingResourceReturnFactor))) 0) ; Would at least one item of this type be returned?
            (Utilities|Array|Add (LocalVariables|GetstockpilesToAdd) (Utilities|Struct|MakeItemAmount (.itemType (Utilities|Struct|BreakItemAmount _array_element)) (Math|Float|Round (* (.amount (Utilities|Struct|BreakItemAmount _array_element)) (CallFunction|BuildingResourceReturnFactor)))))))
        (Default|AddStockpiles _lootbox (LocalVariables|GetstockpilesToAdd)))
      (:then_1
        (return _lootbox)))))

(fn SetOverheadIcon
  ;[1 1 1] Set Overhead Icon (Temporary)
  (bind _astexture_2d (Utilities|Casting|CastToTexture2D (CallFunction|GetBuildingIconDT (Variables|BuildingSpecific|GetbuildingType)))
    (:then
      (Rendering|Components|Sprite|SetSprite (Variables|Default|GetbuildingIcon%28Temp%29) _astexture_2d)
      (Development|SetHiddeninGame (Variables|Default|GetbuildingIcon%28Temp%29) false false))
    (:CastFailed
      (Utilities|PrintStringRed15 "building begin player cast to texture2d failed!"))))

(fn InitiateBuildingType
  (bind _buildingtype (Variables|BuildingSpecific|GetbuildingType))
  (bind _dtsbuilding (CallFunction|GetBuildingDT _buildingtype))
  (bind (_buildingname _displayname _maxhealth _whoworkshere _pulljoblimit _pushjoblimit _constructionrecipe _stockpiles) (Utilities|Struct|BreakDTS_Building _dtsbuilding))
  (Variables|Default|SetplayerLabel (Utilities|String|ToString(Text) _displayname))
  (bind _output_get (Variables|Default|SetmaxHealth _maxhealth))
  (Variables|Default|SetcurrentHealth _output_get)
  (Variables|BuildingSpecific|SetwhoWorksHere _whoworkshere)
  (Variables|Default|SetpullJobLimit (Math|Conversions|ToFloat(Integer) _pulljoblimit))
  (Variables|Default|SetpushJobLimit (Math|Conversions|ToFloat(Integer) _pushjoblimit))
  (Variables|BuildingSpecific|SetconstructionRecipe _constructionrecipe)
  (Variables|Default|Setstockpiles _stockpiles)
  (CallFunction|SetOverheadIcon)
  (Staff|StartMissingStaffTimer))

(fn OpenJobApplications
  (if (Variables|ChangeOccupation|GetjobApplicationsAreOpen)
    (Utilities|PrintStringRed15 (Utilities|String|Append (Variables|Default|GetplayerLabel) " job applications already open!"))
    (elif (Utilities|Name|NotEqual(Name) (Utilities|Struct|BreakDTS_Building (CallFunction|GetBuildingDT (Variables|BuildingSpecific|GetbuildingType))) "None") ; don't do for buildings that need no staff
      (if (Utilities|IsValidandNotNull (Variables|Staff|GetMyStaff))
        (Utilities|PrintError (Utilities|String|Append "attempted to open jobs for " (Variables|Default|GetplayerLabel) ", but still had staff!"))
        (else
          (Variables|ChangeOccupation|SetjobApplicationsAreOpen true)
          (for _array_element (Variables|/Game/WnSAssets/Blueprints/Logics/Managers/BP_ActorManager.BP_ActorManager_C|GetSubjects (Variables|Default|GetactorManager))
            ;[1 0 0] FOR LOOP
            (Default|NewJobAvailable _array_element self))
          (CallFunction|CloseJobApplicationsDelayed))))))

(fn ApplicationforJob
  (params (subjectSuitabilityScore :type Subject%20Suitability%20Score%20Structure))
  (Utilities|Array|Add (Variables|ChangeOccupation|GetjobApplicantsList) subjectSuitabilityScore))

(fn CloseJobApplications
  (if (Variables|ChangeOccupation|GetjobApplicationsAreOpen)
    (Variables|ChangeOccupation|SetjobApplicationsAreOpen false)
    (if (> (Utilities|Array|Length (Variables|ChangeOccupation|GetjobApplicantsList)) 0)
      (Utilities|FlowControl|Sequence
        (:then_0
          (for _array_element (Variables|ChangeOccupation|GetjobApplicantsList)
            ;[1 0 0] FOR LOOP - finds candidate with the highest suitabilityscore, and sets as best candidate.
            (if (Utilities|IsValidandNotNull (.subject (Utilities|Struct|BreakSubjectSuitabilityScore _array_element))) ; check if this subject is still valid
              (if (> (.score (Utilities|Struct|BreakSubjectSuitabilityScore _array_element)) (LocalVariables|GetbestScore))
                (LocalVariables|SetbestCandidate _array_element)
                (LocalVariables|SetbestScore (Utilities|Struct|BreakSubjectSuitabilityScore _array_element))))))
        (:then_1
          (Utilities|Array|Clear (Variables|ChangeOccupation|GetjobApplicantsList)))
        (:then_2
          (if (Utilities|IsValidandNotNull (.subject (Utilities|Struct|BreakSubjectSuitabilityScore (LocalVariables|GetbestCandidate))))
            (bind _asbp_subject (Utilities|Casting|CastToBP_Subject (.subject (Utilities|Struct|BreakSubjectSuitabilityScore (LocalVariables|GetbestCandidate))))
              (:then
                (Default|JobOffer _asbp_subject self (.score (Utilities|Struct|BreakSubjectSuitabilityScore (LocalVariables|GetbestCandidate)))))
              (:CastFailed
                (Utilities|PrintStringRed15 "BP_Building CloseJobApplications cast to bp_subject failed!"
                  (:Exec
                    (ChangeOccupation|OpenJobApplications) ; no valid best candidate applied, reopen.
                  ))))
            (else
              (ChangeOccupation|OpenJobApplications) ; no valid best candidate applied, reopen.
            ))))
      (else
        (ChangeOccupation|OpenJobApplications) ; no candidates applied, reopen job applications!
      ))
    (else
      (Utilities|PrintStringRed15 (Utilities|String|Append (Variables|Default|GetplayerLabel) " job applications were already closed!")))))

(fn JobOfferAnswer
  (params (subject :type BP%20Subject%20Object%20Reference) (acceptedJob :type Boolean))
  (if acceptedJob
    (bind _asbp_housebased (Utilities|Casting|CastToBP_Housebased subject)
      (:then
        (Default|SetNewHome _asbp_housebased self))
      (:CastFailed
        (Utilities|PrintStringRed15 "BP_Building JobOfferAnswer cast to housebased failed!")))
    (else
      (ChangeOccupation|OpenJobApplications)
      (Utilities|PrintStringRed15 (Utilities|String|Append "Candidate " (Variables|/Script/Burghers.Subject|GetplayerLabel subject) " refused job")))))

(fn CheckforStaffMissing
  (if (not (Variables|ChangeOccupation|GetjobApplicationsAreOpen)) ; Job applications already open?
    (if (Utilities|Name|NotEqual(Name) (Variables|BuildingSpecific|GetwhoWorksHere) "None") ; Does this building require a worker?
      (if (not (Utilities|IsValidandNotNull (Variables|Staff|GetMyStaff))) ; Is this building missing its worker?
        (if (< (+ (Variables|Staff|GetmissingStaffStartTime) (Variables|Staff|GetmissingStaffOpenApplicationsDelay)) (Utilities|Time|GetGameTimeinSeconds)) ; has the building been missing \nits worker for the specified duration?
          (ChangeOccupation|OpenJobApplications))))))