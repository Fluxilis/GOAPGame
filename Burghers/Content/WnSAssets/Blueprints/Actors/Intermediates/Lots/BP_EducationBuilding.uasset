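; Building actor that educates queued subjects, paying item costs from its storage and spawning the new subject at its door when done.
; On server Tick it advances education progress or periodically retries the next queued subject, while clients only advance progress visually.
; Queue and cancel requests are relayed through the player controller, and cancelling the current education refunds its cost.
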(event Custom|TryQueueSubjectOnServer
  (params (whatSubject :type Name))
  ;[1 1 1] Replication - Start Education on Server
  (bind _aswn_s_player_controller (Utilities|Casting|CastToWnS_PlayerController (Game|GetPlayerController 0)))
  (Default|TryQueue _aswn_s_player_controller self whatSubject))

(event Custom|CancelCurrentEducationOnServer
  ;[1 1 1] Replication - Cancel Current Education on Server
  (bind _aswn_s_player_controller (Utilities|Casting|CastToWnS_PlayerController (Game|GetPlayerController 0)))
  (Default|CancelCurrentEducation _aswn_s_player_controller self))

(event Custom|CancelQueuedOnServer
  (params (index :type Integer))
  ;[1 1 1] Replication - Cancel a Queued Education on Server
  (bind _aswn_s_player_controller (Utilities|Casting|CastToWnS_PlayerController (Game|GetPlayerController 0)))
  (Default|CancelQueued _aswn_s_player_controller self index))

(event EventBeginPlay
  (|CallParentFunction))

(event Collision|EventActorBeginOverlap
  (params (OtherActor :type Actor%20Object%20Reference)))

(event EventTick
  (params (DeltaSeconds :type Float%20%28single-precision%29))
  (|CallParentFunction DeltaSeconds)
  (Networking|SwitchHasAuthority
    (:Authority
      (if (Variables|EducationBuilding|Geteducating) ; Is already educating?
        (CallFunction|IncreaseEducationProgress DeltaSeconds)
        (else
          (CallFunction|TryEducateAfterSeconds DeltaSeconds))))
    (:Remote
      (CallFunction|IncreaseEducationProgressVisual DeltaSeconds))))

(fn ConstructionScript
  (|CallParentFunction))

(fn TryQueueSubject
  (params (whatSubject :type Name))
  (bind _subjectsqueue (Variables|EducationBuilding|GetsubjectsQueue))
  (if (< (Utilities|Array|Length (Variables|EducationBuilding|GetsubjectsQueue)) (Variables|EducationBuilding|GetmaxQueueSize))
    (Utilities|Array|Add _subjectsqueue whatSubject)
    (if (== (Utilities|Array|Length _subjectsqueue) 1)
      (CallFunction|TryStartEducateNextSubject))))

(fn StartEducateSubject
  (params (whatSubject :type Name))
  (Variables|EducationBuilding|SetcurrentEducating whatSubject)
  (Variables|EducationBuilding|SetcurrentEducationProgress 0.0)
  (Variables|EducationBuilding|Seteducating true)
  (Utilities|Array|RemoveIndex (Variables|EducationBuilding|GetsubjectsQueue))
  (for _array_element (CallFunction|GetSubjectEducateCostDT (Variables|EducationBuilding|GetcurrentEducating))
    (Class|Lot|DeleteItem (.itemtype _array_element) (.amount _array_element))
    (CallFunction|UpdateUI "School")))

(fn CompleteEducation
  (params (whatSubject :type Name))
  (Networking|SwitchHasAuthority ; *multiplayer relevant
    (:Authority
      ;[1 1 1] Spawn and Initialize new Subject
      (Game|SpawnActorfromClass (CallFunction|GetOccupationClassDT whatSubject) (Math|Conversions|ToTransform(Vector) (CallFunction|GetDoorLocation)) "Undefined" 0 (Variables|Default|GetowningPlayerName) whatSubject false 0)
      ;[1 1 1] Reset Education Building
      (Variables|EducationBuilding|Seteducating false)
      (Variables|EducationBuilding|SetcurrentEducating "None")
      (Math|Integer|IncrementInt (Variables|EducationBuilding|GetlifeTimeEducations)
        (:%20%20
          (Variables|EducationBuilding|SetcurrentEducationProgress 0.0)
          (Variables|EducationBuilding|SetcurrentEducateDelay 0.0))))))

(fn TryStartEducateNextSubject
  (bind _subjectsqueue (Variables|EducationBuilding|GetsubjectsQueue))
  (if (not (Variables|EducationBuilding|Geteducating)) ; Is already educating?
    (if (> (Utilities|Array|Length _subjectsqueue) 0) ; Has Subjects left in the queue?
      (LocalVariables|SetsubjectToEducate (Utilities|Array|Get(acopy) _subjectsqueue))
      (if (CallFunction|CanStartEducateSubject (LocalVariables|GetsubjectToEducate)) ; Does the building have the necessary \nitems to educate the Subject?
        (CallFunction|StartEducateSubject (LocalVariables|GetsubjectToEducate))))))

(fn CanStartEducateSubject
  (params (whatSubject :type Name))
  (for _array_element (CallFunction|GetSubjectEducateCostDT whatSubject)
    (if (not (Class|Lot|HasItemStored (.itemtype _array_element) (.amount _array_element)))
      (return false)))
  (return true) ; If not returned false yet,\nhas all items.
)

(fn IncreaseEducationProgress
  (params (DeltaTime :type Float%20%28single-precision%29))
  (if (Variables|EducationBuilding|Geteducating)
    (bind _output_get (Variables|EducationBuilding|SetcurrentEducationProgress (+ (/ DeltaTime (Variables|EducationBuilding|GetEducateDuration)) (Variables|EducationBuilding|GetcurrentEducationProgress))))
    (if (>= _output_get 1.0) ; Progress 100%?
      (CallFunction|CompleteEducation (Variables|EducationBuilding|GetcurrentEducating))
      (CallFunction|UpdateUI "All")
      (else
        (CallFunction|UpdateUI "SchoolProgress")))))

(fn CancelQueued
  (params (index :type Integer))
  (Utilities|Array|RemoveIndex (Variables|EducationBuilding|GetsubjectsQueue) index))

(fn CancelCurrentEducation
  (if (Utilities|Name|NotEqual(Name) (Variables|EducationBuilding|GetcurrentEducating) "None") ; Is actually educating \nsomeone right now?
    ;[1 1 1] Refund the cost
    (for _array_element (CallFunction|GetSubjectEducateCostDT (Variables|EducationBuilding|GetcurrentEducating))
      (Class|Lot|MakeItem (.itemtype _array_element) (.amount _array_element)))
    (Variables|EducationBuilding|SetcurrentEducating "None")
    (Variables|EducationBuilding|SetcurrentEducationProgress 0.0)
    (Variables|EducationBuilding|Seteducating false)
    (CallFunction|UpdateUI "All")))

(fn TryEducateAfterSeconds
  (params (DeltaTime :type Float%20%28single-precision%29))
  (bind _output_get (Variables|EducationBuilding|SetcurrentEducateDelay (+ DeltaTime (Variables|EducationBuilding|GetcurrentEducateDelay))))
  (if (> _output_get (Variables|EducationBuilding|GetstartEducateDelay))
    (Variables|EducationBuilding|SetcurrentEducateDelay 0.0)
    (if (not (Variables|EducationBuilding|Geteducating)) ; Is already educating?
      (CallFunction|TryStartEducateNextSubject))))

(fn IncreaseEducationProgressVisual
  (params (DeltaTime :type Float%20%28single-precision%29))
  (if (Utilities|Name|NotEqual(Name) (Variables|EducationBuilding|GetcurrentEducating) "None")
    (Variables|EducationBuilding|SetcurrentEducationProgress (+ (/ DeltaTime (Variables|EducationBuilding|GetEducateDuration)) (Variables|EducationBuilding|GetcurrentEducationProgress)))
    (CallFunction|UpdateUI "SchoolProgress")))