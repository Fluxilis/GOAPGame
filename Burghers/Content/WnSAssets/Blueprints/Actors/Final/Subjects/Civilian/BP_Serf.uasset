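; Serf civilian subject that hauls items between lots as transport jobs from its player's JobManager.
; On the authority it finds that manager by owning player or spawns one, then takes jobs, picks up and drops off items, and replicates the carried mesh.
; Cancelled jobs reroute carried items or drop them as timed lootboxes; death drops them too.
; It also builds job description text and advances a tutorial when its UI opens.
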(event Custom|ReplicatedSetCarriedItemMesh
  (params (serf :type BP%20Serf%20Object%20Reference) (NewMesh :type Static%20Mesh%20Object%20Reference))
  ;[1 1 1] Replication - Sets CarriedItem Mesh on clients
  (Components|StaticMesh|SetStaticMesh (Variables|BP_Serf_C|GetcarriedItemMesh serf) NewMesh))

(event EventBeginPlay
  (|CallParentFunction)
  (CallFunction|FindJobManager)
  (CallFunction|SetCarriedItemMesh))

(event EventSubjectHandleDie
  (params (invisible :type Boolean))
  ;[1 1 1] Override - Subject die
  (CallFunction|SerfHandleDie invisible)
  (|CallParentFunction invisible))

(event EventUpdateCurrentJobDescription
  ;[1 1 1] Override - Update Job Desctiption
  (if (Variables|Default|GetgoingToEat)
    (Variables|Default|SetCurrentJobDescription "Currently going to eat.")
    (CallFunction|UpdateUI "Job")
    (elif (Variables|Job|GethaveJob)
      (bind _jobdescription (CallFunction|GetJobDescriptionTextHasJob))
      (Variables|Default|SetCurrentJobDescription _jobdescription)
      (CallFunction|UpdateUI "Job")
      (else
        (Variables|Default|SetCurrentJobDescription "Currently Idle.")
        (CallFunction|UpdateUI "Job")))))

(event EventOpenUI
  (params (isOwnerUI :type Boolean))
  ;[1 1 1] Override - Open UI (Handle Tutorial)
  (|CallParentFunction isOwnerUI)
  (Tutorial|HandleTutBasic031))

(fn ConstructionScript
  (|CallParentFunction))

(fn FindandAssignJob
  (bind _jobmanager (Variables|Job|GetJobManager))
  (if (Utilities|IsValidandNotNull _jobmanager)
    (bind _returnvalue (Class|JobManager|FindJob _jobmanager))
    (bind _hasjobnow (CallFunction|AssignJob _returnvalue))
    (return _hasjobnow)))

(fn PickupItem
  (params (fromLot :type BP%20Lot%20Object%20Reference) (item :type Name))
  (Class|Lot|RemoveItem fromLot item 1)
  (Variables|/Script/WarriorsAndSerfs.Job|SetjobStatus (Variables|Job|GetmyJob) "ToDestination")
  (bind _output_get (Variables|Job|SetcarriedItem item))
  (CallFunction|SetCarriedItemMesh (CallFunction|GetItemMeshDT _output_get))
  (CallFunction|UpdateJobDescriptiononServer))

(fn DropOffItem
  (params (ToLot :type BP%20Lot%20Object%20Reference))
  (if (Utilities|Name|Equal(Name) (Variables|/Script/WarriorsAndSerfs.Job|Getitem (Variables|Job|GetmyJob)) (Variables|Job|GetcarriedItem))
    (Class|Lot|AddItem ToLot (Variables|Job|GetcarriedItem) 1)
    (Variables|Job|SetcarriedItem "None")
    (Variables|/Script/WarriorsAndSerfs.Job|SetjobStatus (Variables|Job|GetmyJob) "Finished")
    (Class|JobManager|CancelJob (Variables|Job|GetJobManager) (Variables|Job|GetmyJob))
    (Variables|Job|SetlastJobDestination ToLot)
    (Variables|Job|SetmyJob 0)
    (Variables|Job|SethaveJob false)
    (CallFunction|SetCarriedItemMesh)
    (CallFunction|UpdateJobDescriptiononServer)
    (else
      (Development|PrintString "Job Item and Carried Item do not match!" true true "(R=1.000000,G=0.000000,B=0.000000,A=1.000000)" 1e+01))))

(fn FindandAssignJobfromThisLot
  (params (From%20Which%20Lot :type BP%20Lot%20Object%20Reference))
  (bind _jobmanager (Variables|Job|GetJobManager))
  (if (Utilities|IsValidandNotNull _jobmanager)
    (bind _returnvalue (Class|JobManager|FindJobbyLot _jobmanager From%20Which%20Lot))
    (bind _hasjobnow (CallFunction|AssignJob _returnvalue))
    (return _hasjobnow)))

(fn SerfHandleDie
  (params (invisible :type Boolean))
  (Utilities|FlowControl|Sequence
    (:then_0
      (if (not (Utilities|Name|Equal(Name) (Variables|Job|GetcarriedItem) "None")) ; If carrying an Item
        (CallFunction|MakeLootbox)))
    (:then_1
      (if (Variables|Job|GethaveJob)
        (Class|JobManager|CancelJob (Variables|Job|GetJobManager) (Variables|Job|GetmyJob))))))

(fn FindJobManager
  (Networking|SwitchHasAuthority
    (:Authority
      (if (not (Utilities|IsValidandNotNull (Variables|Job|GetJobManager))) ; Do I already (NOT) have a JobManager?
        (bind _outactors (Actor|GetAllActorswithTag "JobManager"))
        (if (> (Utilities|Array|Length _outactors) 0) ; Are there any job managers yet?
          (for _array_element _outactors
            ;[1 1 1] Check if any of the found Jobmanagers are the one for this player
            (bind _asjob_manager (Utilities|Casting|CastToJobManager _array_element)
              (:then
                (if (Utilities|Name|Equal(Name) (Variables|/Script/WarriorsAndSerfs.JobManager|GetowningPlayerName _asjob_manager) (Variables|Default|GetowningPlayerName)) ; Is this the Jobmanager for my player?
                  ;;[1 1 1] Found the Job manager!
                  ;; Set, then return (so loop breaks)
                  (Variables|Default|SetjobManager _asjob_manager)
                  (return)))
              (:CastFailed
                (Development|PrintString "Serf FindJobManager Could not cast to JobManager!!")))))
        (bind _returnvalue (Game|SpawnActorfromClass "/Game/WnSAssets/Blueprints/Logics/Managers/BP_JobManager.BP_JobManager_C" (Math|Transform|MakeTransform "0, 0, 0") "AlwaysSpawn" 0 0)) ; If no JobManager for this player was found, create a new one!
        (Variables|/Script/WarriorsAndSerfs.JobManager|SetowningPlayerName _returnvalue (Variables|Default|GetowningPlayerName))
        (Variables|Default|SetjobManager _returnvalue)))))

(fn SetCarriedItemMesh
  (params (NewMesh :type Static%20Mesh%20Object%20Reference))
  (Networking|SwitchHasAuthority
    (:Authority
      (CallFunction|ReplicatedSetCarriedItemMesh self NewMesh))))

(fn CancelJob
  (if (Utilities|Name|Equal(Name) (Variables|Job|GetcarriedItem) "None") ; is the serf (not) carrying an item?
    ;[1 1 1] Set to no job
    (Variables|Job|SetmyJob 0)
    (Variables|Job|SethaveJob false)
    (CallFunction|UpdateJobDescriptiononServer)
    (else
      (bind _returnvalue (Class|JobManager|FindJobforItem (Variables|Job|GetJobManager) (Variables|Job|GetcarriedItem)))
      (if (Utilities|IsValidandNotNull _returnvalue) ; Could find a job?
        (bind _hasjobnow (CallFunction|AssignJob _returnvalue))
        (if (not _hasjobnow) ; Successfully assigned job?
          ;[1 1 1] If couldn't find job, or place to dump item, dump it on the ground.
          (CallFunction|MakeLootbox :!label _label)
          (Variables|Job|SetcarriedItem "None")
          (CallFunction|SetCarriedItemMesh))
        (else
          (goto _label))))))

(fn MakeLootbox
  (bind _capsulecomponent (Variables|Default|GetCapsuleComponent))
  (bind _returnvalue (Transformation|GetWorldTransform _capsulecomponent))
  (bind (_location _rotation) (Math|Transform|BreakTransform _returnvalue))
  (if (not (Utilities|Name|Equal(Name) (Variables|Default|GetowningPlayerName) "DONOTHANDLE")) ; Under some conditions, \ndo not make a loot box.
    (Utilities|FlowControl|Sequence
      (:then_0
        (bind _returnvalue_2 (Game|SpawnActorfromClass "/Game/WnSAssets/Blueprints/Actors/Final/LootBox.LootBox_C" (Math|Transform|MakeTransform _location _rotation "0.500000,0.500000,0.500000") "AlwaysSpawn" 0 (Variables|Default|GetowningPlayerName) 0))
        (LocalVariables|SetnewLootBox _returnvalue_2)
        (Default|AddStockpiles (LocalVariables|GetnewLootBox) (Utilities|Array|MakeArray (Utilities|Struct|MakeItemAmount (Variables|Job|GetcarriedItem) 1)))
        (Default|InitLifetime (LocalVariables|GetnewLootBox) 9e+01))
      (:then_1
        (return (LocalVariables|GetnewLootBox))))))

(fn AssignJob
  (params (job :type Job%20Object%20Reference))
  (bind _output_get (Variables|Job|SetmyJob job))
  (bind _output_get_2 (Variables|Job|SethaveJob (Utilities|IsValidandNotNull _output_get)))
  (if _output_get_2
    (CallFunction|UpdateJobDescriptiononServer))
  (return _output_get_2))

(fn GetJobDescriptionTextHasJob
  (bind _myjob (Variables|Job|GetmyJob))
  (bind _myjob_2 (Variables|Job|GetmyJob))
  (bind _source (Variables|/Script/WarriorsAndSerfs.Job|Getsource _myjob))
  (bind _destination (Variables|/Script/WarriorsAndSerfs.Job|Getdestination _myjob_2))
  (if (Utilities|IsValidandNotNull (Variables|Job|GetmyJob))
    (Utilities|FlowControl|Sequence
      (:then_0
        (Utilities|FlowControl|Sequence
          (:then_0
            ;[1 1 1] Source Part
            (if (Utilities|IsValidandNotNull _source)
              (LocalVariables|SetsourceName (Utilities|Text|ToText(String) (Variables|/Script/WarriorsAndSerfs.Lot|GetplayerLabel _source)))
              (else
                (LocalVariables|SetsourceName "None"))))
          (:then_1
            ;[1 1 1] Destination part
            (if (Utilities|IsValidandNotNull _destination)
              (LocalVariables|SetdestinationName (Utilities|Text|ToText(String) (Variables|/Script/WarriorsAndSerfs.Lot|GetplayerLabel _destination)))
              (else
                (LocalVariables|SetdestinationName "None"))))
          (:then_2
            ;[1 1 1] Item part
            (LocalVariables|SetitemName (CallFunction|GetItemDisplayNameDT (Variables|/Script/WarriorsAndSerfs.Job|Getitem (Variables|Job|GetmyJob)))))
          (:then_3
            ;[1 1 1] Status part
            (switch Utilities|FlowControl|Switch|SwitchonEJobStatus (Variables|/Script/WarriorsAndSerfs.Job|GetjobStatus (Variables|Job|GetmyJob))
              (:ToSource
                (LocalVariables|SetstatusPart (Utilities|Text|MakeLiteralText "(Picking up Item)")))
              (:ToDestination
                (LocalVariables|SetstatusPart (Utilities|Text|MakeLiteralText "(Delivering Item)")))))
          (:then_4
            ;[1 1 1] Piecing it together
            (LocalVariables|SetfinalDescription (Utilities|Text|FormatText "Currently transporting {ItemName} from {Source} to {Destination}. {Status}" (LocalVariables|GetitemName) (LocalVariables|GetsourceName) (LocalVariables|GetdestinationName) (LocalVariables|GetstatusPart))))))
      (:then_1
        (return (LocalVariables|GetfinalDescription))))
    (else
      (return "Job was not valid..."))))

(fn HandleTutBasic031
  (Utilities|FlowControl|Sequence
    (:then_0
      (if (Variables|Tutorial|GetBasic03_1Completed) ; Was tutorial basic03_01 completed yet?\n(check local)
        (return)
        (else
          (bind _aswn_s_player_controller (Utilities|Casting|CastToWnS_PlayerController (Game|GetPlayerController 0))
            (:then
              (bind _completed (Default|GetTutorialCompletionStatus (Variables|/Game/WnSAssets/Blueprints/Player/WnS_PlayerController.WnS_PlayerController_C|GettutorialManager _aswn_s_player_controller) "Basic03_1"))
              (if _completed ; Was tutorial basic03_1 ACTUALLY completed yet?\n(Check tutorial manager)
                (Variables|Tutorial|SetBasic03_1Completed true)
                (return)))
            (:CastFailed
              (Utilities|PrintStringRed15 "serf open UI cast to playercontroller failed"))))))
    (:then_1
      (if (not (Variables|Tutorial|GetBasic03Completed)) ; Was the previous tut completed yet?\n(check local)
        (bind _aswn_s_player_controller_2 (Utilities|Casting|CastToWnS_PlayerController (Game|GetPlayerController 0))
          (:then
            (bind _completed_2 (Default|GetTutorialCompletionStatus (Variables|/Game/WnSAssets/Blueprints/Player/WnS_PlayerController.WnS_PlayerController_C|GettutorialManager _aswn_s_player_controller_2) "Basic03"))
            (if _completed_2 ; Was tutorial basic03 ACTUALLY completed yet?\n(Check tutorial manager)
              (Variables|Tutorial|SetBasic03Completed true)
              (else
                (return))))
          (:CastFailed
            (Utilities|PrintStringRed15 "serf open UI cast to playercontroller failed (2)")))))
    (:then_2
      (bind _aswn_s_player_controller_3 (Utilities|Casting|CastToWnS_PlayerController (Game|GetPlayerController 0)))
      (Default|CompleteTutorial (Variables|/Game/WnSAssets/Blueprints/Player/WnS_PlayerController.WnS_PlayerController_C|GettutorialManager _aswn_s_player_controller_3) "Basic03_1"))))