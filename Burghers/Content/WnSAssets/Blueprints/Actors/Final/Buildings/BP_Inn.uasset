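; BP_Inn is an inn building actor where a subject can eat from the building's stockpiles.
; SubjectEatHere removes one item from the first stockpile whose stored and predicted counts are both positive, returning true, or false if none qualifies.
; It does not filter by item type or change the eater, and its no-food debug print is disconnected.
; The event graph holds only disabled default events.
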(event EventBeginPlay
  (|CallParentFunction))

(event Collision|EventActorBeginOverlap
  (params (OtherActor :type Actor%20Object%20Reference)))

(event EventTick
  (params (DeltaSeconds :type Float%20%28single-precision%29))
  (|CallParentFunction DeltaSeconds))

(fn ConstructionScript
  (|CallParentFunction))

(fn SubjectEatHere
  (params (WhoEatsHere :type BP%20Civilian%20Object%20Reference))
  (for _array_element (Variables|Default|Getstockpiles)
    (if (and (> (.currentStored (Utilities|Struct|BreakStockpile _array_element)) 0) (> (.currentPredicted (Utilities|Struct|BreakStockpile _array_element)) 0)) ; If food is in stockpile
      (Class|Lot|DeleteItem (.itemType (Utilities|Struct|BreakStockpile _array_element)) 1)
      (return true)))
  (return false))