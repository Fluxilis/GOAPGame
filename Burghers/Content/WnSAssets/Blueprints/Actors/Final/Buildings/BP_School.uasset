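; BP_School is the school building, a child Blueprint that adds tutorial tracking and coin-job rules to inherited education logic.
; After an education completes, it flags a Forester graduate for the Basic06 tutorial and completes that tutorial once all its steps are done.
; It gates new coin jobs during education, reserving stockpile room for the in-use coin in case education is cancelled.
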(event EventBeginPlay
  (|CallParentFunction))

(event Collision|EventActorBeginOverlap
  (params (OtherActor :type Actor%20Object%20Reference)))

(event EventTick
  (params (DeltaSeconds :type Float%20%28single-precision%29))
  (|CallParentFunction DeltaSeconds))

(event EventCompleteEducation
  (params (whatSubject :type Name :default "None"))
  ;[1 1 1] Override Complete education - check if tutorial was completed
  (|CallParentFunction whatSubject)
  (Tutorial|HandleBasic06 whatSubject))

(event EventMakeJobAfterSeconds
  (params (DeltaTime :type Float%20%28single-precision%29))
  ;[1 1 1] Override Make Job After seconds
  ; School special case: if there is less than max stored coins, while someone is being educated currently, do not make a job for a new coin. (as education may be cancelled).
  (bind _allownewjob (CallFunction|AllowMakeNewCoinJob))
  (if _allownewjob
    (|CallParentFunction DeltaTime)))

(fn ConstructionScript
  (|CallParentFunction))

(fn HandleBasic06
  (params (educatedSubject :type Name))
  (if (not (Variables|Tutorial|GetBasic06Completed))
    (LocalVariables|SetnewlyEducatedSubject educatedSubject)
    (bind _aswn_s_player_controller (Utilities|Casting|CastToWnS_PlayerController (Game|GetPlayerController 0))
      (:then
        (bind _output_get (LocalVariables|SettutManager (Variables|/Game/WnSAssets/Blueprints/Player/WnS_PlayerController.WnS_PlayerController_C|GettutorialManager _aswn_s_player_controller)))
        (bind _completed (Default|GetTutorialCompletionStatus _output_get "Basic06"))
        (if _completed ; Has the tutorial been completed alread?
          (Variables|Tutorial|SetBasic06Completed true)
          (else
            (Utilities|FlowControl|Sequence
              (:then_0
                ;[1 0 0] Sequence Then 0
                (if (Utilities|Name|Equal(Name) (LocalVariables|GetnewlyEducatedSubject) "Forester") ; Was the educated subject\na forester?
                  (Variables|/Game/WnSAssets/Tutorial/TutorialManager.TutorialManager_C|SetBasic06ForesterEdu (LocalVariables|GettutManager) true)))
              (:then_1
                (if (Math|Boolean|ANDBoolean (Variables|/Game/WnSAssets/Tutorial/TutorialManager.TutorialManager_C|GetBasic06ForesterEdu (LocalVariables|GettutManager)) (Variables|/Game/WnSAssets/Tutorial/TutorialManager.TutorialManager_C|GetBasic06ForestingBuilt (LocalVariables|GettutManager)) (Variables|/Game/WnSAssets/Tutorial/TutorialManager.TutorialManager_C|GetBasic06HarvestAreaMoved (LocalVariables|GettutManager))) ; Have all components of \nthe tutorial been completed?
                  (Default|CompleteTutorial (LocalVariables|GettutManager) "Basic06")))))))
      (:CastFailed
        (Utilities|PrintStringRed15 "School HandleBasic06 cast to pc failed!")))))

(fn AllowMakeNewCoinJob
  (bind _stockpiles (Variables|Default|Getstockpiles))
  (bind _output (Utilities|Array|Get(acopy) _stockpiles))
  (bind (_maxstorage _currentpredicted) (Utilities|Struct|BreakStockpile _output))
  (return (or (not (Variables|Default|Geteducating)) (and (Variables|Default|Geteducating) (< _currentpredicted (- _maxstorage 1))))))