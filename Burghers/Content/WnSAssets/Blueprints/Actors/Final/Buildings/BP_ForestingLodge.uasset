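; BP_ForestingLodge is a forestry lodge building whose only added logic completes the "Basic06" tutorial by existing in the world.
; On top of its parent's tick, it calls HandleBasic06 every frame, which queries the TutorialManager on player 0's WnS_PlayerController and completes the tutorial if still open.
; A local flag stops the polling once the manager reports completion, and a failed controller cast prints an error.
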(event EventTick
  (params (DeltaSeconds :type Float%20%28single-precision%29))
  (|CallParentFunction DeltaSeconds)
  (if (not (Variables|Tutorial|Getbasic06Completed))
    (Tutorial|HandleBasic06)))

(fn ConstructionScript
  (|CallParentFunction))

(fn HandleBasic06
  (if (not (Variables|Tutorial|Getbasic06Completed))
    (bind _aswn_s_player_controller (Utilities|Casting|CastToWnS_PlayerController (Game|GetPlayerController 0))
      (:then
        (bind _output_get (Variables|Tutorial|SettutManager (Variables|/Game/WnSAssets/Blueprints/Player/WnS_PlayerController.WnS_PlayerController_C|GettutorialManager _aswn_s_player_controller)))
        (bind _completed (Default|GetTutorialCompletionStatus _output_get "Basic06"))
        (if _completed ; Has the tutorial Basic046\nbeen completed yet?
          (Variables|Tutorial|Setbasic06Completed true)
          (else
            ;[1 1 1] the existance of this building completes the tutorial.
            (Default|CompleteTutorial (Variables|Tutorial|GettutManager) "Basic06"))))
      (:CastFailed
        (Utilities|PrintStringRed15 "ForestingLodge HandleBasic06 cast to pc failed!")))))