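; Palace building whose construction counts as a win condition in the strategic game.
; On BeginPlay it reports a "BuildPalace" win to WnS_StrategicGameMode, unless the owner name is "DONOTHANDLE" or DoNotWinGame is set.
; SubjectEatHere feeds a subject by deleting one item from the first stockpile with positive stored and predicted amounts, returning whether one was found.
; The job priority increase is overridden empty, so the palace never raises priorities.
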(event EventBeginPlay
  (|CallParentFunction)
  (CallFunction|HandleGameWin))

(event Collision|EventActorBeginOverlap
  (params (OtherActor :type Actor%20Object%20Reference)))

(event EventHandleIncreaseJobPriorities
  ;[1 1 1] Override HandleIncreaseJobPriorities
  ; Do not increase job priorities for the palace...
)

(event EventTick
  (params (DeltaSeconds :type Float%20%28single-precision%29))
  (|CallParentFunction DeltaSeconds))

(fn ConstructionScript
  (|CallParentFunction))

(fn SubjectEatHere
  (params (WhoEatsHere :type BP%20Civilian%20Object%20Reference))
  (for _array_element (Variables|Default|Getstockpiles)
    (if (and (> (.currentStored (Utilities|Struct|BreakStockpile _array_element)) 0) (> (.currentPredicted (Utilities|Struct|BreakStockpile _array_element)) 0)) ; If food is in stockpile
      (Class|Lot|DeleteItem (.itemType (Utilities|Struct|BreakStockpile _array_element)) 1)
      (return true)))
  (return false))

(fn HandleGameWin
  (if (not (Utilities|Name|Equal(Name) (Variables|Default|GetowningPlayerName) "DONOTHANDLE"))
    (if (not (Variables|BuildingSpecific|GetdoNotWinGame))
      (bind _aswn_s_strategic_game_mode (Utilities|Casting|CastToWnS_StrategicGameMode (Game|GetGameMode))
        (:then
          (Default|GameWin _aswn_s_strategic_game_mode "BuildPalace"))
        (:CastFailed
          (Utilities|PrintStringRed15 "palace begin play cast to strategic gamemode failed!"))))))