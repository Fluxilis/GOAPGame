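; Woodcutters building actor that tracks its part of the Basic04 tutorial on top of its parent building behavior.
; Each tick until the tutorial completes, it queries the player controller's TutorialManager and caches completion locally to stop further checks.
; Once its Harvesting lifetime count shows it has produced an item, it sets the woodcutter flag on the manager.
; It completes Basic04 when both woodcutter and sawmill flags are set.
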(event EventTick
  (params (DeltaSeconds :type Float%20%28single-precision%29))
  (|CallParentFunction DeltaSeconds)
  (if (not (Variables|Tutorial|Getbasic04Completed))
    (CallFunction|HandleBasic04)))

(fn ConstructionScript
  (|CallParentFunction))

(fn HandleBasic04
  (if (not (Variables|Tutorial|Getbasic04Completed))
    (bind _aswn_s_player_controller (Utilities|Casting|CastToWnS_PlayerController (Game|GetPlayerController 0))
      (:then
        (bind _output_get (LocalVariables|SettutManager (Variables|/Game/WnSAssets/Blueprints/Player/WnS_PlayerController.WnS_PlayerController_C|GettutorialManager _aswn_s_player_controller)))
        (bind _completed (Default|GetTutorialCompletionStatus _output_get "Basic04"))
        (if _completed ; Has the tutorial Basic04 \nbeen completed yet?
          (Variables|Tutorial|Setbasic04Completed true)
          (else
            (Utilities|FlowControl|Sequence
              (:then_0
                ;[1 0 0] Sequence Then 0
                (if (> (Variables|/Script/WarriorsAndSerfs.HarvestingComponent|GetlifeTimePolishes (Variables|Default|GetHarvesting)) 0.0) ; has this woodcutter ever \nmade an item?
                  (Variables|/Game/WnSAssets/Tutorial/TutorialManager.TutorialManager_C|SetBasic04WoodCutter (LocalVariables|GettutManager) true)))
              (:then_1
                (if (and (Variables|/Game/WnSAssets/Tutorial/TutorialManager.TutorialManager_C|GetBasic04WoodCutter (LocalVariables|GettutManager)) (Variables|/Game/WnSAssets/Tutorial/TutorialManager.TutorialManager_C|GetBasic04Sawmill (LocalVariables|GettutManager))) ; Have all components of \nthe tutorial been completed?
                  (Default|CompleteTutorial (LocalVariables|GettutManager) "Basic04")))))))
      (:CastFailed
        (Utilities|PrintStringRed15 "Woodcutters HandleBasic04 cast to pc failed!")))))