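; Residential house building that raises the citizen limit and houses serfs.
; While it has free capacity, Tick spawns a BP_Serf at the door after each delay and sets the house as its residence.
; It tracks residents through add and remove functions, restarting the spawn timer when one is removed.
; Overridden actor manager hooks adjust the citizen limit, and destroying the lot makes every resident lose their residence.
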(event EventBeginPlay
  (|CallParentFunction)
  (Variables|ResidentialHouse|SetcitizenSpawnCounterStartTime (Utilities|Time|GetGameTimeinSeconds)))

(event Collision|EventActorBeginOverlap
  (params (OtherActor :type Actor%20Object%20Reference)))

(event EventTick
  (params (DeltaSeconds :type Float%20%28single-precision%29))
  (|CallParentFunction DeltaSeconds)
  (ResidentialHouse|SpawnNewCitizens))

(event EventRemovefromActorManager
  ;[1 1 1] Override Add/Remove from actor manager, to change Citizen limit.
  (|CallParentFunction)
  (ResidentialHouse|ResidentialHouseRemovefromActorManager))

(event EventAddtoActorManager
  ;[1 1 1] Override Add/Remove from actor manager, to change Citizen limit.
  (|CallParentFunction)
  (ResidentialHouse|ResidentialHouseAddtoActorManager))

(event EventHandleDestroyLot
  (ResidentialHouse|ResidentialHouseHandleDestroyLot)
  (|CallParentFunction))

(fn ConstructionScript
  (|CallParentFunction))

(fn ResidentialHouseAddtoActorManager
  (Default|ChangeCitizenLimit (Variables|Default|GetactorManager) (Variables|ResidentialHouse|GetcitizenCapacity)))

(fn ResidentialHouseRemovefromActorManager
  (Default|ChangeCitizenLimit (Variables|Default|GetactorManager) (* (Variables|ResidentialHouse|GetcitizenCapacity) -1)))

(fn SpawnNewCitizens
  (if (< (Variables|ResidentialHouse|GetcurrentCitizenCount) (Variables|ResidentialHouse|GetcitizenCapacity)) ; capacity for more citizens?
    (if (> (Utilities|Time|GetGameTimeinSeconds) (+ (Variables|ResidentialHouse|GetcitizenSpawnCounterStartTime) (Variables|ResidentialHouse|GetnewCitizenSpawnDelay))) ; time to spawn new?
      (Variables|ResidentialHouse|SetcitizenSpawnCounterStartTime (Utilities|Time|GetGameTimeinSeconds))
      ;[1 1 1] Spawn new citizen
      (bind _returnvalue (Game|SpawnActorfromClass "/Game/WnSAssets/Blueprints/Actors/Final/Subjects/Civilian/BP_Serf.BP_Serf_C" (Math|Conversions|ToTransform(Vector) (CallFunction|GetDoorLocation)) "Undefined" 0 (Variables|Default|GetowningPlayerName) "None" false 0))
      (Default|SetResidence _returnvalue self))))

(fn AddResident
  (params (newResident :type BP%20Subject%20Object%20Reference))
  (Utilities|Array|Add (Variables|ResidentialHouse|Getresidents) newResident)
  (Math|Integer|IncrementInt (Variables|ResidentialHouse|GetcurrentCitizenCount)))

(fn RemoveResident
  (params (newResident :type BP%20Subject%20Object%20Reference))
  (Utilities|Array|RemoveItem (Variables|ResidentialHouse|Getresidents) newResident)
  (Math|Integer|DecrementInt (Variables|ResidentialHouse|GetcurrentCitizenCount)
    (:%20%20
      (Variables|ResidentialHouse|SetcitizenSpawnCounterStartTime (Utilities|Time|GetGameTimeinSeconds)))))

(fn ResidentialHouseHandleDestroyLot
  (for _array_element (Variables|ResidentialHouse|Getresidents)
    ;[1 0 0] FOR LOOP
    (Default|LoseResidence _array_element)))

(fn HasSpaceforNewResident
  (if (< (Variables|ResidentialHouse|GetcurrentCitizenCount) (Variables|ResidentialHouse|GetcitizenCapacity))
    (return true)
    (else
      (return false))))