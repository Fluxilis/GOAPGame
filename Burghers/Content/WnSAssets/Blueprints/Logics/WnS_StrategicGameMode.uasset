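; Game mode for the strategy map that sets up joining players and handles win and game-over screens.
; Players arriving by lobby travel or direct login get generated ownership names and, on authority, data-table-driven building and subject permissions, with schools excluded.
; Game over triggers when CheckGameOver finds no living subjects; the school-with-gold check is disconnected.
; End screens pause the first player controller, and logout calls the game instance to destroy the session.
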(event EventOnSwapPlayerControllers
  (params (OldPC :type Player%20Controller%20Object%20Reference) (NewPC :type Player%20Controller%20Object%20Reference))
  ;[1 1 1] Keeps track of connected player controllers
  ; THIS ONLY HAPPENS IF PLAYERS ARE ENTERING THE MAP AFTER CONNECTING TO THE SERVER IN THE LOBBY MAP!
  (Utilities|Array|Add (Variables|GameInfo|GetallPlayerControllers) NewPC)
  (CallFunction|InitiatePlayer NewPC))

(event EventOnLogout
  (params (ExitingController :type Controller%20Object%20Reference))
  ;[1 1 1] On Logout destroy session caller in gameinstance
  (bind _aswn_s_player_controller (Utilities|Casting|CastToWnS_PlayerController ExitingController))
  (Default|DestroySessionCaller (.AsWn%20SGame%20Instance (Utilities|Casting|CastToWnSGameInstance (Game|GetGameInstance))) _aswn_s_player_controller))

(event EventPostLogin
  (params (NewPlayer :type Player%20Controller%20Object%20Reference))
  ;[1 1 1] Event OnPostLogin
  ; THIS ONLY HAPPENS IF PLAYERS ARE CONNECTING TO THE SERVER IN THE GAME MAP!
  ; (ie when I'm testing!!)
  ; Initiates the player
  (Utilities|Array|Add (Variables|GameInfo|GetallPlayerControllers) NewPlayer)
  (CallFunction|InitiatePlayer NewPlayer))

(fn ConstructionScript)

(fn AllowAllImplementedSubjects
  (params (playerState :type Wn%20S%20Player%20State%20Object%20Reference))
  (bind _outrownames (DataTable|GetDataTableRowNames "/Game/WnSAssets/Data/Subjects/DT_Subjects.DT_Subjects"))
  (for _array_element _outrownames
    (Default|SetAllowSubject playerState _array_element (AllowedActors|IsSubjectImplemented _array_element))))

(fn AllowAllImplementedBuildings
  (params (playerState :type Wn%20S%20Player%20State%20Object%20Reference))
  (bind _outrownames (DataTable|GetDataTableRowNames "/Game/WnSAssets/Data/Buildings/DT_Buildings.DT_Buildings"))
  (for _array_element _outrownames
    (Default|SetAllowBuilding playerState _array_element (AllowedActors|IsBuildingImplemented _array_element))))

(fn AllowAllImplementedforPlayer
  (params (playerController :type Player%20Controller%20Object%20Reference))
  (Networking|SwitchHasAuthority
    (:Authority
      (bind _aswn_splayer_state (Utilities|Casting|CastToWnSPlayerState (Variables|/Script/Engine.Controller|GetPlayerState playerController)))
      (AllowedActors|AllowAllImplementedBuildings _aswn_splayer_state)
      (AllowedActors|AllowAllImplementedSubjects _aswn_splayer_state))))

(fn GetNewPlayerName
  (LocalVariables|SetreturnString (Utilities|String|Append (Variables|PlayerNames|GetplayerNamePrefix) (Utilities|String|ToString(Integer) (Variables|PlayerNames|GetnextPlayerID))))
  (Math|Integer|IncrementInt (Variables|PlayerNames|GetnextPlayerID)
    (:%20%20
      (Utilities|Array|Add (Variables|PlayerNames|GetusedPlayerNames) (Utilities|String|StringToName (LocalVariables|GetreturnString)))
      (return (Utilities|String|StringToName (LocalVariables|GetreturnString))))))

(fn IsUsedPlayerName
  (params (name :type Name))
  (return (!= (Utilities|Array|FindItem (Variables|PlayerNames|GetusedPlayerNames) name) -1)))

(fn IsValidPlayerName
  (params (name :type Name))
  (return (Utilities|String|Contains (Utilities|String|ToString(Name) name) (Variables|PlayerNames|GetplayerNamePrefix))))

(fn InitiatePlayer
  (params (playerController :type Player%20Controller%20Object%20Reference))
  (Networking|SwitchHasAuthority
    (:Authority
      (AllowedActors|AllowAllImplementedforPlayer playerController)
      (bind _aswn_splayer_state (Utilities|Casting|CastToWnSPlayerState (Variables|/Script/Engine.Controller|GetPlayerState playerController))
        (:then
          (bind _name (PlayerNames|GetNewPlayerName))
          (Variables|/Game/WnSAssets/Blueprints/Player/WnSPlayerState.WnSPlayerState_C|SetplayerOwnershipName _aswn_splayer_state _name))
        (:CastFailed
          (Development|PrintString "GameMode InitPlayer Cast to WnSPlayerState Failed!" true true "(R=1.000000,G=0.000000,B=0.000000,A=1.000000)" 1e+03))))))

(fn CheckGameOver
  (if (not (> (Utilities|Array|Length (Variables|/Game/WnSAssets/Blueprints/Logics/Managers/BP_ActorManager.BP_ActorManager_C|GetSubjects (Variables|Default|GetactorManager))) 0)) ; Are any subjects still alive?
    (GameOver|GameOver "NoSubjects")))

(fn DoesSchoolwithGoldExist
  (for _array_element (Variables|/Game/WnSAssets/Blueprints/Logics/Managers/BP_ActorManager.BP_ActorManager_C|GetBuildings (Variables|Default|GetactorManager))
    (bind _asbp_school (Utilities|Casting|CastToBP_School _array_element))
    (if (Class|Lot|HasItemStored _asbp_school "GoldCoins" 1)
      (return true)))
  (return false) ; If not returned true yet..
)

(fn GameOver
  (params (gameOverCause :type Name))
  (Utilities|FlowControl|Sequence
    (:then_0
      (switch name gameOverCause
        (:Default
          (bind _returnvalue (UserInterface|CreateWidget "/Game/WnSAssets/Widgets/Gameplay/GameOver/GameOverWidget.GameOverWidget_C" 0 "No particular reason lol."))
          (LocalVariables|SetgameOverWidget _returnvalue))
        (:NoSubjects
          (bind _returnvalue_2 (UserInterface|CreateWidget "/Game/WnSAssets/Widgets/Gameplay/GameOver/GameOverWidget.GameOverWidget_C" 0 "You govern a Ghost Town.  
Everyone is dead or left, and they will not return."))
          (LocalVariables|SetgameOverWidget _returnvalue_2))))
    (:then_1
      (UserInterface|Viewport|AddtoViewport (LocalVariables|GetgameOverWidget) 0)
      (bind _aswn_s_player_controller (Utilities|Casting|CastToWnS_PlayerController (Game|GetPlayerController 0))
        (:then
          (Default|PauseGame _aswn_s_player_controller))
        (:CastFailed
          (Utilities|PrintStringRed15 "gamemode gameOver cast to playercontroller failed!"))))))

(fn GameWin
  (params (winCause :type Name))
  (Utilities|FlowControl|Sequence
    (:then_0
      (switch name winCause
        (:Default
          (bind _returnvalue (UserInterface|CreateWidget "/Game/WnSAssets/Widgets/Gameplay/GameWin/GameWinWidget.GameWinWidget_C" 0 "No particular reason lol."))
          (LocalVariables|SetgameWinWidget _returnvalue))
        (:BuildPalace
          (bind _returnvalue_2 (UserInterface|CreateWidget "/Game/WnSAssets/Widgets/Gameplay/GameWin/GameWinWidget.GameWinWidget_C" 0 "You have completed the palace. 
There is no doubt that you are a wise and powerful ruler."))
          (LocalVariables|SetgameWinWidget _returnvalue_2))))
    (:then_1
      (UserInterface|Viewport|AddtoViewport (LocalVariables|GetgameWinWidget) 0)
      (bind _aswn_s_player_controller (Utilities|Casting|CastToWnS_PlayerController (Game|GetPlayerController 0))
        (:then
          (Default|PauseGame _aswn_s_player_controller))
        (:CastFailed
          (Utilities|PrintStringRed15 "gamemode gameWin cast to playercontroller failed!"))))))

(fn IsSubjectImplemented
  (params (subjectType :type Name))
  (Utilities|GetDataTableRow "/Game/WnSAssets/Data/Subjects/DT_Subjects.DT_Subjects" subjectType
    (:then
      (return true))
    (:RowNotFound
      (return false))))

(fn IsBuildingImplemented
  (params (buildingType :type Name))
  (Utilities|GetDataTableRow "/Game/WnSAssets/Data/Buildings/DT_Buildings.DT_Buildings" buildingType
    (:then
      ;[1 1 1] Special case, schools are removed from the game.
      (if (Utilities|Name|Equal(Name) buildingType "School")
        (return false)
        (else
          (return true))))
    (:RowNotFound
      (return false))))