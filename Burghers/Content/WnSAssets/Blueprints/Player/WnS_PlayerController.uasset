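; Player controller for the strategy game, handling HUD, pause, help popups, chat and multiplayer player commands.
; BeginPlay loads the saved online profile, passes it to the server, creates the local HUD, spawns a TutorialManager and resets game speed.
; Replication events relay UI commands to subjects, lots, buildings and players, while chat fans out through the GameMode's controller list.
; Pausing freezes the game only for singleplayer authority; one reused widget shows all help.
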(event Custom|PlaceConstructionsite
  (params (whatPlayer :type Wns%20Player%20Object%20Reference) (whatBuilding :type BP%20Building%20Class%20Reference) (location :type Transform) (buildingTypeN :type Name))
  ;[1 1 1] Replication - Place a constructionsite
  (Default|PlaceConstructionSite whatPlayer whatBuilding location buildingTypeN))

(event Custom|SetLotPlayerLabel
  (params (lot :type BP%20Lot%20Object%20Reference) (label :type Text))
  ;[1 1 1] Replication - Changing PlayerLabel on Lot through UI
  (Default|NotifyClientsChangedPlayerLabel lot label))

(event Custom|SetConstructionHarvestingArea
  (params (building :type BP%20Construction%20Site%20Object%20Reference) (location :type Vector))
  ;[1 1 1] Replication - Move Harvesting Area of a constructionsite
  (Default|NotifyClientsNewHarvestingArea building location))

(event Custom|SetHarvestingArea
  (params (building :type BP%20Harvesting%20Building%20Object%20Reference) (location :type Vector))
  ;[1 1 1] Replication - Move Harvesting Area of Lot
  (Default|NotifyClientsNewHarvestingArea building location))

(event Custom|UpdateJobDescription
  (params (subject :type BP%20Subject%20Object%20Reference))
  ;[1 1 1] Replication - Update Job Description of Subject
  (Default|UpdateCurrentJobDescription subject)
  (Default|NotifyClientsUpdatedJobDescription subject (Variables|/Game/WnSAssets/Blueprints/Actors/Intermediates/Subjects/BP_Subject.BP_Subject_C|GetCurrentJobDescription subject)))

(event Custom|SendChatMessage
  (params (textToSend :type Text))
  (bind _returnvalue (Math|DateTime|Now))
  ;[1 1 1] Process and Handle incoming chat, calls updatechat on clients
  (Variables|Multiplayer|SetsenderText textToSend)
  (Variables|Multiplayer|SetsenderName (.myPlayerName (Utilities|Struct|BreakonlineProfile (Variables|Multiplayer|GetonlineProfile))))
  (bind _aswn_s_strategic_game_mode (Utilities|Casting|CastToWnS_StrategicGameMode (Game|GetGameMode)))
  (for _array_element (Variables|/Game/WnSAssets/Blueprints/Logics/WnS_StrategicGameMode.WnS_StrategicGameMode_C|GetallPlayerControllers _aswn_s_strategic_game_mode)
    (bind _aswn_s_player_controller (Utilities|Casting|CastToWnS_PlayerController _array_element))
    (CallFunction|UpdateChat _aswn_s_player_controller (Variables|Multiplayer|GetsenderName) (Utilities|Text|FormatText "{Hour}:{Minute}:{Second}" (CallFunction|AsDoubleDigit (Class|KismetMathLibrary|GetHour _returnvalue)) (CallFunction|AsDoubleDigit (Class|KismetMathLibrary|GetMinute _returnvalue)) (CallFunction|AsDoubleDigit (Class|KismetMathLibrary|GetSecond _returnvalue))) (Variables|Multiplayer|GetsenderText))))

(event Custom|PassPlayerInfoToServer
  (params (onlineProfile :type Online%20Profile%20Structure))
  ;[1 1 1] Pass PlayerSettings to server, call setup chat window
  (Variables|Multiplayer|SetonlineProfile onlineProfile))

(event Custom|CancelQueued
  (params (educationBuilding :type BP%20Education%20Building%20Object%20Reference) (index :type Integer))
  ;[1 1 1] Replication - Cancel a Queued Education
  (Default|CancelQueued educationBuilding index))

(event Custom|DestroyLot
  (params (lot :type BP%20Lot%20Object%20Reference))
  ;[1 1 1] Replication - Destroying Lots
  (Class|Lot|DestroyLot lot))

(event Custom|TryQueue
  (params (educationBuilding :type BP%20Education%20Building%20Object%20Reference) (subjectType :type Name))
  ;[1 1 1] Replication - Start Educating a Subject
  (Default|TryQueueSubject educationBuilding subjectType))

(event Custom|CancelCurrentEducation
  (params (educationBuilding :type BP%20Education%20Building%20Object%20Reference))
  ;[1 1 1] Replication - Cancel Current Education
  (Default|CancelCurrentEducation educationBuilding))

(event Custom|SetupChatWindow
  ;[1 1 1] TO REMOVE
  (bind _returnvalue (UserInterface|CreateWidget "/Game/WnSAssets/Widgets/Menus/GameplayChat.GameplayChat_C"))
  (bind _output_get (Variables|Multiplayer|SetgameplayChatWidget _returnvalue))
  (UserInterface|Viewport|AddtoViewport _output_get 0))

(event Custom|UpdateChat
  (params (senderName :type Text) (senderTime :type Text) (senderText :type Text))
  ;[1 1 1] Updates the client chatwindow
  (Default|UpdateChatWindow (Variables|/Game/WnSAssets/Widgets/Menus/GameplayChat.GameplayChat_C|GetChatWindow (Variables|Multiplayer|GetgameplayChatWidget)) senderName senderTime senderText))

(event Custom|SetSubjectPlayerLabel
  (params (subject :type BP%20Subject%20Object%20Reference) (label :type Text))
  ;[1 1 1] Replication - Changing PlayerLabel on Subject through UI
  (Default|NotifyClientsChangedPlayerLabel subject label))

(event Custom|KillSubject
  (params (subject :type BP%20Subject%20Object%20Reference))
  ;[1 1 1] Replication - Killing Subjects
  (Default|SubjectHandleDie subject false))

(event EventBeginPlay
  ;[1 1 1] Begin Play
  ; Handle Multiplayer stuff
  ; Create Hud
  (|CallParentFunction)
  ;;[1 1 1] Set GameInstance
  (bind _aswn_sgame_instance (Utilities|Casting|CastToWnSGameInstance (Game|GetGameInstance))
    (:then
      (Variables|References|SetgameInstance _aswn_sgame_instance)
      ;;[1 1 1] Multiplayer - Loads player info and pass character info to serverside playercontroller
      (if (Pawn|IsLocalController)
        (Viewport|RemoveAllWidgets)
        (Multiplayer|LoadOnlineProfile)
        (CallFunction|PassPlayerInfotoServer (Variables|Multiplayer|GetonlineProfile)))
      ;;[1 1 1] Create Hud on clients
      (if (Pawn|IsLocalPlayerController)
        (CallFunction|CreateHUDWidget))
      ;;[1 1 1] Spawn and set the reference to tutorialManager
      (bind _returnvalue (Game|SpawnActorfromClass "/Game/WnSAssets/Tutorial/TutorialManager.TutorialManager_C" (Utilities|ZeroTransform) "AlwaysSpawn" 0 0))
      (Variables|References|SettutorialManager _returnvalue)
      ;;[1 1 1] Reset Gamespeed
      (Default|ResetGameSpeed (Variables|References|GetgameInstance)))
    (:CastFailed
      (Utilities|PrintStringRed15 "PC begin play cast to GI failed"))))

(fn ConstructionScript)

(fn IsKeyDown
  (params (InAxisName :type Name))
  (return (Game|Player|IsInputKeyDown (.key (Utilities|Array|Get(acopy) (Class|InputSettings|GetAxisMappingbyName (Class|InputSettings|GetInputSettings) InAxisName))))))

(fn GetWHud
  (if (Utilities|IsValidandNotNull (Variables|References|GetcurrentHudWidget))
    (bind _asw_hud (Utilities|Casting|CastToW_Hud (Variables|References|GetcurrentHudWidget))
      (:then
        (return _asw_hud))
      (:CastFailed
        (Development|PrintString "WnSPlayerController GetWHud Cast To W_Hud Failed")))
    (else
      ;[1 1 1] As this always happen at the start of the game, do not display error logs then...
      (if (> (Utilities|Time|GetGameTimeinSeconds) 0.5)
        (Development|PrintString "WnSPlayerController GetWHud WHud not found!")))))

(fn OpenPauseMenuandPause
  (PauseGame|PauseGame)
  ;[1 1 1] Show Pause Overlay
  (bind _w_hud (CallFunction|GetWHud))
  (Default|ShowPauseOverlay _w_hud true)
  ;[1 1 1] Open Pause Menu
  (bind _aswn_sgame_instance (Utilities|Casting|CastToWnSGameInstance (Game|GetGameInstance))
    (:then
      (Default|ShowPauseMenu _aswn_sgame_instance)
      (Audio|PlaySoundatLocation "/Game/WnSAssets/Audio/Files/UI/click.click" "0, 0, 0" "0, 0, 0" 1.0 1.0 0.0 0 0 0))
    (:CastFailed
      (Utilities|PrintStringRed15 "Player Controller Pause Game second cast to gameinstance failed!"))))

(fn CreateHUDWidget
  (bind _hudwidget (Variables|References|GetHudWidget))
  (if (Pawn|IsLocalPlayerController)
    (if (Utilities|IsValidClass _hudwidget)
      (bind _returnvalue (UserInterface|CreateWidget _hudwidget self))
      (bind _output_get (Variables|References|SetcurrentHudWidget _returnvalue))
      (UserInterface|Viewport|AddtoViewport _output_get 0)
      (else
        (Development|PrintString "PlayerController::CreateHUDWidget Hud Widget not Valid Class")))))

(fn LoadOnlineProfile
  (bind _returnvalue (SaveGame|LoadGamefromSlot (CallFunction|PlayerProfileSaveSlot)))
  (bind _asplayer_profile (Utilities|Casting|CastToPlayerProfile _returnvalue))
  (Variables|Multiplayer|SetonlineProfile (Variables|/Game/WnSAssets/Blueprints/Menus/PlayerProfile.PlayerProfile_C|GetonlineProfile _asplayer_profile)))

(fn GetMyWnSPlayer
  (bind _aswns_player (Utilities|Casting|CastToWnsPlayer (Pawn|GetControlledPawn))
    (:then
      (return _aswns_player))
    (:CastFailed
      (Development|PrintString "WnSPlayerController GetMyWnSPlayer cast to wnsPlayer failed!" true true "(R=1.000000,G=0.070812,B=0.130541,A=1.000000)" 2e+01)
      (return 0))))

(fn UnpauseGame
  (if (Variables|PauseGame|GetisGamePaused)
    (Variables|PauseGame|SetisGamePaused false)
    (Networking|SwitchHasAuthority
      (:Authority
        (Game|SetGamePaused false))
      (:Remote
        _))
    (bind _w_hud (CallFunction|GetWHud))
    (Default|ShowPauseOverlay _w_hud false)))

(fn ShowHelpPopup
  (if (Utilities|IsValidandNotNull (Variables|HelpPopup|GethelpPopup))
    _
    (else
      (bind _returnvalue (UserInterface|CreateWidget "/Game/WnSAssets/Widgets/Gameplay/HelpPopup.HelpPopup_C"))
      (Variables|HelpPopup|SethelpPopup _returnvalue)))
  (if (not (UserInterface|Viewport|IsinViewport (Variables|HelpPopup|GethelpPopup))) ; Is the popup already visible?
    (UserInterface|Viewport|AddtoViewport (Variables|HelpPopup|GethelpPopup) 0)))

(fn ShowBuildingHelp
  (params (buildingType :type Name))
  (HelpPopup|ShowHelpPopup)
  (Default|SetHelpforBuilding (Variables|HelpPopup|GethelpPopup) buildingType))

(fn ShowGenericHelp
  (params (text :type Text))
  (HelpPopup|ShowHelpPopup)
  (Default|SetGenericText (Variables|HelpPopup|GethelpPopup) text))

(fn ShowSubjectHelp
  (params (subjectType :type Name))
  (HelpPopup|ShowHelpPopup)
  (Default|SetHelpforSubject (Variables|HelpPopup|GethelpPopup) subjectType))

(fn ShowConstructionsiteHelp
  (params (building :type Name))
  (HelpPopup|ShowHelpPopup)
  (Default|SetHelpforConstruction (Variables|HelpPopup|GethelpPopup) building))

(fn PauseGame
  (bind _self self)
  (if (not (Variables|PauseGame|GetisGamePaused))
    (Variables|PauseGame|SetisGamePaused true)
    ;[1 1 1] Pause Game
    ; - only allow if singleplayer, and only try if authority (this needs to happen before pause menu is constructed)
    (Networking|SwitchHasAuthority
      (:Authority
        (bind _aswn_sgame_instance (Utilities|Casting|CastToWnSGameInstance (Game|GetGameInstance))
          (:then
            (bind _returnvalue (Default|IsGameSingleplayer _aswn_sgame_instance))
            (if _returnvalue ; Is this game singleplayer?
              (Game|SetGamePaused true))
            (Input|SetInputModeGameandUI _self 0 "DoNotLock" false :!label _label)
            (Variables|/Script/Engine.PlayerController|SetbShowMouseCursor _self true))
          (:CastFailed
            (Utilities|PrintStringRed15 "wns_PC PauseGame first cast to game instance failed"))))
      (:Remote
        (goto _label)))))

(fn ShowHarvestableHelp
  (params (harvestableType :type Name))
  (HelpPopup|ShowHelpPopup)
  (Default|SetHelpforHarvestable (Variables|HelpPopup|GethelpPopup) harvestableType))