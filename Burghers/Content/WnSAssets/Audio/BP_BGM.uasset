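; Background music player that exists in every map and cycles through the in-game playlist.
; On BeginPlay it registers itself as the GameInstance's BgmPlayer and starts the first song, advancing whenever the audio component finishes.
; Next and previous functions wrap around the playlist, and playback stores the song's name without underscores as text.
; It also creates the build version overlay, an admitted hack that piggybacks on its presence in every map.
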(event OnAudioFinished(AudioComponent)
  ;[1 1 1] When a song is over, play the next song.
  (CallFunction|PlayNextSong))

(event EventBeginPlay
  ;[1 1 1] Begin Play. Set reference in GameInstance and play song at index 0
  (bind _aswn_sgame_instance (Utilities|Casting|CastToWnSGameInstance (Game|GetGameInstance))
    (:then
      (Variables|/Game/WnSAssets/Blueprints/Logics/WnSGameInstance.WnSGameInstance_C|SetbgmPlayer _aswn_sgame_instance self)
      (CallFunction|PlaySongatIndex)
      ;;[1 1 1] THIS DOES NOT BELONG HERE
      ;; Create the version overlay. I'm abusing the BGM object, because that one also exists in every map.
      (Utilities|FlowControl|Delay 0.0001)
      (bind _returnvalue (UserInterface|CreateWidget "/Game/WnSAssets/Widgets/BuildVersionOverlay.BuildVersionOverlay_C" (Game|GetPlayerController 0)))
      (UserInterface|Viewport|AddtoViewport _returnvalue 0))
    (:CastFailed
      (Utilities|PrintStringRed15 "BP_BGM begin play cast to wnsgameinstance failed!"))))

(fn ConstructionScript)

(fn PlayNextSong
  (bind _result (Math|Integer|IncrementInt (Variables|BgmPlayer|GetsongIndex))
    (:%20%20
      (if (>= _result (Utilities|Array|Length (Variables|BgmPlayer|GetingamePlaylist)))
        (Variables|BgmPlayer|SetsongIndex 0))
      (CallFunction|PlaySongatIndex (Variables|BgmPlayer|GetsongIndex)))))

(fn PlayPreviousSong
  (bind _result (Math|Integer|DecrementInt (Variables|BgmPlayer|GetsongIndex))
    (:%20%20
      (if (< _result 0)
        (Variables|BgmPlayer|SetsongIndex (- (Utilities|Array|Length (Variables|BgmPlayer|GetingamePlaylist)) 1)))
      (CallFunction|PlaySongatIndex (Variables|BgmPlayer|GetsongIndex)))))

(fn PlaySongatIndex
  (params (index :type Integer))
  (bind _ingameplaylist (Variables|BgmPlayer|GetingamePlaylist))
  (bind _output (Utilities|Array|Get(acopy) _ingameplaylist index))
  (if (not (or (< index 0) (>= index (Utilities|Array|Length (Variables|BgmPlayer|GetingamePlaylist))))) ; is the index invalid?
    (Audio|Components|Audio|SetSound (Variables|Components|GetAudioComponent) _output)
    (Audio|Components|Audio|Play (Variables|Components|GetAudioComponent) 0.0)
    (Variables|BgmPlayer|SetcurrentPlayingSong (Utilities|Text|ToText(String) (Utilities|String|Replace (Utilities|GetDisplayName _output) "_" " ")))))